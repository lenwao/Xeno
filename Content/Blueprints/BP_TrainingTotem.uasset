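; BP_TrainingTotem is an overlap-triggered totem that launches boss training in a shooter.
; When a NEW_Pawn touches it, it hides its cube, pulses BP_AreaSpawn, optionally growls and follows the pawn each Tick.
; After delays it stops its particles, starts spawning with the training boss, and destroys the menu, options and test actors, then itself.
; Separate events fade its audio through a timeline played forward or reversed.
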(event `Audio_Totem_Off`
  (bind (_direction _value) (`Timeline|Timeline_0` :!label _label)
    (:`Update`
      (`AudioComponent.SetVolumeMultiplier` (`self.Audio`) _value))))

(event `Audio_Totem_On`
  (goto _label :!via `Reverse`))

(event `self.ReceiveTick`
  (params (DeltaSeconds :type "Float (single-precision)"))
  (if (`self.Taken`)
    (`self.K2_SetActorLocation` (`self.K2_GetActorLocation` (`self.Ref_Pawn`)))))

(event `self.ReceiveBeginPlay`
  (bind _asgm_shooter (cast `/Game/Blueprints/GM_Shooter` (`GameplayStatics.GetGameMode`)))
  (set `self.Ref_GM` _asgm_shooter))

(event `self.Cube.OnComponentBeginOverlap`
  (params (OverlappedComponent :type "PrimitiveComponent Object Reference") (OtherActor :type "Actor Object Reference") (OtherComp :type "PrimitiveComponent Object Reference") (OtherBodyIndex :type Integer) (bFromSweep :type Boolean) (SweepResult :type "HitResult Structure (by ref)"))
  (bind _asnew_pawn (cast `/Game/Blueprints/Pawn/NEW_Pawn` OtherActor))
  (set `self.Ref_Pawn` _asnew_pawn)
  (bind _outactors (`GameplayStatics.GetAllActorsOfClass` "/Game/Blueprints/Pawn/BP_AreaSpawn.BP_AreaSpawn_C"))
  (`/Game/Blueprints/Pawn/BP_AreaSpawn.Pulse` (`|GetArrayItem` _outactors))
  (`SceneComponent.SetVisibility` (`self.Cube`) false false)
  (set `self.Taken` true)
  (if (`/Game/Blueprints/GM_Shooter.SoundOn?` (`self.Ref_GM`))
    (`GameplayStatics.PlaySound2D` "/Game/Audio/Growl_Boss.Growl_Boss" 1.0 1.0 0.0 null null))
  (`KismetSystemLibrary.Delay` 3.0)
  (`ActorComponent.Deactivate` (`self.P_Shine01`))
  (`ActorComponent.Deactivate` (`self.P_Shine02`))
  (`KismetSystemLibrary.Delay` 1.0)
  (set `self.Taken` false)
  (bind _outactors_2 (`GameplayStatics.GetAllActorsOfClass` "/Game/Blueprints/Pawn/BP_AreaSpawn.BP_AreaSpawn_C"))
  (bind _output (`|GetArrayItem` _outactors_2))
  (`/Game/Blueprints/Pawn/BP_AreaSpawn.StartSpawn` _output)
  (`/Game/Blueprints/Pawn/BP_AreaSpawn.Training` _output (`self.TrainingBoss`) null)
  (`|ExecutionSequence`
    (:`then_0`
      (bind _outactors_3 (`GameplayStatics.GetAllActorsOfClass` "/Game/Blueprints/Widgets/BP_Menu.BP_Menu_C"))
      (`self.K2_DestroyActor` (`|GetArrayItem` _outactors_3)))
    (:`then_1`
      (bind _outactors_4 (`GameplayStatics.GetAllActorsOfClass` "/Game/Blueprints/Widgets/BP_Options.BP_Options_C"))
      (`self.K2_DestroyActor` (`|GetArrayItem` _outactors_4)))
    (:`then_2`
      (bind _outactors_5 (`GameplayStatics.GetAllActorsOfClass` "/Game/Blueprints/Widgets/BP_TEST.BP_TEST_C"))
      (`self.K2_DestroyActor` (`|GetArrayItem` _outactors_5)))
    (:`then_4`
      (`AudioComponent.Stop` (`self.Audio`))
      (`self.K2_DestroyActor`))))

(fn `UserConstructionScript`)