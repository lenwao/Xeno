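; Short-lived bullet actor ("Balas") for the shooter game that destroys itself one second after spawning.
; An externally called Hit event flags it as hit, spawns blood at the Plane component and destroys it.
; Until then, collision overlaps with BP_Dash_Blue_IA spawn sparks and, if GM_Shooter has sound on, a random-pitch metal clang.
; That overlap destroys the bullet, as do overlaps with four boss-type classes, silently and without effects.
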(event `Hit`
  (bind (_returnvalue_x _returnvalue_y _returnvalue_z) (`KismetMathLibrary.BreakVector` (`SceneComponent.K2_GetComponentLocation` (`self.Plane`))))
  (set `self.Hitted` true)
  (`GameplayStatics.SpawnEmitterAtLocation` "/Game/Particles/P_Hit_Blood.P_Hit_Blood" (`KismetMathLibrary.MakeVector` _returnvalue_x _returnvalue_y (- _returnvalue_z 20.0)) (struct) (0.5 0.5 0.5))
  (`self.K2_DestroyActor` :!label _label))

(event `self.ReceiveBeginPlay`
  (bind _asgm_shooter (cast `/Game/Blueprints/GM_Shooter` (`GameplayStatics.GetGameMode`)))
  (set `self.Ref_GM` _asgm_shooter)
  (`KismetSystemLibrary.Delay` 1.0)
  (goto _label))

(event `self.Collision.OnComponentBeginOverlap`
  (params (OverlappedComponent :type "PrimitiveComponent Object Reference") (OtherActor :type "Actor Object Reference") (OtherComp :type "PrimitiveComponent Object Reference") (OtherBodyIndex :type Integer) (bFromSweep :type Boolean) (SweepResult :type "HitResult Structure (by ref)"))
  (if (not (`self.Hitted`))
    (cast `/Game/Blueprints/Aliens/BP_Dash_Blue_IA` OtherActor
      (:`then`
        (if (`/Game/Blueprints/GM_Shooter.SoundOn?` (`self.Ref_GM`))
          (`GameplayStatics.PlaySound2D` "/Game/Audio/metalsound.metalsound" 1.0 (`KismetMathLibrary.RandomFloatInRange` 0.0 1.0) 0.0 null null))
        (`GameplayStatics.SpawnEmitterAtLocation` "/Game/Particles/P_Hit_Sparks.P_Hit_Sparks" (`SceneComponent.K2_GetComponentLocation` (`self.Plane`)))
        (`self.K2_DestroyActor`))
      (:`CastFailed`
        (cast `/Game/Blueprints/Aliens/NEW_Boss_giant_IA` OtherActor
          (:`then`
            _)
          (:`CastFailed`
            (cast `/Game/Blueprints/Aliens/BP_ElBolas` OtherActor
              (:`then`
                _)
              (:`CastFailed`
                (cast `/Game/INUSE/BP_BossWao_IA` OtherActor
                  (:`then`
                    _)
                  (:`CastFailed`
                    (cast `/Game/INUSE/BP_BossWaoHijo` OtherActor)))))))
        (`self.K2_DestroyActor`)))))

(fn `UserConstructionScript`)