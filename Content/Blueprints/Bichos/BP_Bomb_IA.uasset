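; Suicide bomber alien enemy that explodes when shot or when the player pawn lingers in its blast range.
; RangeSphere tracks nearby actors; a pawn inside stops movement, changes the light's blink frequency and starts a short countdown.
; BombDie damages allied enemies, chain-detonates other bombs, kills the pawn and calls AnotherBomb on BP_AreaSpawn.
; Tick jitters leg yaw randomly; close contact also kills the pawn.
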(event `self.ReceiveBeginPlay`
  (bind (_relativerotation_roll _relativerotation_pitch _relativerotation_yaw) (`KismetMathLibrary.BreakRotator` (`SceneComponent.RelativeRotation` (`self.Leg04`))))
  (bind (_relativerotation_roll_2 _relativerotation_pitch_2 _relativerotation_yaw_2) (`KismetMathLibrary.BreakRotator` (`SceneComponent.RelativeRotation` (`self.Leg01`))))
  (bind (_relativerotation_roll_3 _relativerotation_pitch_3 _relativerotation_yaw_3) (`KismetMathLibrary.BreakRotator` (`SceneComponent.RelativeRotation` (`self.Leg02`))))
  (bind (_relativerotation_roll_4 _relativerotation_pitch_4 _relativerotation_yaw_4) (`KismetMathLibrary.BreakRotator` (`SceneComponent.RelativeRotation` (`self.Leg03`))))
  (set `self.Leg1` _relativerotation_yaw_2)
  (set `self.Leg2` _relativerotation_yaw_3)
  (set `self.Leg3` _relativerotation_yaw_4)
  (set `self.Leg4` _relativerotation_yaw)
  (bind _outactors (`GameplayStatics.GetAllActorsOfClass` "/Game/NEW_Blueprints/NEW_Pawn.NEW_Pawn_C"))
  (set `self.Ref_Pawn` (`|GetArrayItem` _outactors))
  (bind _asgm_shooter (cast `/Game/INUSE/GM_Shooter` (`GameplayStatics.GetGameMode`)))
  (set `self.Ref_GM` _asgm_shooter))

(event `self.ReceiveTick`
  (params (DeltaSeconds :type "Float (single-precision)"))
  (`|ExecutionSequence`
    (:`then_0`
      _)
    (:`then_1`
      (`KismetSystemLibrary.Delay` 0.1)
      (`SceneComponent.K2_SetRelativeRotation` (`self.Leg01`) (`KismetMathLibrary.MakeRotator` 0.0 0.0 (+ (`KismetMathLibrary.RandomFloatInRange` -40.0 40.0) (`self.Leg1`))) false false)
      (`SceneComponent.K2_SetRelativeRotation` (`self.Leg02`) (`KismetMathLibrary.MakeRotator` 0.0 0.0 (+ (`KismetMathLibrary.RandomFloatInRange` -40.0 40.0) (`self.Leg2`))) false false)
      (`SceneComponent.K2_SetRelativeRotation` (`self.Leg03`) (`KismetMathLibrary.MakeRotator` 0.0 0.0 (+ (`KismetMathLibrary.RandomFloatInRange` -40.0 40.0) (`self.Leg3`))) false false)
      (`SceneComponent.K2_SetRelativeRotation` (`self.Leg04`) (`KismetMathLibrary.MakeRotator` 0.0 0.0 (+ (`KismetMathLibrary.RandomFloatInRange` -40.0 40.0) (`self.Leg4`))) false false)))
  (if (`self.Count_Down`)
    (`ActorComponent.Deactivate` (`self.CharacterMovement`))
    (`KismetSystemLibrary.Delay` 1.0)
    (if (`self.Count_Down`)
      (`self.Bomb Die`))
    (else
      (`ActorComponent.Activate` (`self.CharacterMovement`) false))))

(event `self.RangeSphere.OnComponentBeginOverlap`
  (params (OverlappedComponent :type "PrimitiveComponent Object Reference") (OtherActor :type "Actor Object Reference") (OtherComp :type "PrimitiveComponent Object Reference") (OtherBodyIndex :type Integer) (bFromSweep :type Boolean) (SweepResult :type "HitResult Structure (by ref)"))
  ;[1 1 1] Add Actors to Range of Explosion / Ignore Self
  (if (not (== OtherActor self))
    (cast `/Game/NEW_Blueprints/NEW_Pawn` OtherActor
      (:`then`
        (`|ExecutionSequence`
          (:`then_0`
            ;[1 1 1] Pawn Enters Range of Explosion / Activate Count Down
            (set `self.Count_Down` true)
            (bind _returnvalue (`PrimitiveComponent.CreateDynamicMaterialInstance` (`self.SM_Light`) 0 "/Game/NEW/Material__3.Material__3" "None"))
            (`MaterialInstanceDynamic.SetScalarParameterValue` _returnvalue "Frequency" 0.3))
          (:`then_1`
            (`KismetArrayLibrary.Array_Add` (`self.In_Range`) OtherActor :!label _label))))
      (:`CastFailed`
        (goto _label)))))

(event `self.RangeSphere.OnComponentEndOverlap`
  (params (OverlappedComponent :type "PrimitiveComponent Object Reference") (OtherActor :type "Actor Object Reference") (OtherComp :type "PrimitiveComponent Object Reference") (OtherBodyIndex :type Integer))
  ;[1 1 1] Remove Actors from Range of Explosion
  (cast `/Game/NEW_Blueprints/NEW_Pawn` OtherActor
    (:`then`
      (`|ExecutionSequence`
        (:`then_0`
          ;[1 1 1] Pawn Exit Range of Explosion  / Deactivate Count Down
          (set `self.Count_Down` false)
          (bind _returnvalue (`PrimitiveComponent.CreateDynamicMaterialInstance` (`self.SM_Light`) 0 "/Game/NEW/Material__3.Material__3" "None"))
          (`MaterialInstanceDynamic.SetScalarParameterValue` _returnvalue "Frequency" 0.6))
        (:`then_1`
          (`KismetArrayLibrary.Array_RemoveItem` (`self.In_Range`) OtherActor :!label _label_2))))
    (:`CastFailed`
      (goto _label_2))))

(event `self.Collision.OnComponentBeginOverlap`
  (params (OverlappedComponent :type "PrimitiveComponent Object Reference") (OtherActor :type "Actor Object Reference") (OtherComp :type "PrimitiveComponent Object Reference") (OtherBodyIndex :type Integer) (bFromSweep :type Boolean) (SweepResult :type "HitResult Structure (by ref)"))
  ;[1 1 1] Kill Pawn by Proximity
  (bind _asnew_pawn (cast `/Game/NEW_Blueprints/NEW_Pawn` OtherActor))
  (`KismetSystemLibrary.Delay` 0.2)
  (`/Engine/EditorBlueprintResources/StandardMacros.IsValid` _asnew_pawn
    (:`Is Valid`
      (`/Game/NEW_Blueprints/NEW_Pawn.PawnDie` _asnew_pawn))))

(event `Bomb Die`
  (bind _torsoo (`self.Torsoo`))
  (bind (_returnvalue_x _returnvalue_y _returnvalue_z) (`KismetMathLibrary.BreakVector` (`SceneComponent.K2_GetComponentLocation` _torsoo)))
  (bind (_returnvalue_roll _returnvalue_pitch _returnvalue_yaw) (`KismetMathLibrary.BreakRotator` (`SceneComponent.K2_GetComponentRotation` _torsoo)))
  (`/Engine/EditorBlueprintResources/StandardMacros.DoOnce` false :!label _label_3
    (:`Completed`
      ;[1 1 1] Bomb DIe
      (bind _outactors (`GameplayStatics.GetAllActorsOfClass` "/Game/INUSE/BP_AreaSpawn.BP_AreaSpawn_C"))
      (`/Game/INUSE/BP_AreaSpawn.AnotherBomb` (`|GetArrayItem` _outactors))
      (`GameplayStatics.SpawnEmitterAtLocation` "/Game/Particles/P_Exp_Bomb.P_Exp_Bomb" (`SceneComponent.K2_GetComponentLocation` (`self.SM_Bomb`)) (struct) (2.0 2.0 1.0))
      (`|SpawnActorFromClass` "/Game/NEW_Blueprints/NEW_Blood_Bomb.NEW_Blood_Bomb_C" (`KismetMathLibrary.MakeTransform` (`KismetMathLibrary.MakeVector` _returnvalue_x _returnvalue_y (- _returnvalue_z 20.0)) (`KismetMathLibrary.MakeRotator` _returnvalue_roll _returnvalue_pitch (+ _returnvalue_yaw 90.0)) (2.0 2.0 1.0)) "Undefined" "OverrideRootScale" null null)
      (`GameplayStatics.PlaySound2D` "/Game/Audio/DeathAlien.DeathAlien" 1.0 1.0 0.0 null null)
      ;[1 1 1] Destroy Everything in Range
      (for _array_element (`self.In_Range`)
        (bind _asbp_slow_ia (cast `/Game/Blueprints/Bichos/BP_Slow_IA` _array_element)
          (:`then`
            (set `/Game/Blueprints/Bichos/BP_Slow_IA.Vida` (- (`/Game/Blueprints/Bichos/BP_Slow_IA.Vida` _asbp_slow_ia) (`self.DamageToAllies`)) _asbp_slow_ia))
          (:`CastFailed`
            (bind _asbp_bomb_ia (cast `/Game/Blueprints/Bichos/BP_Bomb_IA` _array_element)
              (:`then`
                (`self.Bomb Die` _asbp_bomb_ia))
              (:`CastFailed`
                (bind _asbp_dash_blue_ia (cast `/Game/Blueprints/Bichos/BP_Dash_Blue_IA` _array_element)
                  (:`then`
                    (set `/Game/Blueprints/Bichos/BP_Dash_Blue_IA.Vida` (- (`/Game/Blueprints/Bichos/BP_Dash_Blue_IA.Vida` _asbp_dash_blue_ia) (`self.DamageToAllies`)) _asbp_dash_blue_ia))
                  (:`CastFailed`
                    (bind _asnew_pawn (cast `/Game/NEW_Blueprints/NEW_Pawn` _array_element))
                    (`/Game/NEW_Blueprints/NEW_Pawn.PawnDie` _asnew_pawn))))))))
      (if (`/Game/INUSE/GM_Shooter.SoundOn?` (`self.Ref_GM`))
        (`GameplayStatics.PlaySound2D` "/Game/Audio/Explosion_Cue.Explosion_Cue" 1.0 1.0 0.0 null null)
        (`GameplayStatics.PlaySound2D` "/Game/Audio/Growl_Bomb.Growl_Bomb" 1.0 1.0 0.0 null null))
      (`self.K2_DestroyActor`))))

(event `self.Torsoo.OnComponentHit`
  (params (HitComponent :type "PrimitiveComponent Object Reference") (OtherActor :type "Actor Object Reference") (OtherComp :type "PrimitiveComponent Object Reference") (NormalImpulse :type "Vector Structure") (Hit :type "HitResult Structure (by ref)"))
  (cast `/Game/NEW_Blueprints/NEW_Balas` OtherActor
    (:`then`
      _)
    (:`CastFailed`
      (cast `/Game/INUSE/BP_BalasElectricaArma` OtherActor)))
  ;[1 1 1] Got Shot
  (set `self.Vida` (- (`self.Vida`) (`self.DamageRecibido`)))
  (goto _label_3))

(event `self.CapsuleComponent.OnComponentHit`
  (params (HitComponent :type "PrimitiveComponent Object Reference") (OtherActor :type "Actor Object Reference") (OtherComp :type "PrimitiveComponent Object Reference") (NormalImpulse :type "Vector Structure") (Hit :type "HitResult Structure (by ref)")))

(fn `UserConstructionScript`)