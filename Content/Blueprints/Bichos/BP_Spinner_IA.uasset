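; BP_Spinner_IA is an enemy with a constantly spinning torso that kills on contact: the player pawn after a short delay, Slow and Bomb enemies immediately.
; Bullet hits and the danorayo event subtract the player's Damage, cached at BeginPlay, from Vida and briefly flash a particle effect.
; At zero Vida, or via SlowDie, a one-time death calls AnotherSlow on the area spawner, spawns blood and an explosion, then destroys the actor.
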(event `self.ReceiveBeginPlay`
  (bind _outactors (`GameplayStatics.GetAllActorsOfClass` "/Game/NEW_Blueprints/NEW_Pawn.NEW_Pawn_C"))
  (bind _output_get (set `self.Ref_Pawn` (`|GetArrayItem` _outactors)))
  (set `self.DamageRecibido` (`/Game/NEW_Blueprints/NEW_Pawn.Damage` _output_get)))

(event `self.ReceiveTick`
  (params (DeltaSeconds :type "Float (single-precision)"))
  (bind (_returnvalue_roll _returnvalue_pitch _returnvalue_yaw) (`KismetMathLibrary.BreakRotator` (`SceneComponent.K2_GetComponentRotation` (`self.Torso`))))
  (`SceneComponent.K2_SetWorldRotation` (`self.Torso`) (`KismetMathLibrary.MakeRotator` _returnvalue_roll _returnvalue_pitch (+ 3.0 _returnvalue_yaw)) false false))

(event `self.collision.OnComponentBeginOverlap`
  (params (OverlappedComponent :type "PrimitiveComponent Object Reference") (OtherActor :type "Actor Object Reference") (OtherComp :type "PrimitiveComponent Object Reference") (OtherBodyIndex :type Integer) (bFromSweep :type Boolean) (SweepResult :type "HitResult Structure (by ref)"))
  ;[1 1 1] Kill Pawn by Proximity
  (`|ExecutionSequence`
    (:`then_0`
      (bind _asnew_pawn (cast `/Game/NEW_Blueprints/NEW_Pawn` OtherActor))
      (`KismetSystemLibrary.Delay` 0.2)
      (`/Engine/EditorBlueprintResources/StandardMacros.IsValid` _asnew_pawn
        (:`Is Valid`
          (`/Game/NEW_Blueprints/NEW_Pawn.PawnDie` _asnew_pawn))))
    (:`then_1`
      (bind _asbp_slow_ia (cast `/Game/Blueprints/Bichos/BP_Slow_IA` OtherActor))
      (`/Game/Blueprints/Bichos/BP_Slow_IA.SlowDie` _asbp_slow_ia))
    (:`then_2`
      (bind _asbp_bomb_ia (cast `/Game/Blueprints/Bichos/BP_Bomb_IA` OtherActor))
      (`/Game/Blueprints/Bichos/BP_Bomb_IA.Bomb Die` _asbp_bomb_ia))))

(event `danorayo`
  (bind _particlesystem (`self.ParticleSystem`))
  (bind _torso (`self.Torso`))
  (bind (_returnvalue_x _returnvalue_y _returnvalue_z) (`KismetMathLibrary.BreakVector` (`SceneComponent.K2_GetComponentLocation` _torso)))
  (bind (_returnvalue_roll _returnvalue_pitch _returnvalue_yaw) (`KismetMathLibrary.BreakRotator` (`SceneComponent.K2_GetComponentRotation` _torso)))
  (bind _output_get (set `self.Vida` (- (`self.Vida`) (`self.DamageRecibido`)) :!label _label))
  (`|ExecutionSequence`
    (:`then_0`
      _)
    (:`then_1`
      (`/Engine/EditorBlueprintResources/StandardMacros.IsValid` _particlesystem
        (:`Is Valid`
          (`ActorComponent.Activate` _particlesystem false)
          (`KismetSystemLibrary.Delay` 1.5)
          (`ActorComponent.Deactivate` _particlesystem)))))
  (if (<= _output_get 0)
    (`/Engine/EditorBlueprintResources/StandardMacros.DoOnce` false :!label _label_2
      (:`Completed`
        ;[1 1 1] Slow Die
        (bind _outactors (`GameplayStatics.GetAllActorsOfClass` "/Game/INUSE/BP_AreaSpawn.BP_AreaSpawn_C"))
        (`/Game/INUSE/BP_AreaSpawn.Another Slow` (`|GetArrayItem` _outactors))
        (`|SpawnActorFromClass` "/Game/NEW_Blueprints/NEW_Blood.NEW_Blood_C" (`KismetMathLibrary.MakeTransform` (`KismetMathLibrary.MakeVector` _returnvalue_x _returnvalue_y (- _returnvalue_z 20.0)) (`KismetMathLibrary.MakeRotator` _returnvalue_roll _returnvalue_pitch (+ _returnvalue_yaw 90.0)) (1.3 1.3 1.0)) "Undefined" "OverrideRootScale" null null)
        (`GameplayStatics.SpawnEmitterAtLocation` "/Game/Particles/P_Exp_Shot.P_Exp_Shot" (`SceneComponent.K2_GetComponentLocation` _torso))
        (`self.K2_DestroyActor`)))))

(event `SlowDie`
  (goto _label_2))

(event `self.collision.OnComponentHit`
  (params (HitComponent :type "PrimitiveComponent Object Reference") (OtherActor :type "Actor Object Reference") (OtherComp :type "PrimitiveComponent Object Reference") (NormalImpulse :type "Vector Structure") (Hit :type "HitResult Structure (by ref)"))
  ;[1 1 1] Got Shot
  (`|ExecutionSequence`
    (:`then_0`
      (cast `/Game/NEW_Blueprints/NEW_Balas` OtherActor)
      (goto _label))
    (:`then_1`
      (cast `/Game/INUSE/BP_BalasElectricaArma` OtherActor)
      (goto _label))))

(fn `UserConstructionScript`)