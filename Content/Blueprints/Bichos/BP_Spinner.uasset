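; BP_Spinner is an enemy that chases the player's NEW_Pawn and kills it on collision overlap.
; Tick steers the Torso toward the pawn with random jitter, and a delayed DoOnce starts Timeline-driven spins that pause movement and reset afterward.
; NEW_Balas hits reduce Vida only outside spins; death notifies BP_AreaSpawn, spawns blood and explosion effects, then destroys the actor.
; Projectile-spawning logic is present but never runs.
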(event `self.ReceiveBeginPlay`
  (bind _outactors (`GameplayStatics.GetAllActorsOfClass` "/Game/NEW_Blueprints/NEW_Pawn.NEW_Pawn_C"))
  (set `self.Ref_Pawn` (`|GetArrayItem` _outactors)))

(event `self.ReceiveTick`
  (params (DeltaSeconds :type "Float (single-precision)"))
  (bind _sm_torso (`/Game/NEW_Blueprints/NEW_Pawn.SM_Torso` (`self.Ref_Pawn`)))
  (bind _returnvalue (- (`SceneComponent.K2_GetComponentLocation` _sm_torso) (`SceneComponent.K2_GetComponentLocation` (`self.Torso`))))
  (bind (_returnvalue_x _returnvalue_y) (`KismetMathLibrary.BreakVector` (* (`KismetMathLibrary.Normal` _returnvalue) (`self.MovementSpeed`))))
  (bind (_returnvalue_roll _returnvalue_pitch _returnvalue_yaw) (`KismetMathLibrary.BreakRotator` (`KismetMathLibrary.Conv_VectorToRotator` (* _returnvalue DeltaSeconds))))
  (`|ExecutionSequence`
    (:`then_0`
      ;[1 1 1] Movement and Rotation
      (`/Engine/EditorBlueprintResources/StandardMacros.IsValid` _sm_torso
        (:`Is Valid`
          (if (not (`self.Spinning`))
            (`SceneComponent.K2_SetWorldRotation` (`self.Torso`) (`KismetMathLibrary.MakeRotator` 0.0 0.0 (+ _returnvalue_yaw (`KismetMathLibrary.RandomFloatInRange` -3.0 3.0))) false false)
            (`SceneComponent.K2_AddRelativeLocation` (`self.Torso`) (`KismetMathLibrary.MakeVector` (+ _returnvalue_x (`KismetMathLibrary.RandomFloatInRange` -3.0 3.0)) (+ _returnvalue_y (`KismetMathLibrary.RandomFloatInRange` -3.0 3.0))) false false)
            (`KismetSystemLibrary.Delay` 2.0)
            (`/Engine/EditorBlueprintResources/StandardMacros.DoOnce` false :!label _label
              (:`Completed`
                (set `self.Spinning` true)
                (bind (_direction _newtrack_0) (`Timeline|Timeline_0` :!via `PlayFromStart`)
                  (:`Update`
                    (`SceneComponent.K2_SetRelativeRotation` (`self.Torso`) (`KismetMathLibrary.MakeRotator` 0.0 0.0 (+ _newtrack_0 (`KismetMathLibrary.RandomFloatInRange` -3.0 3.0))) false false))
                  (:`Finished`
                    (`self.ResetSpin`)))))))))))

(event `ResetSpin`
  (set `self.Spinning` false)
  (goto _label :!via `Reset`))

(event `self.Collision.OnComponentBeginOverlap`
  (params (OverlappedComponent :type "PrimitiveComponent Object Reference") (OtherActor :type "Actor Object Reference") (OtherComp :type "PrimitiveComponent Object Reference") (OtherBodyIndex :type Integer) (bFromSweep :type Boolean) (SweepResult :type "HitResult Structure (by ref)"))
  ;[1 1 1] Kill Pawn by Proximity
  (bind _asnew_pawn (cast `/Game/NEW_Blueprints/NEW_Pawn` OtherActor))
  (`/Game/NEW_Blueprints/NEW_Pawn.PawnDie` _asnew_pawn))

(event `SlowDie`
  (bind _torso (`self.Torso`))
  (bind _returnvalue (`SceneComponent.K2_GetComponentLocation` _torso))
  (bind (_returnvalue_roll _returnvalue_pitch _returnvalue_yaw) (`KismetMathLibrary.BreakRotator` (`SceneComponent.K2_GetComponentRotation` _torso)))
  (`/Engine/EditorBlueprintResources/StandardMacros.DoOnce` false :!label _label_2
    (:`Completed`
      ;[1 1 1] Slow Die
      (bind _outactors (`GameplayStatics.GetAllActorsOfClass` "/Game/INUSE/BP_AreaSpawn.BP_AreaSpawn_C"))
      (`/Game/INUSE/BP_AreaSpawn.Another Slow` (`|GetArrayItem` _outactors))
      (`|SpawnActorFromClass` "/Game/NEW_Blueprints/NEW_Blood.NEW_Blood_C" (`KismetMathLibrary.MakeTransform` _returnvalue (`KismetMathLibrary.MakeRotator` _returnvalue_roll _returnvalue_pitch (+ _returnvalue_yaw 90.0)) (1.3 1.3 1.0)) "Undefined" "OverrideRootScale" null null)
      (`GameplayStatics.SpawnEmitterAtLocation` "/Game/Particles/P_Exp_Shot.P_Exp_Shot" _returnvalue)
      (`self.K2_DestroyActor`))))

(event `self.Torso.OnComponentHit`
  (params (HitComponent :type "PrimitiveComponent Object Reference") (OtherActor :type "Actor Object Reference") (OtherComp :type "PrimitiveComponent Object Reference") (NormalImpulse :type "Vector Structure") (Hit :type "HitResult Structure (by ref)"))
  ;[1 1 1] Got Shot
  (cast `/Game/NEW_Blueprints/NEW_Balas` OtherActor)
  (if (not (`self.Spinning`))
    (bind _result (`/Engine/EditorBlueprintResources/StandardMacros.DecrementInt` (`self.Vida`))
      (:`  `
        (bind _output_get (set `self.Vida` _result))
        (if (<= _output_get 0)
          (goto _label_2))))))

(fn `UserConstructionScript`)