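; Giant boss enemy that animates its feet with a jittered timeline flip-flopped on Tick, and kills the player pawn shortly after contact.
; Bullet overlaps and the looping-timer lightning event (danorayo) subtract the pawn's damage, cached at BeginPlay, from Vida and briefly flash a particle.
; Death, also triggerable through BIgBossDie, fires BP_AreaSpawn's slow effect, spawns blood and explosion, notifies the pawn, clears BossSpawn and destroys the actor.
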(event `self.ReceiveTick`
  (params (DeltaSeconds :type "Float (single-precision)"))
  ;[1 1 1] movimiento del brazo.(velocidad del tick tocada del even tick)
  (`/Engine/EditorBlueprintResources/StandardMacros.FlipFlop`
    (:`A`
      (bind (_direction _elevation _stepiz _stepder) (`Timeline|Timeline_0` :!via `PlayFromStart` :!label _label)
        (:`Update`
          (bind _returnvalue (+ _elevation (`KismetMathLibrary.RandomFloatInRange` -0.5 0.5)))
          (`SceneComponent.K2_SetRelativeLocation` (`self.FeetDe`) (`KismetMathLibrary.MakeVector` (+ _stepder (`KismetMathLibrary.RandomFloatInRange` -0.5 0.5)) 14.0 _returnvalue) false false)
          (`SceneComponent.K2_SetRelativeLocation` (`self.FeetIz`) (`KismetMathLibrary.MakeVector` (+ _stepiz (`KismetMathLibrary.RandomFloatInRange` -0.5 0.5)) -14.0 _returnvalue) false false))))
    (:`B`
      (goto _label :!via `ReverseFromEnd`))))

(event `self.ReceiveBeginPlay`
  (bind _outactors (`GameplayStatics.GetAllActorsOfClass` "/Game/NEW_Blueprints/NEW_Pawn.NEW_Pawn_C"))
  (bind _output_get (set `self.Ref_Pawn` (`|GetArrayItem` _outactors)))
  (set `self.DamageRecibido` (`/Game/NEW_Blueprints/NEW_Pawn.Damage` _output_get)))

(event `danorayo`
  (bind _particlesystem (`self.ParticleSystem`))
  (bind _torso (`self.Torso`))
  (bind _torso_2 (`self.Torso`))
  (bind (_returnvalue_x _returnvalue_y _returnvalue_z) (`KismetMathLibrary.BreakVector` (`SceneComponent.K2_GetComponentLocation` _torso_2)))
  (bind (_returnvalue_roll _returnvalue_pitch _returnvalue_yaw) (`KismetMathLibrary.BreakRotator` (`SceneComponent.K2_GetComponentRotation` _torso_2)))
  (bind (_returnvalue_x_2 _returnvalue_y_2) (`KismetMathLibrary.BreakVector` (/ (`SceneComponent.K2_GetComponentScale` _torso) 3)))
  (`KismetSystemLibrary.K2_SetTimerDelegate` (delegate `danorayo`) 1.5 true)
  (bind _output_get (set `self.Vida` (- (`self.Vida`) (`self.DamageRecibido`)) :!label _label_2))
  (`|ExecutionSequence`
    (:`then_0`
      _)
    (:`then_1`
      (`/Engine/EditorBlueprintResources/StandardMacros.IsValid` _particlesystem
        (:`Is Valid`
          (`ActorComponent.Activate` _particlesystem false)
          (`KismetSystemLibrary.Delay` 1.5)
          (`ActorComponent.Deactivate` _particlesystem)))))
  (if (<= _output_get 0)
    (`/Engine/EditorBlueprintResources/StandardMacros.DoOnce` false :!label _label_3
      (:`Completed`
        ;[1 1 1] Slow Die
        (bind _outactors (`GameplayStatics.GetAllActorsOfClass` "/Game/INUSE/BP_AreaSpawn.BP_AreaSpawn_C"))
        (`/Game/INUSE/BP_AreaSpawn.Another Slow` (`|GetArrayItem` _outactors))
        (`|SpawnActorFromClass` "/Game/NEW_Blueprints/NEW_Blood.NEW_Blood_C" (`KismetMathLibrary.MakeTransform` (`KismetMathLibrary.MakeVector` _returnvalue_x _returnvalue_y (- _returnvalue_z 20.0)) (`KismetMathLibrary.MakeRotator` _returnvalue_roll _returnvalue_pitch (+ _returnvalue_yaw 90.0)) (1.3 1.3 1.0)) "Undefined" "OverrideRootScale" null null)
        (`GameplayStatics.SpawnEmitterAtLocation` "/Game/Particles/P_Exp_Boss.P_Exp_Boss" (`SceneComponent.K2_GetComponentLocation` _torso) (struct) (`KismetMathLibrary.MakeVector` _returnvalue_x_2 _returnvalue_y_2 0.1))
        (`/Game/NEW_Blueprints/NEW_Pawn.EVENT` (`self.Ref_Pawn`) "BP_Boss_giant_IA_C")
        (bind _outactors_2 (`GameplayStatics.GetAllActorsOfClass` "/Game/INUSE/BP_AreaSpawn.BP_AreaSpawn_C"))
        (set `/Game/INUSE/BP_AreaSpawn.BossSpawn` false (`|GetArrayItem` _outactors_2))
        (`self.K2_DestroyActor`)))))

(event `BIgBossDie`
  (goto _label_3))

(event `self.Collision.OnComponentBeginOverlap`
  (params (OverlappedComponent :type "PrimitiveComponent Object Reference") (OtherActor :type "Actor Object Reference") (OtherComp :type "PrimitiveComponent Object Reference") (OtherBodyIndex :type Integer) (bFromSweep :type Boolean) (SweepResult :type "HitResult Structure (by ref)"))
  ;[1 1 1] Got Shot
  (cast `/Game/NEW_Blueprints/NEW_Balas` OtherActor
    (:`then`
      (goto _label_2))
    (:`CastFailed`
      (cast `/Game/INUSE/BP_BalasElectricaArma` OtherActor
        (:`then`
          (goto _label_2))
        (:`CastFailed`
          ;[1 1 1] Kill Pawn by Proximity
          (bind _asnew_pawn (cast `/Game/NEW_Blueprints/NEW_Pawn` OtherActor))
          (`KismetSystemLibrary.Delay` 0.2)
          (`/Engine/EditorBlueprintResources/StandardMacros.IsValid` _asnew_pawn
            (:`Is Valid`
              (`/Game/NEW_Blueprints/NEW_Pawn.PawnDie` _asnew_pawn))))))))

(fn `UserConstructionScript`)