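; BP_Dash_Blue is an enemy that chases the player pawn, dashes at it and kills it on contact.
; Tick moves and rotates the Torso toward the pawn, or toward DashPoint once DashCube overlap triggers a brief pause and dash.
; Leaving DashCube or entering RangeSphere cancels the dash, and deactivating the Dash component spawns Humo.
; Bullet overlaps drain Vida; at zero it explodes, calls BP_AreaSpawn's AnotherDash and destroys itself.
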(event `self.ReceiveBeginPlay`
  (bind _outactors (`GameplayStatics.GetAllActorsOfClass` "/Game/NEW_Blueprints/NEW_Pawn.NEW_Pawn_C"))
  (set `self.Ref_Pawn` (`|GetArrayItem` _outactors)))

(event `self.ReceiveTick`
  (params (DeltaSeconds :type "Float (single-precision)"))
  (bind _ref_pawn (`self.Ref_Pawn`))
  (bind _returnvalue (- (`SceneComponent.K2_GetComponentLocation` (`/Game/NEW_Blueprints/NEW_Pawn.SM_Torso` _ref_pawn)) (`SceneComponent.K2_GetComponentLocation` (`self.Torso`))))
  ;[1 1 1] Movement and Rotation / Count down
  (if (`self.quieto`)
    (`/Engine/EditorBlueprintResources/StandardMacros.IsValid` _ref_pawn
      (:`Is Valid`
        (if (`self.Dashea`)
          (`SceneComponent.K2_SetWorldRotation` (`self.Torso`) (`KismetMathLibrary.Conv_VectorToRotator` (* (- (`SceneComponent.K2_GetComponentLocation` (`self.DashPoint`)) (`SceneComponent.K2_GetComponentLocation` (`self.Torso`))) DeltaSeconds)) false false)
          (else
            (`SceneComponent.K2_SetWorldRotation` (`self.Torso`) (`KismetMathLibrary.Conv_VectorToRotator` (* _returnvalue DeltaSeconds)) false false)))
        (if (`self.Count_Down`)
          (`SceneComponent.K2_AddRelativeLocation` (`self.Torso`) (* (`KismetMathLibrary.Normal` (- (`SceneComponent.K2_GetComponentLocation` (`self.dashpoint`)) (`SceneComponent.K2_GetComponentLocation` (`self.Torso`)))) 12) false true)
          (else
            (`SceneComponent.K2_AddRelativeLocation` (`self.Torso`) (* (`KismetMathLibrary.Normal` _returnvalue) (`self.MovementSpeed`)) true false)))))))

(event `self.DashCube.OnComponentBeginOverlap`
  (params (OverlappedComponent :type "PrimitiveComponent Object Reference") (OtherActor :type "Actor Object Reference") (OtherComp :type "PrimitiveComponent Object Reference") (OtherBodyIndex :type Integer) (bFromSweep :type Boolean) (SweepResult :type "HitResult Structure (by ref)"))
  ;[1 1 1] Add Actors to Range of Explosion / Ignore Self
  (cast `/Game/NEW_Blueprints/NEW_Pawn` OtherActor
    (:`then`
      (`|ExecutionSequence`
        (:`then_0`
          (set `self.Count_Down` true)
          (`ActorComponent.Activate` (`self.dash`) true)
          ;[1 1 1] quedarse quieto andes del dash
          (if (not (`self.Dashea`))
            (set `self.Dashea` true)
            (set `self.quieto` false)
            (`KismetSystemLibrary.Delay` 0.5)
            (set `self.quieto` true)))
        (:`then_1`
          (`KismetArrayLibrary.Array_Add` (`self.In_Range`) OtherActor :!label _label))))
    (:`CastFailed`
      (goto _label))))

(event `self.DashCube.OnComponentEndOverlap`
  (params (OverlappedComponent :type "PrimitiveComponent Object Reference") (OtherActor :type "Actor Object Reference") (OtherComp :type "PrimitiveComponent Object Reference") (OtherBodyIndex :type Integer))
  ;[1 1 1] Remove Actors from Range of Explosion
  ;[1 1 1] Pawn Exit Range of Explosion  / Deactivate Count Down
  (cast `/Game/NEW_Blueprints/NEW_Pawn` OtherActor)
  (set `self.Count_Down` false :!label _label_2)
  (set `self.Dashea` false)
  (`ActorComponent.Deactivate` (`self.dash`)))

(event `self.Range sphere.OnComponentBeginOverlap`
  (params (OverlappedComponent :type "PrimitiveComponent Object Reference") (OtherActor :type "Actor Object Reference") (OtherComp :type "PrimitiveComponent Object Reference") (OtherBodyIndex :type Integer) (bFromSweep :type Boolean) (SweepResult :type "HitResult Structure (by ref)"))
  ;[1 1 1] Remove Actors from Range of Explosion
  (cast `/Game/NEW_Blueprints/NEW_Pawn` OtherActor
    (:`then`
      (`|ExecutionSequence`
        (:`then_0`
          (goto _label_2))
        (:`then_1`
          _)))
    (:`CastFailed`
      _))
  (`KismetArrayLibrary.Array_RemoveItem` (`self.In_Range`) OtherActor))

(event `self.Collision.OnComponentBeginOverlap`
  (params (OverlappedComponent :type "PrimitiveComponent Object Reference") (OtherActor :type "Actor Object Reference") (OtherComp :type "PrimitiveComponent Object Reference") (OtherBodyIndex :type Integer) (bFromSweep :type Boolean) (SweepResult :type "HitResult Structure (by ref)"))
  ;[1 1 1] Kill Pawn by Proximity
  (bind _asnew_pawn (cast `/Game/NEW_Blueprints/NEW_Pawn` OtherActor))
  (`/Game/NEW_Blueprints/NEW_Pawn.PawnDie` _asnew_pawn))

(event `self.Torso.OnComponentBeginOverlap`
  (params (OverlappedComponent :type "PrimitiveComponent Object Reference") (OtherActor :type "Actor Object Reference") (OtherComp :type "PrimitiveComponent Object Reference") (OtherBodyIndex :type Integer) (bFromSweep :type Boolean) (SweepResult :type "HitResult Structure (by ref)"))
  ;[1 1 1] Got Shot
  (cast `/Game/NEW_Blueprints/NEW_Balas` OtherActor)
  (bind _result (`/Engine/EditorBlueprintResources/StandardMacros.DecrementInt` (`self.Vida`))
    (:`  `
      (bind _output_get (set `self.Vida` _result))
      (if (<= _output_get 0)
        (`GameplayStatics.SpawnEmitterAtLocation` "/Game/Particles/P_Exp_Boss.P_Exp_Boss" (`SceneComponent.K2_GetComponentLocation` (`self.Torso`)))
        (bind _outactors (`GameplayStatics.GetAllActorsOfClass` "/Game/INUSE/BP_AreaSpawn.BP_AreaSpawn_C"))
        (`/Game/INUSE/BP_AreaSpawn.Another Dash` (`|GetArrayItem` _outactors))
        (`self.K2_DestroyActor`)))))

(event `self.dash.OnComponentDeactivated`
  (params (Component :type "ActorComponent Object Reference"))
  ;[1 1 1] spawn humo collision
  (`|SpawnActorFromClass` "/Game/INUSE/Humo.Humo_C" (`KismetMathLibrary.MakeTransform` (`SceneComponent.K2_GetComponentLocation` (`self.Arrow`)) (`KismetMathLibrary.Conv_VectorToRotator` (`SceneComponent.GetForwardVector` (`self.Arrow`)))) "Undefined" "OverrideRootScale" null null))

(fn `UserConstructionScript`)