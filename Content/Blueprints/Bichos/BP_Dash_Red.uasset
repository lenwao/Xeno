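; BP_Dash_Red is an enemy that chases the player pawn, kills it on contact and attacks with bursts of dashes.
; Entering Dash_Range switches Tick from homing to a delay-driven aim, lock and dash cycle.
; A timeline moves Torso along the locked direction with random jitter and splash spawns, returning to chase after three dashes.
; Bullet hits drain Vida; death spawns effects and calls AnotherDash on BP_AreaSpawn.
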(event `self.ReceiveBeginPlay`
  (bind _outactors (`GameplayStatics.GetAllActorsOfClass` "/Game/NEW_Blueprints/NEW_Pawn.NEW_Pawn_C"))
  (set `self.Ref_Pawn` (`|GetArrayItem` _outactors)))

(event `ResetDashes`
  (goto _label :!via `Reset`))

(event `self.ReceiveTick`
  (params (DeltaSeconds :type "Float (single-precision)"))
  (bind _returnvalue (- (`SceneComponent.K2_GetComponentLocation` (`/Game/NEW_Blueprints/NEW_Pawn.SM_Torso` (`self.Ref_Pawn`))) (`SceneComponent.K2_GetComponentLocation` (`self.Torso`))))
  (bind _returnvalue_2 (* (- (`SceneComponent.K2_GetComponentLocation` (`/Game/NEW_Blueprints/NEW_Pawn.SM_Torso` (`self.Ref_Pawn`))) (`SceneComponent.K2_GetComponentLocation` (`self.Torso`))) DeltaSeconds))
  (if (`self.Aim`)
    (if (`self.Dashea`)
      (`/Engine/EditorBlueprintResources/StandardMacros.DoOnce` false :!label _label
        (:`Completed`
          (bind (_direction _route) (`Timeline|Timeline_Dash` :!via `PlayFromStart`)
            (:`Update`
              (bind (_returnvalue_x _returnvalue_y) (`KismetMathLibrary.BreakVector` (* (`KismetMathLibrary.Normal` (`self.Locked_To_Pawn`)) (/ (`self.DashLength`) (`KismetMathLibrary.FTrunc` _route)))))
              (`SceneComponent.K2_AddRelativeLocation` (`self.Torso`) (`KismetMathLibrary.MakeVector` (+ _returnvalue_x (`KismetMathLibrary.RandomFloatInRange` -3.0 3.0)) (+ _returnvalue_y (`KismetMathLibrary.RandomFloatInRange` -3.0 3.0))) false false)
              (`|SpawnActorFromClass` "/Game/Blueprints/Sangre/BP_Dash_Splash.BP_Dash_Splash_C" (`KismetMathLibrary.Conv_VectorToTransform` (`SceneComponent.K2_GetComponentLocation` (`self.Torso`))) "DontSpawnIfColliding" "OverrideRootScale" self null))
            (:`Finished`
              (`KismetSystemLibrary.Delay` (`self.Delay_Post_Dash`))
              (set `self.Dashea` false)
              (bind _result (`/Engine/EditorBlueprintResources/StandardMacros.IncrementInt` (`self.#Times`))
                (:`  `
                  (bind _output_get (set `self.#Times` _result))
                  (if (>= _output_get 3)
                    (set `self.Aim` false)
                    (set `self.#Times` 0)
                    (`self.ResetAim`)
                    (`self.ResetDashes`)
                    (else
                      (`self.ResetDashes`)))))))))
      (elif (`self.Locked`)
        (`KismetSystemLibrary.Delay` (`self.Delay_Pre_Dash`))
        (set `self.Dashea` true)
        (set `self.Locked` false)
        (else
          (`SceneComponent.K2_SetWorldRotation` (`self.Torso`) (`KismetMathLibrary.Conv_VectorToRotator` _returnvalue_2) false false)
          (`KismetSystemLibrary.Delay` (`self.Aim_delay`))
          (set `self.Locked_To_Pawn` _returnvalue_2)
          (set `self.Locked` true))))
    (else
      (`SceneComponent.K2_SetWorldRotation` (`self.Torso`) (`KismetMathLibrary.Conv_VectorToRotator` (* _returnvalue DeltaSeconds)) false false)
      (`SceneComponent.K2_AddRelativeLocation` (`self.Torso`) (* (`KismetMathLibrary.Normal` _returnvalue) (`self.MovementSpeed`)) false false))))

(event `self.Dash_Range.OnComponentBeginOverlap`
  (params (OverlappedComponent :type "PrimitiveComponent Object Reference") (OtherActor :type "Actor Object Reference") (OtherComp :type "PrimitiveComponent Object Reference") (OtherBodyIndex :type Integer) (bFromSweep :type Boolean) (SweepResult :type "HitResult Structure (by ref)"))
  (cast `/Game/NEW_Blueprints/NEW_Pawn` OtherActor)
  (`/Engine/EditorBlueprintResources/StandardMacros.DoOnce` false :!label _label_2
    (:`Completed`
      (set `self.Aim` true))))

(event `ResetAim`
  (goto _label_2 :!via `Reset`))

(event `self.Collision.OnComponentBeginOverlap`
  (params (OverlappedComponent :type "PrimitiveComponent Object Reference") (OtherActor :type "Actor Object Reference") (OtherComp :type "PrimitiveComponent Object Reference") (OtherBodyIndex :type Integer) (bFromSweep :type Boolean) (SweepResult :type "HitResult Structure (by ref)"))
  ;[1 1 1] Kill Pawn by Proximity
  (bind _asnew_pawn (cast `/Game/NEW_Blueprints/NEW_Pawn` OtherActor))
  (`/Game/NEW_Blueprints/NEW_Pawn.PawnDie` _asnew_pawn))

(event `self.Torso.OnComponentHit`
  (params (HitComponent :type "PrimitiveComponent Object Reference") (OtherActor :type "Actor Object Reference") (OtherComp :type "PrimitiveComponent Object Reference") (NormalImpulse :type "Vector Structure") (Hit :type "HitResult Structure (by ref)"))
  (bind _returnvalue (`SceneComponent.K2_GetComponentLocation` (`self.Torso`)))
  ;[1 1 1] Got Shot
  (cast `/Game/NEW_Blueprints/NEW_Balas` OtherActor)
  (bind _result (`/Engine/EditorBlueprintResources/StandardMacros.DecrementInt` (`self.Vida`))
    (:`  `
      (bind _output_get (set `self.Vida` _result))
      (if (<= _output_get 0)
        (`GameplayStatics.SpawnEmitterAtLocation` "/Game/Particles/P_Exp_Boss.P_Exp_Boss" _returnvalue (struct) (1.6 1.6 1.0))
        (`|SpawnActorFromClass` "/Game/NEW_Blueprints/NEW_Blood.NEW_Blood_C" (`KismetMathLibrary.MakeTransform` _returnvalue (struct) (2.0 2.0 1.0)) "Undefined" "OverrideRootScale" null null)
        (bind _outactors (`GameplayStatics.GetAllActorsOfClass` "/Game/INUSE/BP_AreaSpawn.BP_AreaSpawn_C"))
        (`/Game/INUSE/BP_AreaSpawn.Another Dash` (`|GetArrayItem` _outactors))
        (`self.K2_DestroyActor`)))))

(fn `UserConstructionScript`)