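; Alien bomb enemy that turns to face the player, jitters its legs and explodes when shot or after a short proximity countdown.
; The player entering its range sphere halts movement and changes the light's blink frequency; leaving cancels the countdown.
; A once-only death asks BP_AreaSpawn for another bomb, spawns effects and kills tracked player, slow aliens and bombs, chaining explosions.
; Direct body contact kills the player.
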(event `self.ReceiveBeginPlay`
  (bind (_relativerotation_roll _relativerotation_pitch _relativerotation_yaw) (`KismetMathLibrary.BreakRotator` (`SceneComponent.RelativeRotation` (`self.SM_Bomb_Leg04`))))
  (bind (_relativerotation_roll_2 _relativerotation_pitch_2 _relativerotation_yaw_2) (`KismetMathLibrary.BreakRotator` (`SceneComponent.RelativeRotation` (`self.SM_Bomb_Leg01`))))
  (bind (_relativerotation_roll_3 _relativerotation_pitch_3 _relativerotation_yaw_3) (`KismetMathLibrary.BreakRotator` (`SceneComponent.RelativeRotation` (`self.SM_Bomb_Leg02`))))
  (bind (_relativerotation_roll_4 _relativerotation_pitch_4 _relativerotation_yaw_4) (`KismetMathLibrary.BreakRotator` (`SceneComponent.RelativeRotation` (`self.SM_Bomb_Leg03`))))
  (set `self.Leg1` _relativerotation_yaw_2)
  (set `self.Leg2` _relativerotation_yaw_3)
  (set `self.Leg3` _relativerotation_yaw_4)
  (set `self.Leg4` _relativerotation_yaw)
  (bind _outactors (`GameplayStatics.GetAllActorsOfClass` "/Game/Blueprints/Pawn/NEW_Pawn.NEW_Pawn_C"))
  (set `self.Ref_Pawn` (`|GetArrayItem` _outactors))
  (bind _asgm_shooter (cast `/Game/Blueprints/GM_Shooter` (`GameplayStatics.GetGameMode`)))
  (set `self.Ref_GM` _asgm_shooter))

(event `self.ReceiveTick`
  (params (DeltaSeconds :type "Float (single-precision)"))
  (bind (_returnvalue_roll _returnvalue_pitch _returnvalue_yaw) (`KismetMathLibrary.BreakRotator` (`KismetMathLibrary.FindLookAtRotation` (`SceneComponent.K2_GetComponentLocation` (`self.CapsuleComponent`)) (`SceneComponent.K2_GetComponentLocation` (`Actor.RootComponent` (`GameplayStatics.GetPlayerPawn` 0))))))
  (`/Engine/EditorBlueprintResources/StandardMacros.IsValid` self
    (:`Is Valid`
      (`SceneComponent.K2_SetWorldRotation` (`self.CapsuleComponent`) (`KismetMathLibrary.MakeRotator` 0.0 0.0 _returnvalue_yaw) false false)
      (if (`self.Count_Down`)
        (`ActorComponent.Deactivate` (`self.CharacterMovement`))
        (`KismetSystemLibrary.Delay` 1.0)
        (if (`self.Count_Down`)
          (`self.Bomb Die`))
        (else
          (`ActorComponent.Activate` (`self.CharacterMovement`) false)
          (`SceneComponent.K2_SetRelativeRotation` (`self.SM_Bomb_Leg01`) (`KismetMathLibrary.MakeRotator` 0.0 0.0 (+ (`KismetMathLibrary.RandomFloatInRange` -40.0 40.0) (`self.Leg1`))) false false)
          (`SceneComponent.K2_SetRelativeRotation` (`self.SM_Bomb_Leg02`) (`KismetMathLibrary.MakeRotator` 0.0 0.0 (+ (`KismetMathLibrary.RandomFloatInRange` -40.0 40.0) (`self.Leg2`))) false false)
          (`SceneComponent.K2_SetRelativeRotation` (`self.SM_Bomb_Leg03`) (`KismetMathLibrary.MakeRotator` 0.0 0.0 (+ (`KismetMathLibrary.RandomFloatInRange` -40.0 40.0) (`self.Leg3`))) false false)
          (`SceneComponent.K2_SetRelativeRotation` (`self.SM_Bomb_Leg04`) (`KismetMathLibrary.MakeRotator` 0.0 0.0 (+ (`KismetMathLibrary.RandomFloatInRange` -40.0 40.0) (`self.Leg4`))) false false))))))

(event `self.RangeSphere.OnComponentBeginOverlap`
  (params (OverlappedComponent :type "PrimitiveComponent Object Reference") (OtherActor :type "Actor Object Reference") (OtherComp :type "PrimitiveComponent Object Reference") (OtherBodyIndex :type Integer) (bFromSweep :type Boolean) (SweepResult :type "HitResult Structure (by ref)"))
  ;[1 1 1] Add Actors to Range of Explosion / Ignore Self
  (if (not (== OtherActor self))
    (cast `/Game/Blueprints/Pawn/NEW_Pawn` OtherActor
      (:`then`
        (`|ExecutionSequence`
          (:`then_0`
            ;[1 1 1] Pawn Enters Range of Explosion / Activate Count Down
            (set `self.Count_Down` true)
            (bind _returnvalue (`PrimitiveComponent.CreateDynamicMaterialInstance` (`self.SM_Bomb_Light`) 0 "/Game/Materials/NEW_M_Light.NEW_M_Light" "None"))
            (`MaterialInstanceDynamic.SetScalarParameterValue` _returnvalue "Frequency" 0.3))
          (:`then_1`
            (`KismetArrayLibrary.Array_Add` (`self.In_Range`) OtherActor :!label _label))))
      (:`CastFailed`
        (goto _label)))))

(event `self.RangeSphere.OnComponentEndOverlap`
  (params (OverlappedComponent :type "PrimitiveComponent Object Reference") (OtherActor :type "Actor Object Reference") (OtherComp :type "PrimitiveComponent Object Reference") (OtherBodyIndex :type Integer))
  ;[1 1 1] Remove Actors from Range of Explosion
  (cast `/Game/Blueprints/Pawn/NEW_Pawn` OtherActor
    (:`then`
      (`|ExecutionSequence`
        (:`then_0`
          ;[1 1 1] Pawn Exit Range of Explosion  / Deactivate Count Down
          (set `self.Count_Down` false)
          (bind _returnvalue (`PrimitiveComponent.CreateDynamicMaterialInstance` (`self.SM_Bomb_Light`) 0 "/Game/Materials/NEW_M_Light.NEW_M_Light" "None"))
          (`MaterialInstanceDynamic.SetScalarParameterValue` _returnvalue "Frequency" 0.6))
        (:`then_1`
          (`KismetArrayLibrary.Array_RemoveItem` (`self.In_Range`) OtherActor :!label _label_2))))
    (:`CastFailed`
      (goto _label_2))))

(event `Bomb Die`
  (bind _sm_bomb_torso (`self.SM_Bomb_Torso`))
  (bind (_returnvalue_x _returnvalue_y _returnvalue_z) (`KismetMathLibrary.BreakVector` (`SceneComponent.K2_GetComponentLocation` _sm_bomb_torso)))
  (bind (_returnvalue_roll _returnvalue_pitch _returnvalue_yaw) (`KismetMathLibrary.BreakRotator` (`SceneComponent.K2_GetComponentRotation` _sm_bomb_torso)))
  (`/Engine/EditorBlueprintResources/StandardMacros.DoOnce` false :!label _label_3
    (:`Completed`
      ;[1 1 1] Bomb DIe
      (bind _outactors (`GameplayStatics.GetAllActorsOfClass` "/Game/Blueprints/Pawn/BP_AreaSpawn.BP_AreaSpawn_C"))
      (`/Game/Blueprints/Pawn/BP_AreaSpawn.AnotherBomb` (`|GetArrayItem` _outactors))
      (`GameplayStatics.SpawnEmitterAtLocation` "/Game/Particles/P_Die_Bomb.P_Die_Bomb" (`SceneComponent.K2_GetComponentLocation` (`self.SM_Bomb_Torso`)) (struct) (2.0 2.0 1.0))
      (`|SpawnActorFromClass` "/Game/Blueprints/Sangre/NEW_Blood_Bomb.NEW_Blood_Bomb_C" (`KismetMathLibrary.MakeTransform` (`KismetMathLibrary.MakeVector` _returnvalue_x _returnvalue_y _returnvalue_z) (`KismetMathLibrary.MakeRotator` _returnvalue_roll _returnvalue_pitch (+ _returnvalue_yaw 90.0)) (2.0 2.0 1.0)) "Undefined" "OverrideRootScale" null null)
      (if (`/Game/Blueprints/GM_Shooter.SoundOn?` (`self.Ref_GM`))
        (`GameplayStatics.PlaySound2D` "/Game/Audio/DeathAlien.DeathAlien" 1.0 1.0 0.0 null null))
      ;[1 1 1] Destroy Everything in Range
      (for _array_element (`self.In_Range`)
        (bind _asnew_slow_ia (cast `/Game/Blueprints/Aliens/NEW_Slow_IA` _array_element)
          (:`then`
            (`/Game/Blueprints/Aliens/NEW_Slow_IA.SlowDie` _asnew_slow_ia))
          (:`CastFailed`
            (bind _asnew_bomb_ia (cast `/Game/Blueprints/Aliens/NEW_Bomb_IA` _array_element)
              (:`then`
                (`self.Bomb Die` _asnew_bomb_ia))
              (:`CastFailed`
                (bind _asnew_pawn (cast `/Game/Blueprints/Pawn/NEW_Pawn` _array_element))
                (`/Game/Blueprints/Pawn/NEW_Pawn.PawnDie` _asnew_pawn (`KismetSystemLibrary.GetDisplayName` self)))))))
      (if (`/Game/Blueprints/GM_Shooter.SoundOn?` (`self.Ref_GM`))
        (`GameplayStatics.PlaySound2D` "/Game/Audio/Explosion_Cue.Explosion_Cue" 1.0 1.0 0.0 null null)
        (`GameplayStatics.PlaySound2D` "/Game/Audio/Growl_Bomb.Growl_Bomb" 1.0 1.0 0.0 null null))
      (`self.K2_DestroyActor`))))

(event `self.SM_Bomb_Collision.OnComponentBeginOverlap`
  (params (OverlappedComponent :type "PrimitiveComponent Object Reference") (OtherActor :type "Actor Object Reference") (OtherComp :type "PrimitiveComponent Object Reference") (OtherBodyIndex :type Integer) (bFromSweep :type Boolean) (SweepResult :type "HitResult Structure (by ref)"))
  (bind _asnew_balas (cast `/Game/Blueprints/Pawn/NEW_Balas` OtherActor)
    (:`then`
      (`/Game/Blueprints/Pawn/NEW_Balas.Hit` _asnew_balas)
      (goto _label_3))
    (:`CastFailed`
      (bind _asnew_pawn (cast `/Game/Blueprints/Pawn/NEW_Pawn` OtherActor))
      (`/Game/Blueprints/Pawn/NEW_Pawn.PawnDie` _asnew_pawn (`KismetSystemLibrary.GetDisplayName` self)))))

(fn `UserConstructionScript`)