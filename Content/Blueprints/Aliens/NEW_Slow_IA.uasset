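; Slow alien enemy that turns its capsule every tick to face the player and kills the player pawn on contact.
; Bullet overlaps on its collision mesh subtract health by the player's Damage value, cached at BeginPlay.
; At zero health, or via the SlowDie event, a one-shot death calls AnotherSlow on the area spawner, spawns blood and a particle effect, then destroys the actor.
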(event `self.ReceiveBeginPlay`
  (bind _outactors (`GameplayStatics.GetAllActorsOfClass` "/Game/Blueprints/Pawn/NEW_Pawn.NEW_Pawn_C"))
  (bind _output_get (set `self.Ref_Pawn` (`|GetArrayItem` _outactors)))
  (set `self.DamageRecibido` (`/Game/Blueprints/Pawn/NEW_Pawn.Damage` _output_get)))

(event `SlowDie`
  (bind _returnvalue (`SceneComponent.K2_GetComponentLocation` (`self.SM_Slow_Torso`)))
  (`/Engine/EditorBlueprintResources/StandardMacros.DoOnce` false :!label _label
    (:`Completed`
      (bind _outactors (`GameplayStatics.GetAllActorsOfClass` "/Game/Blueprints/Pawn/BP_AreaSpawn.BP_AreaSpawn_C"))
      (`/Game/Blueprints/Pawn/BP_AreaSpawn.Another Slow` (`|GetArrayItem` _outactors))
      (`|SpawnActorFromClass` "/Game/Blueprints/Sangre/NEW_Blood.NEW_Blood_C" (`KismetMathLibrary.MakeTransform` _returnvalue (struct) (1.2 1.2 1.0)) "Undefined" "OverrideRootScale" null null)
      (`GameplayStatics.SpawnEmitterAtLocation` "/Game/Particles/P_Die_Slow.P_Die_Slow" _returnvalue)
      (`self.K2_DestroyActor`))))

(event `self.SM_Collision.OnComponentBeginOverlap`
  (params (OverlappedComponent :type "PrimitiveComponent Object Reference") (OtherActor :type "Actor Object Reference") (OtherComp :type "PrimitiveComponent Object Reference") (OtherBodyIndex :type Integer) (bFromSweep :type Boolean) (SweepResult :type "HitResult Structure (by ref)"))
  (bind _asnew_balas (cast `/Game/Blueprints/Pawn/NEW_Balas` OtherActor)
    (:`then`
      (`/Game/Blueprints/Pawn/NEW_Balas.Hit` _asnew_balas)
      (bind _output_get (set `self.Vida` (- (`self.Vida`) (`self.DamageRecibido`))))
      (if (<= _output_get 0)
        (goto _label)))
    (:`CastFailed`
      (bind _asnew_pawn (cast `/Game/Blueprints/Pawn/NEW_Pawn` OtherActor))
      (`/Game/Blueprints/Pawn/NEW_Pawn.PawnDie` _asnew_pawn (`KismetSystemLibrary.GetDisplayName` self)))))

(event `self.ReceiveTick`
  (params (DeltaSeconds :type "Float (single-precision)"))
  (bind (_returnvalue_roll _returnvalue_pitch _returnvalue_yaw) (`KismetMathLibrary.BreakRotator` (`KismetMathLibrary.FindLookAtRotation` (`SceneComponent.K2_GetComponentLocation` (`self.CapsuleComponent`)) (`SceneComponent.K2_GetComponentLocation` (`Actor.RootComponent` (`GameplayStatics.GetPlayerPawn` 0))))))
  (`SceneComponent.K2_SetWorldRotation` (`self.CapsuleComponent`) (`KismetMathLibrary.MakeRotator` 0.0 0.0 _returnvalue_yaw) false false))

(fn `UserConstructionScript`)