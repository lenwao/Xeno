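; BP_Dash_Splash is a temporary blood splash left by a BP_Dash_Blue_IA dash that slows any NEW_Pawn inside it.
; On spawn it orients its plane from the owner's torso rotation with a yaw offset.
; A timeline drives the blood material's opacity, creating a new dynamic instance each update, then destroys the actor.
; The Ralentiza overlap sets pawn MovementSpeed to fixed values on entry and exit.
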(event `self.ReceiveBeginPlay`
  (bind _asbp_dash_blue_ia (cast `/Game/Blueprints/Bichos/BP_Dash_Blue_IA` (`self.GetOwner`)))
  (bind (_returnvalue_roll _returnvalue_pitch _returnvalue_yaw) (`KismetMathLibrary.BreakRotator` (`SceneComponent.K2_GetComponentRotation` (`/Game/Blueprints/Bichos/BP_Dash_Blue_IA.Torso` _asbp_dash_blue_ia))))
  (`SceneComponent.K2_SetWorldRotation` (`self.Plane`) (`KismetMathLibrary.MakeRotator` _returnvalue_roll _returnvalue_pitch (+ _returnvalue_yaw 90.0)) false false)
  (bind (_direction _newtrack_0) (`Timeline|TimFadeAway`)
    (:`Update`
      (bind _returnvalue (`PrimitiveComponent.CreateDynamicMaterialInstance` (`self.Plane`) 0 "/Game/Materials/M_Blood_Dash_Inst.M_Blood_Dash_Inst" "None"))
      (`MaterialInstanceDynamic.SetScalarParameterValue` _returnvalue "Opacity_Value" _newtrack_0))
    (:`Finished`
      (`self.K2_DestroyActor`))))

(event `self.Ralentiza.OnComponentBeginOverlap`
  (params (OverlappedComponent :type "PrimitiveComponent Object Reference") (OtherActor :type "Actor Object Reference") (OtherComp :type "PrimitiveComponent Object Reference") (OtherBodyIndex :type Integer) (bFromSweep :type Boolean) (SweepResult :type "HitResult Structure (by ref)"))
  (bind _asnew_pawn (cast `/Game/NEW_Blueprints/NEW_Pawn` OtherActor))
  (set `/Game/NEW_Blueprints/NEW_Pawn.MovementSpeed` 500.0 _asnew_pawn))

(event `self.Ralentiza.OnComponentEndOverlap`
  (params (OverlappedComponent :type "PrimitiveComponent Object Reference") (OtherActor :type "Actor Object Reference") (OtherComp :type "PrimitiveComponent Object Reference") (OtherBodyIndex :type Integer))
  (bind _asnew_pawn (cast `/Game/NEW_Blueprints/NEW_Pawn` OtherActor))
  (set `/Game/NEW_Blueprints/NEW_Pawn.MovementSpeed` 750.0 _asnew_pawn))

(fn `UserConstructionScript`)