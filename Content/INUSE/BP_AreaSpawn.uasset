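; Arena spawner that places Slow, Bomb and Dash enemies and timed bosses at random points inside its box areas.
; When game-mode time hits NextEventAtTime, and BossSpawn is clear, it plays a pulse and fading text, spawns a random actor or AI boss, and notifies NEW_Pawn.
; Overlaps with MURO-tagged components remove areas from the pool until they end.
; Spawns draw only from pool indices 0–3, re-rolling each lookup.
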(event `self.ReceiveBeginPlay`
  (bind _outactors (`GameplayStatics.GetAllActorsOfClass` "/Game/NEW_Blueprints/NEW_Pawn.NEW_Pawn_C"))
  (set `self.Ref_Pawn` (`|GetArrayItem` _outactors))
  (bind _asgm_shooter (cast `/Game/INUSE/GM_Shooter` (`GameplayStatics.GetGameMode`)))
  (set `self.Ref_GM` _asgm_shooter)
  (set `self.AreasPool` (`|MakeArray` (`self.Area`) (`self.Area3`) (`self.Area4`) (`self.Area2`) (`self.Box`) (`self.Box1`) (`self.Box2`) (`self.Box3`) (`self.Box4`) (`self.Box5`) (`self.Box6`) (`self.Box7`))))

(event `Reset`
  (goto _label :!via `Reset`))

(event `self.ReceiveTick`
  (params (DeltaSeconds :type "Float (single-precision)"))
  (if (== (`/Game/INUSE/GM_Shooter.Time` (`self.Ref_GM`)) (`self.NextEventAtTime`))
    (`/Engine/EditorBlueprintResources/StandardMacros.DoOnce` false :!label _label
      (:`Completed`
        (if (`self.BossSpawn`)
          (`KismetSystemLibrary.PrintString` "No se ha matado al anterior Boss")
          (else
            (set `self.BossSpawn` true)
            (`self.NewEvent`)))))))

(event `Pulse`
  (bind _pulseplane (`self.PulsePlane`))
  (bind (_returnvalue_x _returnvalue_y _returnvalue_z) (`KismetMathLibrary.BreakVector` (`SceneComponent.K2_GetComponentScale` _pulseplane)))
  (`SceneComponent.SetVisibility` _pulseplane true false)
  (bind (_direction _x) (`Timeline|Timeline_0` :!via `PlayFromStart`)
    (:`Update`
      (`SceneComponent.SetWorldScale3D` _pulseplane (`KismetMathLibrary.MakeVector` _x _x _returnvalue_z)))
    (:`Finished`
      (`SceneComponent.SetVisibility` _pulseplane false false))))

(event `Training`
  (params (Boss :type "Actor Class Reference") (BossIA :type "Character Class Reference"))
  (bind _output (`|GetArrayItem` (`self.AreasPool`) (`KismetMathLibrary.RandomIntegerInRange` 0 3)))
  (bind _returnvalue (`KismetMathLibrary.RandomPointInBoundingBox` (`SceneComponent.K2_GetComponentLocation` _output) (`BoxComponent.BoxExtent` _output)))
  (`|ExecutionSequence`
    (:`then_0`
      (`AIBlueprintHelperLibrary.SpawnAIFromClass` BossIA "/Game/Blueprints/Bichos/IA/IAbichos.IAbichos" _returnvalue))
    (:`then_1`
      (`|SpawnActorFromClass` Boss (`KismetMathLibrary.Conv_VectorToTransform` _returnvalue) "Undefined" "OverrideRootScale" null null)))
  (`/Game/NEW_Blueprints/NEW_Pawn.EVENT` (`self.Ref_Pawn`) null))

(event `NewEvent`
  (bind _output (`|GetArrayItem` (`self.AreasPool`) (`KismetMathLibrary.RandomIntegerInRange` 0 3)))
  (bind _output_2 (`|GetArrayItem` (`self.Boss_List`) (`KismetMathLibrary.RandomIntegerInRange` 0 3)))
  (bind _output_3 (`|GetArrayItem` (`self.Boss_List_IA`) (`KismetMathLibrary.RandomIntegerInRange` 0 3)))
  (bind _returnvalue (`KismetMathLibrary.RandomPointInBoundingBox` (`SceneComponent.K2_GetComponentLocation` _output) (`BoxComponent.BoxExtent` _output)))
  (`TextRenderComponent.K2_SetText` (`self.TextRender`) (`KismetTextLibrary.Conv_IntToText` (`self.NextEventAtTime`)))
  (`self.Pulse`)
  (bind (_direction _opa) (`Timeline|OpacityTime` :!via `PlayFromStart`)
    (:`Update`
      (bind _returnvalue_2 (`PrimitiveComponent.CreateDynamicMaterialInstance` (`self.TextRender`) 0 null "None"))
      (`MaterialInstanceDynamic.SetScalarParameterValue` _returnvalue_2 "Opa" _opa))
    (:`Finished`
      (set `self.NextEventAtTime` (+ (`self.NextEventAtTime`) 25))
      (`/Engine/EditorBlueprintResources/StandardMacros.IsValid` _output
        (:`Is Valid`
          (if (== (`KismetMathLibrary.RandomIntegerInRange` 0 1) 0)
            (`|SpawnActorFromClass` _output_2 (`KismetMathLibrary.Conv_VectorToTransform` _returnvalue) "Undefined" "OverrideRootScale" null null)
            (`/Game/NEW_Blueprints/NEW_Pawn.EVENT` (`self.Ref_Pawn`) _output_2)
            (else
              (`AIBlueprintHelperLibrary.SpawnAIFromClass` _output_3 null _returnvalue)
              (`/Game/NEW_Blueprints/NEW_Pawn.EVENT` (`self.Ref_Pawn`) _output_3)))
          (`KismetSystemLibrary.Delay` 1.5)
          (`self.Reset`))))))

(event `StartSpawn`
  (bind _output (`|GetArrayItem` (`self.AreasPool`) (`KismetMathLibrary.RandomIntegerInRange` 0 3)))
  (bind _returnvalue (`KismetMathLibrary.RandomPointInBoundingBox` (`SceneComponent.K2_GetComponentLocation` _output) (`BoxComponent.BoxExtent` _output)))
  (`|ExecutionSequence`
    (:`then_0`
      (for _ (range (+ (`self.#Slow to Spawn`) 1))
        (`/Engine/EditorBlueprintResources/StandardMacros.IsValid` _output :!label _label_2
          (:`Is Valid`
            (`AIBlueprintHelperLibrary.SpawnAIFromClass` "/Game/NEW_Blueprints/NEW_Slow_IA.NEW_Slow_IA_C" "/Game/Blueprints/Bichos/IA/IAbichos.IAbichos" _returnvalue)))))
    (:`then_1`
      (for _ (range (+ (`self.#Bomb to Spawn`) 1))
        (`AIBlueprintHelperLibrary.SpawnAIFromClass` "/Game/NEW_Blueprints/NEW_Bomb_IA.NEW_Bomb_IA_C" "/Game/Blueprints/Bichos/IA/IAbichos.IAbichos" _returnvalue :!label _label_3)))
    (:`then_2`
      (`AIBlueprintHelperLibrary.SpawnAIFromClass` "/Game/Blueprints/Bichos/BP_Dash_Blue_IA.BP_Dash_Blue_IA_C" "/Game/Blueprints/Bichos/IA_Dash/DashBehaviorTree.DashBehaviorTree" _returnvalue :!label _label_4))))

(event `self.Area.OnComponentBeginOverlap`
  (params (OverlappedComponent :type "PrimitiveComponent Object Reference") (OtherActor :type "Actor Object Reference") (OtherComp :type "PrimitiveComponent Object Reference") (OtherBodyIndex :type Integer) (bFromSweep :type Boolean) (SweepResult :type "HitResult Structure (by ref)"))
  (`self.AreaRemover` (`self.Area`) OtherComp))

(event `self.Area.OnComponentEndOverlap`
  (params (OverlappedComponent :type "PrimitiveComponent Object Reference") (OtherActor :type "Actor Object Reference") (OtherComp :type "PrimitiveComponent Object Reference") (OtherBodyIndex :type Integer))
  (`self.AreaAdder` (`self.Area`) OtherComp))

(event `Another Slow`
  (goto _label_2))

(event `AnotherBomb`
  (goto _label_3))

(event `self.Area2.OnComponentEndOverlap`
  (params (OverlappedComponent :type "PrimitiveComponent Object Reference") (OtherActor :type "Actor Object Reference") (OtherComp :type "PrimitiveComponent Object Reference") (OtherBodyIndex :type Integer))
  (`self.AreaAdder` (`self.Area2`) OtherComp))

(event `self.Area2.OnComponentBeginOverlap`
  (params (OverlappedComponent :type "PrimitiveComponent Object Reference") (OtherActor :type "Actor Object Reference") (OtherComp :type "PrimitiveComponent Object Reference") (OtherBodyIndex :type Integer) (bFromSweep :type Boolean) (SweepResult :type "HitResult Structure (by ref)"))
  (`self.AreaRemover` (`self.Area2`) OtherComp))

(event `self.Area3.OnComponentEndOverlap`
  (params (OverlappedComponent :type "PrimitiveComponent Object Reference") (OtherActor :type "Actor Object Reference") (OtherComp :type "PrimitiveComponent Object Reference") (OtherBodyIndex :type Integer))
  (`self.AreaAdder` (`self.Area3`) OtherComp))

(event `self.Area3.OnComponentBeginOverlap`
  (params (OverlappedComponent :type "PrimitiveComponent Object Reference") (OtherActor :type "Actor Object Reference") (OtherComp :type "PrimitiveComponent Object Reference") (OtherBodyIndex :type Integer) (bFromSweep :type Boolean) (SweepResult :type "HitResult Structure (by ref)"))
  (`self.AreaRemover` (`self.Area3`) OtherComp))

(event `self.Area4.OnComponentEndOverlap`
  (params (OverlappedComponent :type "PrimitiveComponent Object Reference") (OtherActor :type "Actor Object Reference") (OtherComp :type "PrimitiveComponent Object Reference") (OtherBodyIndex :type Integer))
  (`self.AreaAdder` (`self.Area4`) OtherComp))

(event `self.Area4.OnComponentBeginOverlap`
  (params (OverlappedComponent :type "PrimitiveComponent Object Reference") (OtherActor :type "Actor Object Reference") (OtherComp :type "PrimitiveComponent Object Reference") (OtherBodyIndex :type Integer) (bFromSweep :type Boolean) (SweepResult :type "HitResult Structure (by ref)"))
  (`self.AreaRemover` (`self.Area4`) OtherComp))

(event `self.Box1.OnComponentEndOverlap`
  (params (OverlappedComponent :type "PrimitiveComponent Object Reference") (OtherActor :type "Actor Object Reference") (OtherComp :type "PrimitiveComponent Object Reference") (OtherBodyIndex :type Integer))
  (`self.AreaAdder` (`self.Box1`) OtherComp))

(event `Another Dash`
  (`/Engine/EditorBlueprintResources/StandardMacros.IsValid` (`|GetArrayItem` (`self.AreasPool`) (`KismetMathLibrary.RandomIntegerInRange` 0 3))
    (:`Is Valid`
      (goto _label_4))))

(event `self.Box2.OnComponentEndOverlap`
  (params (OverlappedComponent :type "PrimitiveComponent Object Reference") (OtherActor :type "Actor Object Reference") (OtherComp :type "PrimitiveComponent Object Reference") (OtherBodyIndex :type Integer))
  (`self.AreaAdder` (`self.Box2`) OtherComp))

(event `self.Box.OnComponentBeginOverlap`
  (params (OverlappedComponent :type "PrimitiveComponent Object Reference") (OtherActor :type "Actor Object Reference") (OtherComp :type "PrimitiveComponent Object Reference") (OtherBodyIndex :type Integer) (bFromSweep :type Boolean) (SweepResult :type "HitResult Structure (by ref)"))
  (`self.AreaRemover` (`self.Box`) OtherComp))

(event `self.Box3.OnComponentEndOverlap`
  (params (OverlappedComponent :type "PrimitiveComponent Object Reference") (OtherActor :type "Actor Object Reference") (OtherComp :type "PrimitiveComponent Object Reference") (OtherBodyIndex :type Integer))
  (`self.AreaAdder` (`self.Box3`) OtherComp))

(event `self.Box1.OnComponentBeginOverlap`
  (params (OverlappedComponent :type "PrimitiveComponent Object Reference") (OtherActor :type "Actor Object Reference") (OtherComp :type "PrimitiveComponent Object Reference") (OtherBodyIndex :type Integer) (bFromSweep :type Boolean) (SweepResult :type "HitResult Structure (by ref)"))
  (`self.AreaRemover` (`self.Box1`) OtherComp))

(event `self.Box4.OnComponentEndOverlap`
  (params (OverlappedComponent :type "PrimitiveComponent Object Reference") (OtherActor :type "Actor Object Reference") (OtherComp :type "PrimitiveComponent Object Reference") (OtherBodyIndex :type Integer))
  (`self.AreaAdder` (`self.Box4`) OtherComp))

(event `self.Box2.OnComponentBeginOverlap`
  (params (OverlappedComponent :type "PrimitiveComponent Object Reference") (OtherActor :type "Actor Object Reference") (OtherComp :type "PrimitiveComponent Object Reference") (OtherBodyIndex :type Integer) (bFromSweep :type Boolean) (SweepResult :type "HitResult Structure (by ref)"))
  (`self.AreaRemover` (`self.Box2`) OtherComp))

(event `self.Box5.OnComponentEndOverlap`
  (params (OverlappedComponent :type "PrimitiveComponent Object Reference") (OtherActor :type "Actor Object Reference") (OtherComp :type "PrimitiveComponent Object Reference") (OtherBodyIndex :type Integer))
  (`self.AreaAdder` (`self.Box5`) OtherComp))

(event `self.Box3.OnComponentBeginOverlap`
  (params (OverlappedComponent :type "PrimitiveComponent Object Reference") (OtherActor :type "Actor Object Reference") (OtherComp :type "PrimitiveComponent Object Reference") (OtherBodyIndex :type Integer) (bFromSweep :type Boolean) (SweepResult :type "HitResult Structure (by ref)"))
  (`self.AreaRemover` (`self.Box3`) OtherComp))

(event `self.Box6.OnComponentEndOverlap`
  (params (OverlappedComponent :type "PrimitiveComponent Object Reference") (OtherActor :type "Actor Object Reference") (OtherComp :type "PrimitiveComponent Object Reference") (OtherBodyIndex :type Integer))
  (`self.AreaAdder` (`self.Box6`) OtherComp))

(event `self.Box7.OnComponentEndOverlap`
  (params (OverlappedComponent :type "PrimitiveComponent Object Reference") (OtherActor :type "Actor Object Reference") (OtherComp :type "PrimitiveComponent Object Reference") (OtherBodyIndex :type Integer))
  (`self.AreaAdder` (`self.Box7`) OtherComp))

(event `self.Box4.OnComponentBeginOverlap`
  (params (OverlappedComponent :type "PrimitiveComponent Object Reference") (OtherActor :type "Actor Object Reference") (OtherComp :type "PrimitiveComponent Object Reference") (OtherBodyIndex :type Integer) (bFromSweep :type Boolean) (SweepResult :type "HitResult Structure (by ref)"))
  (`self.AreaRemover` (`self.Box4`) OtherComp))

(event `self.Box5.OnComponentBeginOverlap`
  (params (OverlappedComponent :type "PrimitiveComponent Object Reference") (OtherActor :type "Actor Object Reference") (OtherComp :type "PrimitiveComponent Object Reference") (OtherBodyIndex :type Integer) (bFromSweep :type Boolean) (SweepResult :type "HitResult Structure (by ref)"))
  (`self.AreaRemover` (`self.Box5`) OtherComp))

(event `self.Box6.OnComponentBeginOverlap`
  (params (OverlappedComponent :type "PrimitiveComponent Object Reference") (OtherActor :type "Actor Object Reference") (OtherComp :type "PrimitiveComponent Object Reference") (OtherBodyIndex :type Integer) (bFromSweep :type Boolean) (SweepResult :type "HitResult Structure (by ref)"))
  (`self.AreaRemover` (`self.Box6`) OtherComp))

(event `self.Box7.OnComponentBeginOverlap`
  (params (OverlappedComponent :type "PrimitiveComponent Object Reference") (OtherActor :type "Actor Object Reference") (OtherComp :type "PrimitiveComponent Object Reference") (OtherBodyIndex :type Integer) (bFromSweep :type Boolean) (SweepResult :type "HitResult Structure (by ref)"))
  (`self.AreaRemover` (`self.Box7`) OtherComp))

(fn `AreaAdder`
  (params (Item :type "BoxComponent Object Reference (by ref)") (Target :type "ActorComponent Object Reference"))
  (if (`ActorComponent.ComponentHasTag` Target "MURO")
    (`KismetArrayLibrary.Array_Add` (`self.AreasPool`) Item)
    (`KismetSystemLibrary.PrintString` "AreaAdded")))

(fn `AreaRemover`
  (params (Item :type "BoxComponent Object Reference (by ref)") (Target :type "ActorComponent Object Reference"))
  (if (`ActorComponent.ComponentHasTag` Target "MURO")
    (`KismetArrayLibrary.Array_RemoveItem` (`self.AreasPool`) Item)
    (`KismetSystemLibrary.PrintString` "AreaRemoved")))

(fn `UserConstructionScript`)