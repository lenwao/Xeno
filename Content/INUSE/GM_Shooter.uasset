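; Shooter game mode that runs the camera-driven menus, game start, timer and kill tallies.
; Menu events blend the view to tagged actors, then add the matching widget after a delay.
; StartGame possesses the NEW_Pawn found at BeginPlay, blends to it and sets its Start flag.
; Tick counts seconds through a Delay; EnemyDeath, noted as unused, tallies kills by type and requests another from BP_AreaSpawn.
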(event `GoToMenu`
  (bind _outactors (`GameplayStatics.GetAllActorsWithTag` "MAIN"))
  (`PlayerController.SetViewTargetWithBlend` (`GameplayStatics.GetPlayerController` 0) (`|GetArrayItem` _outactors) 1.0 "VTBlend_Cubic" 2.0 false)
  (`KismetSystemLibrary.Delay` 1.0)
  (bind _returnvalue (`|CreateWidget` "/Game/Blueprints/Widgets/Start.Start_C"))
  (`UserWidget.AddToViewport` _returnvalue 0))

(event `Advanced`
  (bind _outactors (`GameplayStatics.GetAllActorsWithTag` "ADVANCED"))
  (`PlayerController.SetViewTargetWithBlend` (`GameplayStatics.GetPlayerController` 0) (`|GetArrayItem` _outactors) 1.0 "VTBlend_Cubic" 2.0 false)
  (`KismetSystemLibrary.Delay` 1.0)
  (bind _returnvalue (`|CreateWidget` "/Game/Blueprints/Widgets/Test1.Test1_C"))
  (`UserWidget.AddToViewport` _returnvalue 0))

(event `Options`
  (bind _outactors (`GameplayStatics.GetAllActorsWithTag` "OPTIONS"))
  (`PlayerController.SetViewTargetWithBlend` (`GameplayStatics.GetPlayerController` 0) (`|GetArrayItem` _outactors) 1.0 "VTBlend_Cubic" 2.0 false)
  (`KismetSystemLibrary.Delay` 1.0)
  (bind _returnvalue (`|CreateWidget` "/Game/Blueprints/Widgets/Options1.Options1_C"))
  (`UserWidget.AddToViewport` _returnvalue 0))

(event `Start Game`
  (bind _returnvalue (`GameplayStatics.GetPlayerController` 0))
  (bind _ref_pawn (`self.Ref_Pawn`))
  (`Controller.Possess` _returnvalue _ref_pawn)
  (`PlayerController.SetViewTargetWithBlend` _returnvalue _ref_pawn 4.0 "VTBlend_EaseInOut" 1.0 false)
  (`KismetSystemLibrary.Delay` 4.0)
  (set `/Game/NEW_Blueprints/NEW_Pawn.Start` true _ref_pawn))

(event `self.ReceiveBeginPlay`
  (set `PlayerController.bShowMouseCursor` true (`GameplayStatics.GetPlayerController` 0))
  (bind _outactors (`GameplayStatics.GetAllActorsOfClass` "/Game/NEW_Blueprints/NEW_Pawn.NEW_Pawn_C"))
  (set `self.Ref_Pawn` (`|GetArrayItem` _outactors))
  (bind _returnvalue (`|CreateWidget` "/Game/Blueprints/Widgets/Start.Start_C"))
  (`UserWidget.AddToViewport` _returnvalue 0))

(event `self.ReceiveTick`
  (params (DeltaSeconds :type "Float (single-precision)"))
  (bind _time (`self.Time`))
  (if (`self.StartTimer`)
    (`KismetSystemLibrary.Delay` 1.0)
    (bind _result (`/Engine/EditorBlueprintResources/StandardMacros.IncrementInt` _time)
      (:`  `
        (set `self.Time` _result)
        (`KismetSystemLibrary.PrintString` (`KismetStringLibrary.Conv_IntToString` _time))))))

(event `EnemyDeath`
  (params (Type :type Name))
  ;[1 0 0.08212] NoSeUSA
  (if (== Type "Slow")
    (bind _result (`/Engine/EditorBlueprintResources/StandardMacros.IncrementInt` (`self.#SlowKill`))
      (:`  `
        (bind _output_get (set `self.#SlowKill` _result))
        (bind _outactors (`GameplayStatics.GetAllActorsOfClass` "/Game/INUSE/BP_AreaSpawn.BP_AreaSpawn_C"))
        (`/Game/INUSE/BP_AreaSpawn.Another Slow` (`|GetArrayItem` _outactors))))
    (elif (== Type "Bomb")
      (bind _result_2 (`/Engine/EditorBlueprintResources/StandardMacros.IncrementInt` (`self.#BombKill`))
        (:`  `
          (bind _output_get_2 (set `self.#BombKill` _result_2))
          (bind _outactors_2 (`GameplayStatics.GetAllActorsOfClass` "/Game/INUSE/BP_AreaSpawn.BP_AreaSpawn_C"))
          (`/Game/INUSE/BP_AreaSpawn.AnotherBomb` (`|GetArrayItem` _outactors_2))))
      (elif (== Type "Dash")
        (bind _result_3 (`/Engine/EditorBlueprintResources/StandardMacros.IncrementInt` (`self.#DashKill`))
          (:`  `
            (bind _output_get_3 (set `self.#DashKill` _result_3))
            (bind _outactors_3 (`GameplayStatics.GetAllActorsOfClass` "/Game/INUSE/BP_AreaSpawn.BP_AreaSpawn_C"))
            (`/Game/INUSE/BP_AreaSpawn.Another Dash` (`|GetArrayItem` _outactors_3))))))))

(fn `UserConstructionScript`)