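; Weapon pickup actor that gives NEW_Pawn one of six weapon types on overlap and destroys itself unless NoRandom is set.
; BeginPlay uses the preset type with NoRandom, otherwise rolls among the first three TypeArray entries, then colours the mesh by type.
; Overlap copies the indexed FireRate to the pawn, clears its equip flags, sets the matching one and briefly plays particles.
; NoRandom pickups re-arm afterwards for reuse.
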(event `self.ReceiveBeginPlay`
  (bind _typeselected (`self.TypeSelected`))
  (bind _typeselected_2 (`self.TypeSelected`))
  (`/Engine/EditorBlueprintResources/StandardMacros.DoOnce` false
    (:`Completed`
      (if (`self.NoRandom`)
        (if (== _typeselected "Pistola")
          (set `self.Index_Selected` 0)
          (`PrimitiveComponent.SetMaterial` (`self.StaticMesh`) 0 "/Game/Materials/M_Cube_Purple.M_Cube_Purple" :!label _label)
          (elif (== _typeselected "Escopeta")
            (set `self.Index_Selected` 1)
            (`PrimitiveComponent.SetMaterial` (`self.StaticMesh`) 0 "/Game/Materials/M_Cube_Orange.M_Cube_Orange" :!label _label_2)
            (elif (== _typeselected "Ametralladora")
              (set `self.Index_Selected` 2)
              (`PrimitiveComponent.SetMaterial` (`self.StaticMesh`) 0 "/Game/Materials/M_Cube_Green.M_Cube_Green" :!label _label_3)
              (elif (== _typeselected "Electrico")
                (set `self.Index_Selected` 3)
                (`PrimitiveComponent.SetMaterial` (`self.StaticMesh`) 0 "/Game/Materials/M_Cube_Blue.M_Cube_Blue" :!label _label_4)
                (elif (== _typeselected "Laser")
                  (set `self.Index_Selected` 4)
                  (`PrimitiveComponent.SetMaterial` (`self.StaticMesh`) 0 "/Game/Materials/M_Cube_Red.M_Cube_Red" :!label _label_5)
                  (elif (== _typeselected "Rayo")
                    (set `self.Index_Selected` 5)
                    (`PrimitiveComponent.SetMaterial` (`self.StaticMesh`) 0 "/Game/Materials/M_Cube_Yellow.M_Cube_Yellow" :!label _label_6)))))))
        (else
          (bind _output_get (set `self.Index_Selected` (`KismetMathLibrary.RandomIntegerInRange` 0 2)))
          (set `self.TypeSelected` (`|GetArrayItem` (`self.Type_Array`) _output_get))
          (if (== _typeselected_2 "Pistola")
            (goto _label)
            (elif (== _typeselected_2 "Escopeta")
              (goto _label_2)
              (elif (== _typeselected_2 "Ametralladora")
                (goto _label_3)
                (elif (== _typeselected_2 "Electrico")
                  (goto _label_4)
                  (elif (== _typeselected_2 "Laser")
                    (goto _label_5)
                    (elif (== _typeselected_2 "Rayo")
                      (goto _label_6))))))))))))

(event `self.Box.OnComponentBeginOverlap`
  (params (OverlappedComponent :type "PrimitiveComponent Object Reference") (OtherActor :type "Actor Object Reference") (OtherComp :type "PrimitiveComponent Object Reference") (OtherBodyIndex :type Integer) (bFromSweep :type Boolean) (SweepResult :type "HitResult Structure (by ref)"))
  (bind _particlesystem (`self.ParticleSystem`))
  (bind _index_selected (`self.Index_Selected`))
  (bind _typeselected (`self.TypeSelected`))
  (bind _output (`|GetArrayItem` (`self.FireRate`) _index_selected))
  (bind _asnew_pawn (cast `/Game/NEW_Blueprints/NEW_Pawn` OtherActor))
  (`/Engine/EditorBlueprintResources/StandardMacros.DoOnce` false :!label _label_7
    (:`Completed`
      (`KismetSystemLibrary.PrintString` (`KismetStringLibrary.Conv_IntToString` _index_selected))
      (`KismetSystemLibrary.PrintString` (`KismetStringLibrary.Conv_DoubleToString` _output))
      (set `/Game/NEW_Blueprints/NEW_Pawn.FireRate` _output _asnew_pawn)
      (`KismetSystemLibrary.PrintString` (`KismetStringLibrary.Conv_NameToString` _typeselected))
      (if (== _typeselected "Pistola")
        (`self.ResetWeapon`)
        (set `/Game/NEW_Blueprints/NEW_Pawn.Equip_Pistola` true _asnew_pawn)
        (`SceneComponent.SetVisibility` (`self.Box`) false false :!label _label_8)
        (`ActorComponent.Activate` _particlesystem false)
        (`KismetSystemLibrary.Delay` 0.3)
        (`ActorComponent.Deactivate` _particlesystem)
        (if (`self.NoRandom`)
          (goto _label_7 :!via `Reset`)
          (else
            (`self.K2_DestroyActor`)))
        (elif (== _typeselected "Escopeta")
          (`self.ResetWeapon`)
          (set `/Game/NEW_Blueprints/NEW_Pawn.Equip_Escopeta` true _asnew_pawn)
          (goto _label_8)
          (elif (== _typeselected "Ametralladora")
            (`self.ResetWeapon`)
            (set `/Game/NEW_Blueprints/NEW_Pawn.Equip_Metra` true _asnew_pawn)
            (goto _label_8)
            (elif (== _typeselected "Electrico")
              (`self.ResetWeapon`)
              (set `/Game/NEW_Blueprints/NEW_Pawn.Equip_Electric` true _asnew_pawn)
              (goto _label_8)
              (elif (== _typeselected "Laser")
                (`self.ResetWeapon`)
                (set `/Game/NEW_Blueprints/NEW_Pawn.Equip_Laser` true _asnew_pawn)
                (goto _label_8)
                (elif (== _typeselected "Rayo")
                  (`self.ResetWeapon`)
                  (set `/Game/NEW_Blueprints/NEW_Pawn.Equip_Rayo` true _asnew_pawn)
                  (goto _label_8))))))))))

(event `ResetWeapon`
  (set `/Game/NEW_Blueprints/NEW_Pawn.Equip_Pistola` false (stale `self.Box.OnComponentBeginOverlap` _asnew_pawn))
  (set `/Game/NEW_Blueprints/NEW_Pawn.Equip_Escopeta` false (stale `self.Box.OnComponentBeginOverlap` _asnew_pawn))
  (set `/Game/NEW_Blueprints/NEW_Pawn.Equip_Laser` false (stale `self.Box.OnComponentBeginOverlap` _asnew_pawn))
  (set `/Game/NEW_Blueprints/NEW_Pawn.Equip_Electric` false (stale `self.Box.OnComponentBeginOverlap` _asnew_pawn))
  (set `/Game/NEW_Blueprints/NEW_Pawn.Equip_Metra` false (stale `self.Box.OnComponentBeginOverlap` _asnew_pawn))
  (set `/Game/NEW_Blueprints/NEW_Pawn.Equip_Rayo` false (stale `self.Box.OnComponentBeginOverlap` _asnew_pawn)))

(fn `UserConstructionScript`)