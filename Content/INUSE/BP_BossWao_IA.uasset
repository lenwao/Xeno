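; Boss character that spawns three numbered BP_BossWaoHijo minions at its attach points on BeginPlay and kills the player pawn on overlap with its GrabSphere.
; Bullet overlaps and the SlowDie and danorayo events share one wound counter.
; A wound threshold changes the movement speed of boss and minions.
; The final threshold plays a death effect, kills the minions, notifies the player pawn, clears BP_AreaSpawn's BossSpawn flag and destroys the boss.
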(event `self.ReceiveBeginPlay`
  (bind _outactors (`GameplayStatics.GetAllActorsOfClass` "/Game/Blueprints/Pawn/NEW_Pawn.NEW_Pawn_C"))
  (set `self.Ref_Pawn` (`|GetArrayItem` _outactors))
  (`|SpawnActorFromClass` "/Game/INUSE/BP_BossWaoHijo.BP_BossWaoHijo_C" (`KismetMathLibrary.MakeTransform` (`SceneComponent.K2_GetComponentLocation` (`self.Hijo1SItio`))) "AlwaysSpawn" "OverrideRootScale" null null)
  (`|SpawnActorFromClass` "/Game/INUSE/BP_BossWaoHijo.BP_BossWaoHijo_C" (`KismetMathLibrary.MakeTransform` (`SceneComponent.K2_GetComponentLocation` (`self.Hijo2Sitio`))) "AlwaysSpawn" "OverrideRootScale" null null)
  (`|SpawnActorFromClass` "/Game/INUSE/BP_BossWaoHijo.BP_BossWaoHijo_C" (`KismetMathLibrary.MakeTransform` (`SceneComponent.K2_GetComponentLocation` (`self.Hijo3Stio`))) "AlwaysSpawn" "OverrideRootScale" null null)
  (bind _outactors_2 (`GameplayStatics.GetAllActorsOfClass` "/Game/INUSE/BP_BossWaoHijo.BP_BossWaoHijo_C"))
  (bind _output_get (set `self.NewVar_1` (`|GetArrayItem` _outactors_2)))
  (set `/Game/INUSE/BP_BossWaoHijo.NumeroHijo` 0 _output_get)
  (bind _output_get_2 (set `self.NewVar_4` (`|GetArrayItem` _outactors_2 1)))
  (set `/Game/INUSE/BP_BossWaoHijo.NumeroHijo` 1 _output_get_2)
  (bind _output_get_3 (set `self.NewVar_5` (`|GetArrayItem` _outactors_2 2)))
  (set `/Game/INUSE/BP_BossWaoHijo.NumeroHijo` 2 _output_get_3))

(event `self.GrabSphere.OnComponentBeginOverlap`
  (params (OverlappedComponent :type "PrimitiveComponent Object Reference") (OtherActor :type "Actor Object Reference") (OtherComp :type "PrimitiveComponent Object Reference") (OtherBodyIndex :type Integer) (bFromSweep :type Boolean) (SweepResult :type "HitResult Structure (by ref)"))
  (bind _heridas (`self.Heridas`))
  (bind _newvar_1 (`self.NewVar_1`))
  ;[1 1 1] Kill Pawn by Proximity
  (`|ExecutionSequence`
    (:`then_0`
      (bind _asnew_pawn (cast `/Game/Blueprints/Pawn/NEW_Pawn` OtherActor))
      (`/Game/Blueprints/Pawn/NEW_Pawn.PawnDie` _asnew_pawn ""))
    (:`then_1`
      ;[1 1 1] Got Shot
      (cast `/Game/Blueprints/Pawn/NEW_Balas` OtherActor)
      ;[1 1 1] Slow Die
      (`/Engine/EditorBlueprintResources/StandardMacros.IncrementInt` _heridas :!label _label
        (:`  `
          (if (== _heridas 20)
            (`GameplayStatics.SpawnEmitterAtLocation` "/Game/Particles/P_Die_Boss.P_Die_Boss" (`SceneComponent.K2_GetComponentLocation` (`self.Torso`)) (struct) (1.5 1.5 1.0))
            (`/Game/INUSE/BP_BossWaoHijo.Muerte` _newvar_1)
            (`/Game/INUSE/BP_BossWaoHijo.Muerte` (`self.NewVar_4`))
            (`/Game/INUSE/BP_BossWaoHijo.Muerte` (`self.NewVar_5`))
            (`/Game/Blueprints/Pawn/NEW_Pawn.EVENT` (`self.Ref_Pawn`) "BP_BossWao_IA_C")
            (bind _outactors (`GameplayStatics.GetAllActorsOfClass` "/Game/Blueprints/Pawn/BP_AreaSpawn.BP_AreaSpawn_C"))
            (set `/Game/Blueprints/Pawn/BP_AreaSpawn.BossSpawn` false (`|GetArrayItem` _outactors))
            (`self.K2_DestroyActor`)
            (elif (== _heridas 14)
              (set `CharacterMovementComponent.MaxWalkSpeed` 450.0 (`self.CharacterMovement`))
              (set `/Game/INUSE/BP_BossWaoHijo.MovementSpeed` 7 _newvar_1)
              (set `/Game/INUSE/BP_BossWaoHijo.MovementSpeed` 7 (`self.NewVar_4`))
              (set `/Game/INUSE/BP_BossWaoHijo.MovementSpeed` 7 (`self.NewVar_5`)))))))))

(event `danorayo`
  ;[1 1 1] Slow Die
  (goto _label))

(event `SlowDie`
  ;[1 1 1] Slow Die
  (goto _label))

(fn `UserConstructionScript`)