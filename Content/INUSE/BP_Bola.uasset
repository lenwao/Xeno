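; BP_Bola is an enemy that homes in on the player's NEW_Pawn and kills it on overlap.
; Tick nudges Torso toward the pawn's SMTorso in X and Y with random jitter, unless Blood is set.
; Overlapping a NEW_Balas projectile or receiving the danorayo event spawns the P_Die_Slow emitter and destroys the actor.
; Logic to rotate Torso toward the pawn exists but is disconnected.
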(event `self.ReceiveBeginPlay`
  (bind _outactors (`GameplayStatics.GetAllActorsOfClass` "/Game/Blueprints/Pawn/NEW_Pawn.NEW_Pawn_C"))
  (set `self.pawn` (`|GetArrayItem` _outactors)))

(event `self.ReceiveTick`
  (params (DeltaSeconds :type "Float (single-precision)"))
  (bind _sm_torso (`/Game/Blueprints/Pawn/NEW_Pawn.SM_Torso` (`self.pawn`)))
  (bind (_returnvalue_x _returnvalue_y) (`KismetMathLibrary.BreakVector` (* (`KismetMathLibrary.Normal` (- (`SceneComponent.K2_GetComponentLocation` _sm_torso) (`SceneComponent.K2_GetComponentLocation` (`self.Torso`)))) (`self.MovementSpeed`))))
  ;[1 1 1] Movement and Rotation
  (`/Engine/EditorBlueprintResources/StandardMacros.IsValid` _sm_torso
    (:`Is Valid`
      (if (not (`self.Blood`))
        (`SceneComponent.K2_AddRelativeLocation` (`self.Torso`) (`KismetMathLibrary.MakeVector` (+ _returnvalue_x (`KismetMathLibrary.RandomFloatInRange` -3.0 3.0)) (+ _returnvalue_y (`KismetMathLibrary.RandomFloatInRange` -3.0 3.0))) false false)))))

(event `self.Collision.OnComponentBeginOverlap`
  (params (OverlappedComponent :type "PrimitiveComponent Object Reference") (OtherActor :type "Actor Object Reference") (OtherComp :type "PrimitiveComponent Object Reference") (OtherBodyIndex :type Integer) (bFromSweep :type Boolean) (SweepResult :type "HitResult Structure (by ref)"))
  (`|ExecutionSequence`
    (:`then_0`
      ;[1 1 1] Kill Pawn by Proximity
      (bind _asnew_pawn (cast `/Game/Blueprints/Pawn/NEW_Pawn` OtherActor))
      (`/Game/Blueprints/Pawn/NEW_Pawn.PawnDie` _asnew_pawn ""))
    (:`then_1`
      ;[1 1 1] Got Shot
      (cast `/Game/Blueprints/Pawn/NEW_Balas` OtherActor)
      ;[1 1 1] Slow Die
      (`GameplayStatics.SpawnEmitterAtLocation` "/Game/Particles/P_Die_Slow.P_Die_Slow" (`SceneComponent.K2_GetComponentLocation` (`self.Torso`)) :!label _label)
      (`self.K2_DestroyActor`))))

(event `danorayo`
  ;[1 1 1] Slow Die
  (goto _label))

(fn `UserConstructionScript`)