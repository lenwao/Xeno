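; Dash enemy that randomly becomes a blue smoke variant or a splash variant on BeginPlay.
; The player entering DashCube triggers a timed speed boost: blue activates its Dash component and drops smoke on deactivation, the other spawns splashes every tick.
; Only rear bullet hits deal damage, while the Collision component deflects bullets with sparks and kills the player on touch.
; Death spawns an explosion effect and calls AnotherDash on BP_AreaSpawn.
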(event `self.ReceiveTick`
  (params (DeltaSeconds :type "Float (single-precision)"))
  (if (`self.quieto`)
    (if (not (`self.Azul/Rojo`))
      (`|SpawnActorFromClass` "/Game/CORE/Blueprints/Sangre/BP_Dash_Splash.BP_Dash_Splash_C" (`KismetMathLibrary.MakeTransform` (`SceneComponent.K2_GetComponentLocation` (`self.Torso`))) "DontSpawnIfColliding" "OverrideRootScale" self null))))

(event `self.ReceiveBeginPlay`
  (bind _outactors (`GameplayStatics.GetAllActorsOfClass` "/Game/CORE/Blueprints/Pawn/NEW_Pawn.NEW_Pawn_C"))
  (set `self.Ref_Pawn` (`|GetArrayItem` _outactors))
  (set `self.Azul/Rojo` (`KismetMathLibrary.RandomBool`))
  (if (`self.Azul/Rojo`)
    (`StaticMeshComponent.SetStaticMesh` (`self.Torso`) "/Game/CORE/StaticMeshes/Characters/SM_Dash_Blue.SM_Dash_Blue")))

(event `self.DashCube.OnComponentBeginOverlap`
  (params (OverlappedComponent :type "PrimitiveComponent Object Reference") (OtherActor :type "Actor Object Reference") (OtherComp :type "PrimitiveComponent Object Reference") (OtherBodyIndex :type Integer) (bFromSweep :type Boolean) (SweepResult :type "HitResult Structure (by ref)"))
  (bind _charactermovement (`self.CharacterMovement`))
  ;[1 1 1] Add Actors to Range of Explosion / Ignore Self
  (cast `/Game/CORE/Blueprints/Pawn/NEW_Pawn` OtherActor
    (:`then`
      (`|ExecutionSequence`
        (:`then_0`
          (set `self.Count_Down` true)
          (if (`self.Azul/Rojo`)
            ;[1 1 1] quedarse quieto andes del dash
            (`ActorComponent.Activate` (`self.dash`) true))
          (if (not (`self.Dashea`))
            (set `self.Dashea` true)
            (set `self.quieto` true)
            (set `CharacterMovementComponent.MaxWalkSpeed` 1000.0 _charactermovement)
            (`KismetSystemLibrary.Delay` 4.0)
            (set `self.quieto` false)
            (set `CharacterMovementComponent.MaxWalkSpeed` 400.0 _charactermovement)))
        (:`then_1`
          (`KismetArrayLibrary.Array_Add` (`self.In_Range`) OtherActor :!label _label))))
    (:`CastFailed`
      (goto _label))))

(event `self.DashCube.OnComponentEndOverlap`
  (params (OverlappedComponent :type "PrimitiveComponent Object Reference") (OtherActor :type "Actor Object Reference") (OtherComp :type "PrimitiveComponent Object Reference") (OtherBodyIndex :type Integer))
  ;[1 1 1] Pawn Exit Range of Explosion  / Deactivate Count Down
  (cast `/Game/CORE/Blueprints/Pawn/NEW_Pawn` OtherActor)
  (set `self.Count_Down` false :!label _label_2)
  (set `self.Dashea` false)
  (`ActorComponent.Deactivate` (`self.dash`)))

(event `self.Range sphere.OnComponentBeginOverlap`
  (params (OverlappedComponent :type "PrimitiveComponent Object Reference") (OtherActor :type "Actor Object Reference") (OtherComp :type "PrimitiveComponent Object Reference") (OtherBodyIndex :type Integer) (bFromSweep :type Boolean) (SweepResult :type "HitResult Structure (by ref)"))
  ;[1 1 1] Remove Actors from Range of Explosion
  (cast `/Game/CORE/Blueprints/Pawn/NEW_Pawn` OtherActor
    (:`then`
      (`|ExecutionSequence`
        (:`then_0`
          (goto _label_2))
        (:`then_1`
          _)))
    (:`CastFailed`
      _))
  (`KismetArrayLibrary.Array_RemoveItem` (`self.In_Range`) OtherActor))

(event `self.dash.OnComponentDeactivated`
  (params (Component :type "ActorComponent Object Reference"))
  (bind _arrow1 (`self.Arrow1`))
  ;[1 1 1] spawn humo collision
  (if (`self.Azul/Rojo`)
    (`|SpawnActorFromClass` "/Game/OLD/BP_Dash_Humo.BP_Dash_Humo_C" (`KismetMathLibrary.MakeTransform` (`SceneComponent.K2_GetComponentLocation` _arrow1) (`KismetMathLibrary.Conv_VectorToRotator` (`SceneComponent.GetForwardVector` _arrow1))) "Undefined" "OverrideRootScale" null null)))

(event `self.parteTrasera.OnComponentBeginOverlap`
  (params (OverlappedComponent :type "PrimitiveComponent Object Reference") (OtherActor :type "Actor Object Reference") (OtherComp :type "PrimitiveComponent Object Reference") (OtherBodyIndex :type Integer) (bFromSweep :type Boolean) (SweepResult :type "HitResult Structure (by ref)"))
  ;[1 1 1] Got Shot
  (bind _asbp_bullets (cast `/Game/CORE/Blueprints/Pawn/BP_Bullets` OtherActor))
  (`/Game/CORE/Blueprints/Pawn/BP_Bullets.Hit` _asbp_bullets)
  (bind _output_get (set `self.Vida` (- (`self.Vida`) (`/Game/CORE/Blueprints/Pawn/NEW_Pawn.Damage` (`self.Ref_Pawn`)))))
  (if (<= _output_get 0)
    (`GameplayStatics.SpawnEmitterAtLocation` "/Game/CORE/Particles/P_Die_Boss.P_Die_Boss" (`SceneComponent.K2_GetComponentLocation` (`self.Torso`)))
    (bind _outactors (`GameplayStatics.GetAllActorsOfClass` "/Game/CORE/Blueprints/Pawn/BP_AreaSpawn.BP_AreaSpawn_C"))
    (`/Game/CORE/Blueprints/Pawn/BP_AreaSpawn.Another Dash` (`|GetArrayItem` _outactors))
    (`self.K2_DestroyActor`)))

(event `self.Collision.OnComponentBeginOverlap`
  (params (OverlappedComponent :type "PrimitiveComponent Object Reference") (OtherActor :type "Actor Object Reference") (OtherComp :type "PrimitiveComponent Object Reference") (OtherBodyIndex :type Integer) (bFromSweep :type Boolean) (SweepResult :type "HitResult Structure (by ref)"))
  ;[1 1 1] Kill Pawn by Proximity
  (bind _asnew_pawn (cast `/Game/CORE/Blueprints/Pawn/NEW_Pawn` OtherActor)
    (:`then`
      (`/Game/CORE/Blueprints/Pawn/NEW_Pawn.PawnDie` _asnew_pawn (`KismetSystemLibrary.GetDisplayName` self)))
    (:`CastFailed`
      (bind _asbp_bullets (cast `/Game/CORE/Blueprints/Pawn/BP_Bullets` OtherActor))
      (`GameplayStatics.PlaySound2D` "/Game/CORE/Audio/metalsound.metalsound" 1.0 (`KismetMathLibrary.RandomFloatInRange` 0.0 1.0) 0.0 null null)
      (bind (_returnvalue_x _returnvalue_y _returnvalue_z) (`KismetMathLibrary.BreakVector` (`SceneComponent.K2_GetComponentLocation` (`/Game/CORE/Blueprints/Pawn/BP_Bullets.Plane` _asbp_bullets))))
      (`GameplayStatics.SpawnEmitterAtLocation` "/Game/CORE/Particles/P_Hit_Sparks.P_Hit_Sparks" (`KismetMathLibrary.MakeVector` _returnvalue_x _returnvalue_y _returnvalue_z) (struct) (0.5 0.5 0.5))
      (`self.K2_DestroyActor` _asbp_bullets))))

(fn `UserConstructionScript`)