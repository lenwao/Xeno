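; Proximity sensor that tracks nearby enemies for the player pawn (NEW_Pawn), which it looks up on BeginPlay.
; Two overlap spheres cast entering actors against seven enemy and boss classes.
; Sphere adds matches to the pawn's CercaArray (near), Sphere1 to MuyCercaArray (very near).
; Only Sphere1 handles end overlap, so this asset never removes entries from CercaArray.
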(event `self.ReceiveBeginPlay`
  (bind _outactors (`GameplayStatics.GetAllActorsOfClass` "/Game/CORE/Blueprints/Pawn/NEW_Pawn.NEW_Pawn_C"))
  (set `self.RefPawn` (`|GetArrayItem` _outactors)))

(event `self.Sphere.OnComponentBeginOverlap`
  (params (OverlappedComponent :type "PrimitiveComponent Object Reference") (OtherActor :type "Actor Object Reference") (OtherComp :type "PrimitiveComponent Object Reference") (OtherBodyIndex :type Integer) (bFromSweep :type Boolean) (SweepResult :type "HitResult Structure (by ref)"))
  (bind _refpawn (`self.RefPawn`))
  (bind _cercaarray (`/Game/CORE/Blueprints/Pawn/NEW_Pawn.CercaArray` (`self.RefPawn`)))
  (bind _cercaarray_2 (`/Game/CORE/Blueprints/Pawn/NEW_Pawn.CercaArray` (`self.RefPawn`)))
  (`|ExecutionSequence`
    (:`then_0`
      (bind _asnew_slow_ia (cast `/Game/CORE/Blueprints/Aliens/NEW_Slow_IA` OtherActor))
      (`KismetArrayLibrary.Array_Add` (`/Game/CORE/Blueprints/Pawn/NEW_Pawn.CercaArray` (`self.RefPawn`)) _asnew_slow_ia))
    (:`then_1`
      (bind _asnew_bomb_ia (cast `/Game/CORE/Blueprints/Aliens/NEW_Bomb_IA` OtherActor))
      (`KismetArrayLibrary.Array_Add` (`/Game/CORE/Blueprints/Pawn/NEW_Pawn.CercaArray` _refpawn) _asnew_bomb_ia))
    (:`then_2`
      (bind _asnew_dash_fran (cast `/Game/CORE/Blueprints/Aliens/NEW_Dash_Fran` OtherActor))
      (`KismetArrayLibrary.Array_Add` (`/Game/CORE/Blueprints/Pawn/NEW_Pawn.CercaArray` _refpawn) _asnew_dash_fran))
    (:`then_3`
      (bind _asnew_boss_giant_ia (cast `/Game/CORE/Blueprints/Aliens/NEW_Boss_giant_IA` OtherActor))
      (`KismetArrayLibrary.Array_Add` _cercaarray _asnew_boss_giant_ia))
    (:`then_4`
      (bind _asbp_boss_wao_ia (cast `/Game/CORE/Blueprints/Aliens/BP_BossWao_IA` OtherActor))
      (`KismetArrayLibrary.Array_Add` _cercaarray _asbp_boss_wao_ia))
    (:`then_5`
      (bind _asbp_el_bolas (cast `/Game/CORE/Blueprints/Aliens/BP_ElBolas` OtherActor))
      (`KismetArrayLibrary.Array_Add` _cercaarray_2 _asbp_el_bolas))
    (:`then_6`
      (bind _asnew_cienpies (cast `/Game/CORE/Blueprints/Aliens/NEW_Cienpies` OtherActor))
      (`KismetArrayLibrary.Array_Add` _cercaarray_2 _asnew_cienpies))))

(event `self.Sphere1.OnComponentBeginOverlap`
  (params (OverlappedComponent :type "PrimitiveComponent Object Reference") (OtherActor :type "Actor Object Reference") (OtherComp :type "PrimitiveComponent Object Reference") (OtherBodyIndex :type Integer) (bFromSweep :type Boolean) (SweepResult :type "HitResult Structure (by ref)"))
  (bind _muycercaarray (`/Game/CORE/Blueprints/Pawn/NEW_Pawn.MuyCercaArray` (`self.RefPawn`)))
  (bind _muycercaarray_2 (`/Game/CORE/Blueprints/Pawn/NEW_Pawn.MuyCercaArray` (`self.RefPawn`)))
  (bind _muycercaarray_3 (`/Game/CORE/Blueprints/Pawn/NEW_Pawn.MuyCercaArray` (`self.RefPawn`)))
  (`|ExecutionSequence`
    (:`then_0`
      (bind _asnew_slow_ia (cast `/Game/CORE/Blueprints/Aliens/NEW_Slow_IA` OtherActor))
      (`KismetArrayLibrary.Array_Add` (`/Game/CORE/Blueprints/Pawn/NEW_Pawn.MuyCercaArray` (`self.RefPawn`)) _asnew_slow_ia))
    (:`then_1`
      (bind _asnew_bomb_ia (cast `/Game/CORE/Blueprints/Aliens/NEW_Bomb_IA` OtherActor))
      (`KismetArrayLibrary.Array_Add` _muycercaarray _asnew_bomb_ia))
    (:`then_2`
      (bind _asnew_dash_fran (cast `/Game/CORE/Blueprints/Aliens/NEW_Dash_Fran` OtherActor))
      (`KismetArrayLibrary.Array_Add` _muycercaarray _asnew_dash_fran))
    (:`then_3`
      (bind _asnew_boss_giant_ia (cast `/Game/CORE/Blueprints/Aliens/NEW_Boss_giant_IA` OtherActor))
      (`KismetArrayLibrary.Array_Add` _muycercaarray_2 _asnew_boss_giant_ia))
    (:`then_4`
      (bind _asbp_boss_wao_ia (cast `/Game/CORE/Blueprints/Aliens/BP_BossWao_IA` OtherActor))
      (`KismetArrayLibrary.Array_Add` _muycercaarray_2 _asbp_boss_wao_ia))
    (:`then_5`
      (bind _asbp_el_bolas (cast `/Game/CORE/Blueprints/Aliens/BP_ElBolas` OtherActor))
      (`KismetArrayLibrary.Array_Add` _muycercaarray_3 _asbp_el_bolas))
    (:`then_6`
      (bind _asnew_cienpies (cast `/Game/CORE/Blueprints/Aliens/NEW_Cienpies` OtherActor))
      (`KismetArrayLibrary.Array_Add` _muycercaarray_3 _asnew_cienpies))))

(event `self.Sphere1.OnComponentEndOverlap`
  (params (OverlappedComponent :type "PrimitiveComponent Object Reference") (OtherActor :type "Actor Object Reference") (OtherComp :type "PrimitiveComponent Object Reference") (OtherBodyIndex :type Integer))
  (`KismetArrayLibrary.Array_RemoveItem` (`/Game/CORE/Blueprints/Pawn/NEW_Pawn.MuyCercaArray` (`self.RefPawn`)) OtherActor))

(fn `UserConstructionScript`)