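; Bullet actor that takes its mesh, particle effect and damage from a data table row keyed by the player pawn's current weapon.
; BeginPlay caches the pawn and game mode, spawns a shot effect, applies the row, then destroys the bullet after a one-second lifetime if the row was found.
; The Hit event flags the bullet as hit, spawns a blood effect just below the mesh and destroys the actor.
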(event `Hit`
  (bind (_returnvalue_x _returnvalue_y _returnvalue_z) (`KismetMathLibrary.BreakVector` (`SceneComponent.K2_GetComponentLocation` (`self.Plane`))))
  (set `self.Hitted` true)
  (`GameplayStatics.SpawnEmitterAtLocation` "/Game/CORE/Particles/P_Hit_Blood.P_Hit_Blood" (`KismetMathLibrary.MakeVector` _returnvalue_x _returnvalue_y (- _returnvalue_z 20.0)))
  (`self.K2_DestroyActor` :!label _label))

(event `self.ReceiveBeginPlay`
  (`|ExecutionSequence`
    (:`then_0`
      (bind _asnew_pawn (cast `/Game/CORE/Blueprints/Pawn/NEW_Pawn` (`GameplayStatics.GetPlayerPawn` 0)))
      (set `self.Ref_Pawn` _asnew_pawn)
      (bind _asgm_shooter (cast `/Game/CORE/Blueprints/GM_Shooter` (`GameplayStatics.GetGameMode`)))
      (set `self.Ref_GM` _asgm_shooter))
    (:`then_1`
      (`GameplayStatics.SpawnEmitterAtLocation` "/Game/CORE/Particles/P_Shots.P_Shots" (`SceneComponent.K2_GetComponentLocation` (`self.Plane`)) (struct) (0.5 0.5 0.5))
      (bind _returnvalue (`|GetDataTableRow` "/Game/CORE/Blueprints/DataTable_Bullets.DataTable_Bullets" (`/Game/CORE/Blueprints/Pawn/NEW_Pawn.Weapon` (`self.Ref_Pawn`)))
        (:`then`
          (bind (_nombre _color _damage _rate _velocity _sonido _mesh _particle) (break `/Game/CORE/Blueprints/Struct_Bullets` _returnvalue))
          (`StaticMeshComponent.SetStaticMesh` (`self.Plane`) _mesh)
          (`ParticleSystemComponent.SetTemplate` (`self.ParticleSystem`) _particle)
          (set `self.Damage` _damage)
          (`KismetSystemLibrary.Delay` 1.0)
          (goto _label))))))

(fn `UserConstructionScript`)