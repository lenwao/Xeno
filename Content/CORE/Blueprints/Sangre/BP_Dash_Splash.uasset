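; Blood splash actor that slows any NEW_Pawn standing in it, then fades away and destroys itself.
; On BeginPlay it gives its plane a random yaw and plays a timeline driving the material's opacity, creating a new dynamic material instance every update.
; The Ralentiza component's overlap events set the pawn's MovementSpeed2 to a hardcoded slow value on entry and a hardcoded restore value on exit.
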(event `self.ReceiveBeginPlay`
  (`SceneComponent.K2_SetWorldRotation` (`self.Plane`) (`KismetMathLibrary.MakeRotator` 0.0 0.0 (`KismetMathLibrary.RandomFloatInRange` 0.0 180.0)) false false)
  (bind (_direction _newtrack_0) (`Timeline|TimFadeAway`)
    (:`Update`
      (bind _returnvalue (`PrimitiveComponent.CreateDynamicMaterialInstance` (`self.Plane`) 0 "/Game/CORE/Materials/NEW_M_Aliens_Inst.NEW_M_Aliens_Inst" "None"))
      (`MaterialInstanceDynamic.SetScalarParameterValue` _returnvalue "Opacity_Value" _newtrack_0))
    (:`Finished`
      (`self.K2_DestroyActor`))))

(event `self.Ralentiza.OnComponentBeginOverlap`
  (params (OverlappedComponent :type "PrimitiveComponent Object Reference") (OtherActor :type "Actor Object Reference") (OtherComp :type "PrimitiveComponent Object Reference") (OtherBodyIndex :type Integer) (bFromSweep :type Boolean) (SweepResult :type "HitResult Structure (by ref)"))
  (bind _asnew_pawn (cast `/Game/CORE/Blueprints/Pawn/NEW_Pawn` OtherActor))
  (set `/Game/CORE/Blueprints/Pawn/NEW_Pawn.MovementSpeed2` 180.0 _asnew_pawn))

(event `self.Ralentiza.OnComponentEndOverlap`
  (params (OverlappedComponent :type "PrimitiveComponent Object Reference") (OtherActor :type "Actor Object Reference") (OtherComp :type "PrimitiveComponent Object Reference") (OtherBodyIndex :type Integer))
  (bind _asnew_pawn (cast `/Game/CORE/Blueprints/Pawn/NEW_Pawn` OtherActor))
  (set `/Game/CORE/Blueprints/Pawn/NEW_Pawn.MovementSpeed2` 220.0 _asnew_pawn))

(fn `UserConstructionScript`)