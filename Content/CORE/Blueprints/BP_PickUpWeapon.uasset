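; BP_PickUpWeapon is a weapon pickup that gives an overlapping NEW_Pawn a weapon and ammo.
; On BeginPlay, unless NoRandom is set, it picks a random DataTable_Bullets row, stores its name and ammo, and tints the cube via a dynamic material.
; Overlap assigns the weapon, then once disables collision, hides the cube and activates an effect.
; After a short delay it adds an ammo widget, sets pawn ammo and destroys itself.
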(event `self.ReceiveBeginPlay`
  (bind _weaponlist (`self.WeaponList`))
  (if (not (`self.NoRandom`))
    (bind _returnvalue (`DataTableFunctionLibrary.GetDataTableColumnAsString` "/Game/CORE/Blueprints/DataTable_Bullets.DataTable_Bullets" "Nombre"))
    (for _array_element _returnvalue
      (`KismetArrayLibrary.Array_Add` (`self.WeaponList`) _array_element))
    (bind _returnvalue_2 (`|GetDataTableRow` "/Game/CORE/Blueprints/DataTable_Bullets.DataTable_Bullets" (`KismetStringLibrary.Conv_StringToName` (`|GetArrayItem` _weaponlist (`KismetMathLibrary.RandomIntegerInRange` 0 (- (`KismetArrayLibrary.Array_Length` _weaponlist) 1)))))
      (:`then`
        (bind _returnvalue_3 (`PrimitiveComponent.CreateDynamicMaterialInstance` (`self.SM_Cube`) 0 "/Game/CORE/Materials/M_BaseMaterial.M_BaseMaterial" "None"))
        (bind (_nombre _color _damage _rate _velocity _ammo) (break `/Game/CORE/Blueprints/Struct_Bullets` _returnvalue_2))
        (`MaterialInstanceDynamic.SetVectorParameterValue` _returnvalue_3 "DiffuseColor" (`KismetMathLibrary.Conv_ColorToLinearColor` _color))
        (set `self.WeaponSelected` _nombre)
        (set `self.Ammo` _ammo)))))

(event `self.Collision.OnComponentBeginOverlap`
  (params (OverlappedComponent :type "PrimitiveComponent Object Reference") (OtherActor :type "Actor Object Reference") (OtherComp :type "PrimitiveComponent Object Reference") (OtherBodyIndex :type Integer) (bFromSweep :type Boolean) (SweepResult :type "HitResult Structure (by ref)"))
  (bind _asnew_pawn (cast `/Game/CORE/Blueprints/Pawn/NEW_Pawn` OtherActor))
  (set `/Game/CORE/Blueprints/Pawn/NEW_Pawn.Weapon` (`self.WeaponSelected`) _asnew_pawn)
  (set `self.Ref_Pawn` _asnew_pawn)
  (`KismetSystemLibrary.PrintString` (`KismetStringLibrary.Conv_NameToString` (`self.WeaponSelected`)))
  (`/Engine/EditorBlueprintResources/StandardMacros.DoOnce` false
    (:`Completed`
      (`PrimitiveComponent.SetCollisionEnabled` (`self.Collision`) "NoCollision")
      (`SceneComponent.SetVisibility` (`self.SM_Cube`) false false)
      (`ActorComponent.Activate` (`self.P_Totem_WeaponPick`) false)
      (`KismetSystemLibrary.Delay` 0.8)
      (bind _returnvalue (`|CreateWidget` "/Game/NEW/Widg_Ammo.Widg_Ammo_C"))
      (`UserWidget.AddToViewport` _returnvalue 0)
      (set `/Game/CORE/Blueprints/Pawn/NEW_Pawn.Ammo` (`self.Ammo`) (`self.Ref_Pawn`))
      (`self.K2_DestroyActor`))))

(fn `UserConstructionScript`)