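; Centipede boss alien that steers its head through three waypoint components on the player pawn, cycling via overlap flags.
; Each Tick, body segments chase the joint component ahead of them, forming a follow-the-leader chain.
; Bullets on the head or danorayo damage bleed it, removing tail segments every second hit until it dies and clears BP_AreaSpawn's BossSpawn.
; Body segments absorb bullets with an optional metal sound; contact kills the pawn.
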(event `self.ReceiveBeginPlay`
  (`KismetSystemLibrary.PrintString` (`KismetStringLibrary.Conv_NameToString` (`self.Type`)))
  (bind _outactors (`GameplayStatics.GetAllActorsOfClass` "/Game/CORE/Blueprints/Pawn/NEW_Pawn.NEW_Pawn_C"))
  (set `self.RefPawn` (`|GetArrayItem` _outactors))
  (bind _asgm_shooter (cast `/Game/CORE/Blueprints/GM_Shooter` (`GameplayStatics.GetGameMode`)))
  (set `self.Ref_GM` _asgm_shooter))

(event `self.ReceiveTick`
  (params (DeltaSeconds :type "Float (single-precision)"))
  (bind _puntocienpies (`/Game/CORE/Blueprints/Pawn/NEW_Pawn.PuntoCienpies` (`self.RefPawn`)))
  (bind _returnvalue (- (`SceneComponent.K2_GetComponentLocation` _puntocienpies) (`SceneComponent.K2_GetComponentLocation` (`self.Torso_01`))))
  (bind (_returnvalue_roll _returnvalue_pitch _returnvalue_yaw) (`KismetMathLibrary.BreakRotator` (`KismetMathLibrary.Conv_VectorToRotator` (* _returnvalue DeltaSeconds))))
  (bind (_returnvalue_x _returnvalue_y) (`KismetMathLibrary.BreakVector` (* (`KismetMathLibrary.Normal` _returnvalue) (`self.MovementSpeed`))))
  ;[1 1 1] Movement and Rotation
  (`|ExecutionSequence`
    (:`then_0`
      (if (`self.Punto2Cogido`)
        (`self.CAmbio a punto2` DeltaSeconds)
        (elif (`self.Punto1Cogido`)
          (`self.Cambio a punto1` DeltaSeconds)
          (else
            (`/Engine/EditorBlueprintResources/StandardMacros.IsValid` _puntocienpies
              (:`Is Valid`
                (if (not (`self.Blood`))
                  (`SceneComponent.K2_SetWorldRotation` (`self.Torso_01`) (`KismetMathLibrary.MakeRotator` 0.0 0.0 _returnvalue_yaw) false false)
                  (`SceneComponent.K2_AddRelativeLocation` (`self.Torso_01`) (`KismetMathLibrary.MakeVector` _returnvalue_x _returnvalue_y) false false))))))))
    (:`then_1`
      ;[1 1 1] movimiento torsos
      (`self.Mover torso1` DeltaSeconds))
    (:`then_2`
      (`self.Mover torso2` DeltaSeconds))
    (:`then_3`
      (`self.mover torso3` DeltaSeconds))
    (:`then_4`
      (`self.mover torso4` DeltaSeconds))
    (:`then_5`
      (`self.mover torso5` DeltaSeconds))
    (:`then_6`
      (`self.mover torso6` DeltaSeconds))
    (:`then_7`
      (`self.mover torso7` DeltaSeconds))))

(event `danorayo`
  (bind _torso_01 (`self.Torso_01`))
  (bind (_returnvalue_x _returnvalue_y _returnvalue_z) (`KismetMathLibrary.BreakVector` (`SceneComponent.K2_GetComponentLocation` _torso_01)))
  (bind (_returnvalue_roll _returnvalue_pitch _returnvalue_yaw) (`KismetMathLibrary.BreakRotator` (`SceneComponent.K2_GetComponentRotation` _torso_01)))
  ;[1 1 1] Slow Die
  (`|SpawnActorFromClass` "/Game/CORE/Blueprints/Sangre/NEW_Blood.NEW_Blood_C" (`KismetMathLibrary.MakeTransform` (`KismetMathLibrary.MakeVector` _returnvalue_x _returnvalue_y (- _returnvalue_z 2.0)) (`KismetMathLibrary.MakeRotator` _returnvalue_roll _returnvalue_pitch (+ _returnvalue_yaw 90.0)) (1.3 1.3 1.0)) "Undefined" "OverrideRootScale" null null :!label _label)
  (`GameplayStatics.SpawnEmitterAtLocation` "/Game/CORE/Particles/P_Die_Slow.P_Die_Slow" (`KismetMathLibrary.MakeVector` _returnvalue_x _returnvalue_y _returnvalue_z))
  ;[1 1 1] numero disparos por torso para destruir
  (bind _result (`/Engine/EditorBlueprintResources/StandardMacros.IncrementInt` (`self.CuerposDestroy`))
    (:`  `
      (if (== _result 2)
        (`self.Destruir_Torso` (`self.head_07`) (`self.Torso_08`) (`self.colision_08`) (`self.Light_08`))
        (set `self.Torso_08_Destroyed` true)
        (elif (== _result 4)
          (`self.Destruir_Torso` (`self.head_06`) (`self.Torso_07`) (`self.colision_07`) (`self.Light_07`))
          (set `self.Torso_07_Destroyed` true)
          (elif (== _result 6)
            (`self.Destruir_Torso` (`self.head_05`) (`self.Torso_06`) (`self.Collision_06`) (`self.Light_06`))
            (set `self.Torso_06_Destroyed` true)
            (elif (== _result 8)
              (`self.Destruir_Torso` (`self.Head_04`) (`self.Torso_05`) (`self.Light_05`) (`self.Collision_05`))
              (set `self.Torso_05_Destroyed` true)
              (elif (== _result 10)
                (`self.Destruir_Torso` (`self.Head_03`) (`self.Torso_04`) (`self.Collision_04`) (`self.Light_04`))
                (set `self.Torso_04_Destroyed` true)
                (elif (== _result 12)
                  (`self.Destruir_Torso` (`self.Head_02`) (`self.Torso_03`) (`self.Collision_03`) (`self.Light_03`))
                  (set `self.Torso_03_Destroyed` true)
                  (elif (== _result 14)
                    (`self.Destruir_Torso` (`self.Head_01`) (`self.Torso_02`) (`self.Collision_02`) (`self.Light_02`))
                    (set `self.Torso_02_Destroyed` true)
                    (elif (== _result 16)
                      (`/Engine/EditorBlueprintResources/StandardMacros.DoOnce` false
                        (:`Completed`
                          (`GameplayStatics.SpawnEmitterAtLocation` "/Game/CORE/Particles/P_Die_Boss.P_Die_Boss" (`SceneComponent.K2_GetComponentLocation` (`self.Torso_01`)))
                          (`/Game/CORE/Blueprints/Pawn/NEW_Pawn.EVENT` (`self.RefPawn`) "NEW_Cienpies_C")
                          (bind _outactors (`GameplayStatics.GetAllActorsOfClass` "/Game/CORE/Blueprints/Pawn/BP_AreaSpawn.BP_AreaSpawn_C"))
                          (set `/Game/CORE/Blueprints/Pawn/BP_AreaSpawn.BossSpawn` false (`|GetArrayItem` _outactors))
                          (`self.K2_DestroyActor`))))))))))))))

(event `self.Collision_01.OnComponentBeginOverlap`
  (params (OverlappedComponent :type "PrimitiveComponent Object Reference") (OtherActor :type "Actor Object Reference") (OtherComp :type "PrimitiveComponent Object Reference") (OtherBodyIndex :type Integer) (bFromSweep :type Boolean) (SweepResult :type "HitResult Structure (by ref)"))
  (`|ExecutionSequence`
    (:`then_0`
      ;[1 1 1] Got Shot
      (cast `/Game/CORE/Blueprints/Pawn/BP_Bullets` OtherActor)
      (goto _label))
    (:`then_1`
      ;[1 1 1] Kill Pawn by Proximity
      (bind _asnew_pawn (cast `/Game/CORE/Blueprints/Pawn/NEW_Pawn` OtherActor))
      (`|ExecutionSequence`
        (:`then_0`
          (`self.ColisionContraPawn` _asnew_pawn OtherComp _asnew_pawn))
        (:`then_1`
          (`self.ColisionContraPuntocinpies` _asnew_pawn _asnew_pawn OtherComp))
        (:`then_2`
          (`self.Colision conta Punto1cienpies` _asnew_pawn OtherComp))
        (:`then_3`
          (`self.Colision contra punto2 cienpies` _asnew_pawn OtherComp))))))

(event `self.Collision_02.OnComponentBeginOverlap`
  (params (OverlappedComponent :type "PrimitiveComponent Object Reference") (OtherActor :type "Actor Object Reference") (OtherComp :type "PrimitiveComponent Object Reference") (OtherBodyIndex :type Integer) (bFromSweep :type Boolean) (SweepResult :type "HitResult Structure (by ref)"))
  ;[1 1 1] colisiones con torso
  (bind _asnew_pawn (cast `/Game/CORE/Blueprints/Pawn/NEW_Pawn` OtherActor)
    (:`then`
      (if (== OtherComp (`/Game/CORE/Blueprints/Pawn/NEW_Pawn.Collision` _asnew_pawn))
        (`/Game/CORE/Blueprints/Pawn/NEW_Pawn.PawnDie` _asnew_pawn "")))
    (:`CastFailed`
      (bind _asbp_bullets (cast `/Game/CORE/Blueprints/Pawn/BP_Bullets` OtherActor))
      (if (`/Game/CORE/Blueprints/GM_Shooter.SoundOn?` (`self.Ref_GM`)) :!label _label_2
        (`GameplayStatics.PlaySound2D` "/Game/CORE/Audio/metalsound.metalsound" 1.0 (`KismetMathLibrary.RandomFloatInRange` 0.0 1.0) 0.0 null null))
      (`KismetSystemLibrary.Delay` 0.2)
      (`self.K2_DestroyActor` (stale `self.Collision_04.OnComponentBeginOverlap` _asbp_bullets))
      (`self.K2_DestroyActor` (stale `self.Collision_05.OnComponentBeginOverlap` _asbp_bullets))
      (`self.K2_DestroyActor` (stale `self.Collision_03.OnComponentBeginOverlap` _asbp_bullets))
      (`self.K2_DestroyActor` _asbp_bullets))))

(event `self.Collision_03.OnComponentBeginOverlap`
  (params (OverlappedComponent :type "PrimitiveComponent Object Reference") (OtherActor :type "Actor Object Reference") (OtherComp :type "PrimitiveComponent Object Reference") (OtherBodyIndex :type Integer) (bFromSweep :type Boolean) (SweepResult :type "HitResult Structure (by ref)"))
  ;[1 1 1] colisiones con torso
  (bind _asnew_pawn (cast `/Game/CORE/Blueprints/Pawn/NEW_Pawn` OtherActor)
    (:`then`
      (if (== OtherComp (`/Game/CORE/Blueprints/Pawn/NEW_Pawn.Collision` _asnew_pawn))
        (`/Game/CORE/Blueprints/Pawn/NEW_Pawn.PawnDie` _asnew_pawn "")))
    (:`CastFailed`
      (bind _asbp_bullets (cast `/Game/CORE/Blueprints/Pawn/BP_Bullets` OtherActor))
      (goto _label_2))))

(event `self.Collision_04.OnComponentBeginOverlap`
  (params (OverlappedComponent :type "PrimitiveComponent Object Reference") (OtherActor :type "Actor Object Reference") (OtherComp :type "PrimitiveComponent Object Reference") (OtherBodyIndex :type Integer) (bFromSweep :type Boolean) (SweepResult :type "HitResult Structure (by ref)"))
  ;[1 1 1] colisiones con torso
  (bind _asnew_pawn (cast `/Game/CORE/Blueprints/Pawn/NEW_Pawn` OtherActor)
    (:`then`
      (if (== OtherComp (`/Game/CORE/Blueprints/Pawn/NEW_Pawn.Collision` _asnew_pawn))
        (`/Game/CORE/Blueprints/Pawn/NEW_Pawn.PawnDie` _asnew_pawn "")))
    (:`CastFailed`
      (bind _asbp_bullets (cast `/Game/CORE/Blueprints/Pawn/BP_Bullets` OtherActor))
      (goto _label_2))))

(event `self.Collision_05.OnComponentBeginOverlap`
  (params (OverlappedComponent :type "PrimitiveComponent Object Reference") (OtherActor :type "Actor Object Reference") (OtherComp :type "PrimitiveComponent Object Reference") (OtherBodyIndex :type Integer) (bFromSweep :type Boolean) (SweepResult :type "HitResult Structure (by ref)"))
  ;[1 1 1] colisiones con torso
  (bind _asnew_pawn (cast `/Game/CORE/Blueprints/Pawn/NEW_Pawn` OtherActor)
    (:`then`
      (if (== OtherComp (`/Game/CORE/Blueprints/Pawn/NEW_Pawn.Collision` _asnew_pawn))
        (`/Game/CORE/Blueprints/Pawn/NEW_Pawn.PawnDie` _asnew_pawn "")))
    (:`CastFailed`
      (bind _asbp_bullets (cast `/Game/CORE/Blueprints/Pawn/BP_Bullets` OtherActor))
      (goto _label_2))))

(event `self.Collision_06.OnComponentBeginOverlap`
  (params (OverlappedComponent :type "PrimitiveComponent Object Reference") (OtherActor :type "Actor Object Reference") (OtherComp :type "PrimitiveComponent Object Reference") (OtherBodyIndex :type Integer) (bFromSweep :type Boolean) (SweepResult :type "HitResult Structure (by ref)"))
  ;[1 1 1] colisiones con torso
  (bind _asnew_pawn (cast `/Game/CORE/Blueprints/Pawn/NEW_Pawn` OtherActor)
    (:`then`
      (if (== OtherComp (`/Game/CORE/Blueprints/Pawn/NEW_Pawn.Collision` _asnew_pawn))
        (`/Game/CORE/Blueprints/Pawn/NEW_Pawn.PawnDie` _asnew_pawn "")))
    (:`CastFailed`
      (bind _asbp_bullets (cast `/Game/CORE/Blueprints/Pawn/BP_Bullets` OtherActor))
      (if (`/Game/CORE/Blueprints/GM_Shooter.SoundOn?` (`self.Ref_GM`)) :!label _label_3
        (`GameplayStatics.PlaySound2D` "/Game/CORE/Audio/metalsound.metalsound" 1.0 (`KismetMathLibrary.RandomFloatInRange` 0.0 1.0) 0.0 null null))
      (`self.K2_DestroyActor` _asbp_bullets)
      (`self.K2_DestroyActor` (stale `self.colision_07.OnComponentBeginOverlap` _asbp_bullets))
      (`self.K2_DestroyActor` (stale `self.colision_08.OnComponentBeginOverlap` _asbp_bullets)))))

(event `self.colision_07.OnComponentBeginOverlap`
  (params (OverlappedComponent :type "PrimitiveComponent Object Reference") (OtherActor :type "Actor Object Reference") (OtherComp :type "PrimitiveComponent Object Reference") (OtherBodyIndex :type Integer) (bFromSweep :type Boolean) (SweepResult :type "HitResult Structure (by ref)"))
  ;[1 1 1] colisiones con torso
  (bind _asnew_pawn (cast `/Game/CORE/Blueprints/Pawn/NEW_Pawn` OtherActor)
    (:`then`
      (if (== OtherComp (`/Game/CORE/Blueprints/Pawn/NEW_Pawn.Collision` _asnew_pawn))
        (`/Game/CORE/Blueprints/Pawn/NEW_Pawn.PawnDie` _asnew_pawn "")))
    (:`CastFailed`
      (bind _asbp_bullets (cast `/Game/CORE/Blueprints/Pawn/BP_Bullets` OtherActor))
      (goto _label_3))))

(event `self.colision_08.OnComponentBeginOverlap`
  (params (OverlappedComponent :type "PrimitiveComponent Object Reference") (OtherActor :type "Actor Object Reference") (OtherComp :type "PrimitiveComponent Object Reference") (OtherBodyIndex :type Integer) (bFromSweep :type Boolean) (SweepResult :type "HitResult Structure (by ref)"))
  ;[1 1 1] colisiones con torso
  (bind _asnew_pawn (cast `/Game/CORE/Blueprints/Pawn/NEW_Pawn` OtherActor)
    (:`then`
      (if (== OtherComp (`/Game/CORE/Blueprints/Pawn/NEW_Pawn.Collision` _asnew_pawn))
        (`/Game/CORE/Blueprints/Pawn/NEW_Pawn.PawnDie` _asnew_pawn "")))
    (:`CastFailed`
      (bind _asbp_bullets (cast `/Game/CORE/Blueprints/Pawn/BP_Bullets` OtherActor))
      (goto _label_3))))

(fn `Cambio a punto1`
  (params (B :type "Float (double-precision)"))
  (bind _puntocienpies1 (`/Game/CORE/Blueprints/Pawn/NEW_Pawn.PuntoCienpies1` (`self.RefPawn`)))
  (bind _returnvalue (- (`SceneComponent.K2_GetComponentLocation` _puntocienpies1) (`SceneComponent.K2_GetComponentLocation` (`self.Torso_01`))))
  (bind (_returnvalue_x _returnvalue_y) (`KismetMathLibrary.BreakVector` (* (`KismetMathLibrary.Normal` _returnvalue) (`self.MovementSpeed`))))
  ;[1 1 1] cambio a punto 1
  (`/Engine/EditorBlueprintResources/StandardMacros.IsValid` _puntocienpies1
    (:`Is Valid`
      (if (not (`self.Blood`))
        (`SceneComponent.K2_SetWorldRotation` (`self.Torso_01`) (`KismetMathLibrary.Conv_VectorToRotator` (* _returnvalue B)) false false)
        (`SceneComponent.K2_AddRelativeLocation` (`self.Torso_01`) (`KismetMathLibrary.MakeVector` _returnvalue_x _returnvalue_y) false false)))))

(fn `CAmbio a punto2`
  (params (InputPin :type "Float (double-precision)"))
  (bind _puntocienpies2 (`/Game/CORE/Blueprints/Pawn/NEW_Pawn.PuntoCienpies2` (`self.RefPawn`)))
  (bind _returnvalue (- (`SceneComponent.K2_GetComponentLocation` _puntocienpies2) (`SceneComponent.K2_GetComponentLocation` (`self.Torso_01`))))
  (bind (_returnvalue_x _returnvalue_y) (`KismetMathLibrary.BreakVector` (* (`KismetMathLibrary.Normal` _returnvalue) (`self.MovementSpeed`))))
  ;[1 1 1] cambio a punto 2
  (`/Engine/EditorBlueprintResources/StandardMacros.IsValid` _puntocienpies2
    (:`Is Valid`
      (if (not (`self.Blood`))
        (`SceneComponent.K2_SetWorldRotation` (`self.Torso_01`) (`KismetMathLibrary.Conv_VectorToRotator` (* _returnvalue InputPin)) false false)
        (`SceneComponent.K2_AddRelativeLocation` (`self.Torso_01`) (`KismetMathLibrary.MakeVector` _returnvalue_x _returnvalue_y) false false)))))

(fn `Colision conta Punto1cienpies`
  (params (self2 :type "/Game/CORE/Blueprints/Pawn/NEW_Pawn Object Reference") (A :type "Object Object Reference"))
  (if (== A (`/Game/CORE/Blueprints/Pawn/NEW_Pawn.PuntoCienpies1` self2))
    (set `self.Punto2Cogido` true)
    (set `self.Punto1Cogido` false)))

(fn `Colision contra punto2 cienpies`
  (params (self2 :type "/Game/CORE/Blueprints/Pawn/NEW_Pawn Object Reference") (A :type "Object Object Reference"))
  (if (== A (`/Game/CORE/Blueprints/Pawn/NEW_Pawn.PuntoCienpies2` self2))
    (set `self.Punto1Cogido` false)
    (set `self.Punto2Cogido` false)))

(fn `ColisionContraPawn`
  (params (self2 :type "/Game/CORE/Blueprints/Pawn/NEW_Pawn Object Reference") (A :type "Object Object Reference") (self3 :type "/Game/CORE/Blueprints/Pawn/NEW_Pawn Object Reference"))
  (if (== A (`/Game/CORE/Blueprints/Pawn/NEW_Pawn.Collision` self2))
    (`/Game/CORE/Blueprints/Pawn/NEW_Pawn.PawnDie` self3 "")))

(fn `ColisionContraPuntocinpies`
  (params (self2 :type "/Game/CORE/Blueprints/Pawn/NEW_Pawn Object Reference") (self3 :type "/Game/CORE/Blueprints/Pawn/NEW_Pawn Object Reference") (B :type "Object Object Reference"))
  (if (== (`/Game/CORE/Blueprints/Pawn/NEW_Pawn.PuntoCienpies` self2) B)
    (set `self.Punto1Cogido` true)))

(fn `Destruir_Torso`
  (params (`UnionConSiguiente(Head)` :type "SceneComponent Object Reference") (Torso :type "PrimitiveComponent Object Reference") (Collision :type "PrimitiveComponent Object Reference") (Light :type "PrimitiveComponent Object Reference"))
  (`SceneComponent.SetVisibility` `UnionConSiguiente(Head)` false false)
  (`SceneComponent.SetVisibility` Torso false false)
  (`SceneComponent.SetVisibility` Collision false false)
  (`SceneComponent.SetVisibility` Light false false)
  (`GameplayStatics.SpawnEmitterAtLocation` "/Game/CORE/Particles/P_Die_Boss.P_Die_Boss" (`SceneComponent.K2_GetComponentLocation` Torso))
  (`ActorComponent.K2_DestroyComponent` Torso)
  (`ActorComponent.K2_DestroyComponent` Collision)
  (`ActorComponent.K2_DestroyComponent` Light))

(fn `Mover torso1`
  (params (B :type "Float (double-precision)"))
  (bind _head_01 (`self.Head_01`))
  (bind _returnvalue (- (`SceneComponent.K2_GetComponentLocation` _head_01) (`SceneComponent.K2_GetComponentLocation` (`self.Torso_02`))))
  (bind (_returnvalue_roll _returnvalue_pitch _returnvalue_yaw) (`KismetMathLibrary.BreakRotator` (`KismetMathLibrary.Conv_VectorToRotator` (* _returnvalue B))))
  (bind (_returnvalue_x _returnvalue_y) (`KismetMathLibrary.BreakVector` (* (`KismetMathLibrary.Normal` _returnvalue) (`self.MovementSpeed`))))
  ;[1 1 1] mover torso 1
  (if (not (`self.Torso_02_Destroyed`))
    (`/Engine/EditorBlueprintResources/StandardMacros.IsValid` _head_01
      (:`Is Valid`
        (if (not (`self.Blood`))
          (`SceneComponent.K2_SetWorldRotation` (`self.Torso_02`) (`KismetMathLibrary.MakeRotator` 0.0 0.0 _returnvalue_yaw) false false)
          (`SceneComponent.K2_AddRelativeLocation` (`self.Torso_02`) (`KismetMathLibrary.MakeVector` _returnvalue_x _returnvalue_y) false false))))))

(fn `Mover torso2`
  (params (InputPin :type "Float (double-precision)"))
  (bind _head_02 (`self.Head_02`))
  (bind _returnvalue (- (`SceneComponent.K2_GetComponentLocation` _head_02) (`SceneComponent.K2_GetComponentLocation` (`self.Torso_03`))))
  (bind (_returnvalue_roll _returnvalue_pitch _returnvalue_yaw) (`KismetMathLibrary.BreakRotator` (`KismetMathLibrary.Conv_VectorToRotator` (* _returnvalue InputPin))))
  (bind (_returnvalue_x _returnvalue_y) (`KismetMathLibrary.BreakVector` (* (`KismetMathLibrary.Normal` _returnvalue) (`self.MovementSpeed`))))
  ;[1 1 1] mover torso 2
  (if (not (`self.Torso_03_Destroyed`))
    (`/Engine/EditorBlueprintResources/StandardMacros.IsValid` _head_02
      (:`Is Valid`
        (if (not (`self.Blood`))
          (`SceneComponent.K2_SetWorldRotation` (`self.Torso_03`) (`KismetMathLibrary.MakeRotator` 0.0 0.0 _returnvalue_yaw) false false)
          (`SceneComponent.K2_AddRelativeLocation` (`self.Torso_03`) (`KismetMathLibrary.MakeVector` _returnvalue_x _returnvalue_y) false false))))))

(fn `mover torso3`
  (params (InputPin :type "Float (double-precision)"))
  (bind _head_03 (`self.Head_03`))
  (bind _returnvalue (- (`SceneComponent.K2_GetComponentLocation` _head_03) (`SceneComponent.K2_GetComponentLocation` (`self.Torso_04`))))
  (bind (_returnvalue_roll _returnvalue_pitch _returnvalue_yaw) (`KismetMathLibrary.BreakRotator` (`KismetMathLibrary.Conv_VectorToRotator` (* _returnvalue InputPin))))
  (bind (_returnvalue_x _returnvalue_y) (`KismetMathLibrary.BreakVector` (* (`KismetMathLibrary.Normal` _returnvalue) (`self.MovementSpeed`))))
  (if (not (`self.Torso_04_Destroyed`))
    (`/Engine/EditorBlueprintResources/StandardMacros.IsValid` _head_03
      (:`Is Valid`
        (if (not (`self.Blood`))
          (`SceneComponent.K2_SetWorldRotation` (`self.Torso_04`) (`KismetMathLibrary.MakeRotator` 0.0 0.0 _returnvalue_yaw) false false)
          (`SceneComponent.K2_AddRelativeLocation` (`self.Torso_04`) (`KismetMathLibrary.MakeVector` _returnvalue_x _returnvalue_y) false false))))))

(fn `mover torso4`
  (params (InputPin :type "Float (double-precision)"))
  (bind _head_04 (`self.Head_04`))
  (bind _returnvalue (- (`SceneComponent.K2_GetComponentLocation` _head_04) (`SceneComponent.K2_GetComponentLocation` (`self.Torso_05`))))
  (bind (_returnvalue_roll _returnvalue_pitch _returnvalue_yaw) (`KismetMathLibrary.BreakRotator` (`KismetMathLibrary.Conv_VectorToRotator` (* _returnvalue InputPin))))
  (bind (_returnvalue_x _returnvalue_y) (`KismetMathLibrary.BreakVector` (* (`KismetMathLibrary.Normal` _returnvalue) (`self.MovementSpeed`))))
  (if (not (`self.Torso_05_Destroyed`))
    (`/Engine/EditorBlueprintResources/StandardMacros.IsValid` _head_04
      (:`Is Valid`
        (if (not (`self.Blood`))
          (`SceneComponent.K2_SetWorldRotation` (`self.Torso_05`) (`KismetMathLibrary.MakeRotator` 0.0 0.0 _returnvalue_yaw) false false)
          (`SceneComponent.K2_AddRelativeLocation` (`self.Torso_05`) (`KismetMathLibrary.MakeVector` _returnvalue_x _returnvalue_y) false false))))))

(fn `mover torso5`
  (params (InputPin :type "Float (double-precision)"))
  (bind _head_05 (`self.head_05`))
  (bind _returnvalue (- (`SceneComponent.K2_GetComponentLocation` _head_05) (`SceneComponent.K2_GetComponentLocation` (`self.Torso_06`))))
  (bind (_returnvalue_roll _returnvalue_pitch _returnvalue_yaw) (`KismetMathLibrary.BreakRotator` (`KismetMathLibrary.Conv_VectorToRotator` (* _returnvalue InputPin))))
  (bind (_returnvalue_x _returnvalue_y) (`KismetMathLibrary.BreakVector` (* (`KismetMathLibrary.Normal` _returnvalue) (`self.MovementSpeed`))))
  (if (not (`self.Torso_06_Destroyed`))
    (`/Engine/EditorBlueprintResources/StandardMacros.IsValid` _head_05
      (:`Is Valid`
        (if (not (`self.Blood`))
          (`SceneComponent.K2_SetWorldRotation` (`self.Torso_06`) (`KismetMathLibrary.MakeRotator` 0.0 0.0 _returnvalue_yaw) false false)
          (`SceneComponent.K2_AddRelativeLocation` (`self.Torso_06`) (`KismetMathLibrary.MakeVector` _returnvalue_x _returnvalue_y) false false))))))

(fn `mover torso6`
  (params (InputPin :type "Float (double-precision)"))
  (bind _head_06 (`self.head_06`))
  (bind _returnvalue (- (`SceneComponent.K2_GetComponentLocation` _head_06) (`SceneComponent.K2_GetComponentLocation` (`self.Torso_07`))))
  (bind (_returnvalue_roll _returnvalue_pitch _returnvalue_yaw) (`KismetMathLibrary.BreakRotator` (`KismetMathLibrary.Conv_VectorToRotator` (* _returnvalue InputPin))))
  (bind (_returnvalue_x _returnvalue_y) (`KismetMathLibrary.BreakVector` (* (`KismetMathLibrary.Normal` _returnvalue) (`self.MovementSpeed`))))
  (if (not (`self.Torso_07_Destroyed`))
    (`/Engine/EditorBlueprintResources/StandardMacros.IsValid` _head_06
      (:`Is Valid`
        (if (not (`self.Blood`))
          (`SceneComponent.K2_SetWorldRotation` (`self.Torso_07`) (`KismetMathLibrary.MakeRotator` 0.0 0.0 _returnvalue_yaw) false false)
          (`SceneComponent.K2_AddRelativeLocation` (`self.Torso_07`) (`KismetMathLibrary.MakeVector` _returnvalue_x _returnvalue_y) false false))))))

(fn `mover torso7`
  (params (InputPin :type "Float (double-precision)"))
  (bind _head_07 (`self.head_07`))
  (bind _returnvalue (- (`SceneComponent.K2_GetComponentLocation` _head_07) (`SceneComponent.K2_GetComponentLocation` (`self.Torso_08`))))
  (bind (_returnvalue_roll _returnvalue_pitch _returnvalue_yaw) (`KismetMathLibrary.BreakRotator` (`KismetMathLibrary.Conv_VectorToRotator` (* _returnvalue InputPin))))
  (bind (_returnvalue_x _returnvalue_y) (`KismetMathLibrary.BreakVector` (* (`KismetMathLibrary.Normal` _returnvalue) (`self.MovementSpeed`))))
  (if (not (`self.Torso_08_Destroyed`))
    (`/Engine/EditorBlueprintResources/StandardMacros.IsValid` _head_07
      (:`Is Valid`
        (if (not (`self.Blood`))
          (`SceneComponent.K2_SetWorldRotation` (`self.Torso_08`) (`KismetMathLibrary.MakeRotator` 0.0 0.0 _returnvalue_yaw) false false)
          (`SceneComponent.K2_AddRelativeLocation` (`self.Torso_08`) (`KismetMathLibrary.MakeVector` _returnvalue_x _returnvalue_y) false false))))))

(fn `UserConstructionScript`)