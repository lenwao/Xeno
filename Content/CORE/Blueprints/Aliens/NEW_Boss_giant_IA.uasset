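; Giant boss alien for a shooter that takes bullet damage and kills the player pawn shortly after contact.
; Tick flip-flops a timeline forward and backward to sway both arms with random jitter, relying on an adjusted tick rate per the author's note.
; Zero health or BIgBossDie runs a one-time death: slow effect, blood and particles, pawn notification, scheduling BP_AreaSpawn's next event from game-mode time, then self-destruction.
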(event `self.ReceiveTick`
  (params (DeltaSeconds :type "Float (single-precision)"))
  ;[1 1 1] movimiento del brazo.(velocidad del tick tocada del even tick)
  (`/Engine/EditorBlueprintResources/StandardMacros.FlipFlop`
    (:`A`
      (bind (_direction _elevation _stepiz _stepder) (`Timeline|Timeline_0` :!via `PlayFromStart` :!label _label)
        (:`Update`
          (bind _returnvalue (+ _elevation (`KismetMathLibrary.RandomFloatInRange` -0.5 0.5)))
          (`SceneComponent.K2_SetRelativeLocation` (`self.SM_Regular_Arm_Der`) (`KismetMathLibrary.MakeVector` (+ _stepder (`KismetMathLibrary.RandomFloatInRange` -0.5 0.5)) 63.355705 _returnvalue) false false)
          (`SceneComponent.K2_SetRelativeLocation` (`self.SM_Regular_Arm_Iz`) (`KismetMathLibrary.MakeVector` (+ _stepiz (`KismetMathLibrary.RandomFloatInRange` -0.5 0.5)) -63.355705 _returnvalue) false false))))
    (:`B`
      (goto _label :!via `ReverseFromEnd`))))

(event `self.ReceiveBeginPlay`
  (bind _outactors (`GameplayStatics.GetAllActorsOfClass` "/Game/CORE/Blueprints/Pawn/NEW_Pawn.NEW_Pawn_C"))
  (set `self.Ref_Pawn` (`|GetArrayItem` _outactors)))

(event `BIgBossDie`
  (bind _torso (`self.Torso`))
  (bind _torso_2 (`self.Torso`))
  (bind (_returnvalue_x _returnvalue_y _returnvalue_z) (`KismetMathLibrary.BreakVector` (`SceneComponent.K2_GetComponentLocation` _torso)))
  (bind (_returnvalue_roll _returnvalue_pitch _returnvalue_yaw) (`KismetMathLibrary.BreakRotator` (`SceneComponent.K2_GetComponentRotation` _torso)))
  (bind (_returnvalue_x_2 _returnvalue_y_2) (`KismetMathLibrary.BreakVector` (/ (`SceneComponent.K2_GetComponentScale` _torso_2) 3)))
  (`/Engine/EditorBlueprintResources/StandardMacros.DoOnce` false :!label _label_2
    (:`Completed`
      ;[1 1 1] Slow Die
      (bind _outactors (`GameplayStatics.GetAllActorsOfClass` "/Game/CORE/Blueprints/Pawn/BP_AreaSpawn.BP_AreaSpawn_C"))
      (`/Game/CORE/Blueprints/Pawn/BP_AreaSpawn.Another Slow` (`|GetArrayItem` _outactors))
      (`|SpawnActorFromClass` "/Game/CORE/Blueprints/Sangre/NEW_Blood.NEW_Blood_C" (`KismetMathLibrary.MakeTransform` (`KismetMathLibrary.MakeVector` _returnvalue_x _returnvalue_y (- _returnvalue_z 20.0)) (`KismetMathLibrary.MakeRotator` _returnvalue_roll _returnvalue_pitch (+ _returnvalue_yaw 90.0)) (1.3 1.3 1.0)) "Undefined" "OverrideRootScale" null null)
      (`GameplayStatics.SpawnEmitterAtLocation` "/Game/CORE/Particles/P_Die_Boss.P_Die_Boss" (`SceneComponent.K2_GetComponentLocation` _torso_2) (struct) (`KismetMathLibrary.MakeVector` _returnvalue_x_2 _returnvalue_y_2 0.1))
      (`/Game/CORE/Blueprints/Pawn/NEW_Pawn.EVENT` (`self.Ref_Pawn`) "NEW_Boss_giant_IA_C")
      (bind _outactors_2 (`GameplayStatics.GetAllActorsOfClass` "/Game/CORE/Blueprints/Pawn/BP_AreaSpawn.BP_AreaSpawn_C"))
      (bind _asgm_shooter (cast `/Game/CORE/Blueprints/GM_Shooter` (`GameplayStatics.GetGameMode`)))
      (set `/Game/CORE/Blueprints/Pawn/BP_AreaSpawn.NextEventAtTime` (+ (`/Game/CORE/Blueprints/GM_Shooter.Time` _asgm_shooter) 26) (`|GetArrayItem` _outactors_2))
      (`self.K2_DestroyActor`))))

(event `self.Collision.OnComponentBeginOverlap`
  (params (OverlappedComponent :type "PrimitiveComponent Object Reference") (OtherActor :type "Actor Object Reference") (OtherComp :type "PrimitiveComponent Object Reference") (OtherBodyIndex :type Integer) (bFromSweep :type Boolean) (SweepResult :type "HitResult Structure (by ref)"))
  ;[1 1 1] Got Shot
  (bind _asbp_bullets (cast `/Game/CORE/Blueprints/Pawn/BP_Bullets` OtherActor)
    (:`then`
      (bind _output_get (set `self.Vida` (- (`self.Vida`) (`/Game/CORE/Blueprints/Pawn/BP_Bullets.Damage` _asbp_bullets))))
      (`/Game/CORE/Blueprints/Pawn/BP_Bullets.Hit` _asbp_bullets)
      (if (<= _output_get 0)
        (goto _label_2)))
    (:`CastFailed`
      ;[1 1 1] Kill Pawn by Proximity
      (bind _asnew_pawn (cast `/Game/CORE/Blueprints/Pawn/NEW_Pawn` OtherActor))
      (`KismetSystemLibrary.Delay` 0.2)
      (`/Engine/EditorBlueprintResources/StandardMacros.IsValid` _asnew_pawn
        (:`Is Valid`
          (`/Game/CORE/Blueprints/Pawn/NEW_Pawn.PawnDie` _asnew_pawn ""))))))

(fn `UserConstructionScript`)