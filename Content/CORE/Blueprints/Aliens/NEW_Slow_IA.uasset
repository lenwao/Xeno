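; Slow alien enemy character that loses health to player bullets and costs the player a life on contact unless they are blinking.
; Death from damage, wall overlap or straying too far shares one path: count the kill, notify BP_AreaSpawn, spawn effects, destroy.
; Radio overlap flags player proximity, turning the idle torso toward them and allowing a timed walk-speed change.
; A delayed Tick counter times that change and the distance-based death.
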(event `self.ReceiveBeginPlay`
  (bind _outactors (`GameplayStatics.GetAllActorsOfClass` "/Game/CORE/Blueprints/Pawn/NEW_Pawn.NEW_Pawn_C"))
  (set `self.Ref_Pawn` (`|GetArrayItem` _outactors))
  (bind _asgm_shooter (cast `/Game/CORE/Blueprints/GM_Shooter` (`GameplayStatics.GetGameMode`)))
  (set `self.refGM` _asgm_shooter)
  (`KismetSystemLibrary.Delay` 6.0)
  (set `self.Cerca?` true))

(event `self.CapsuleComponent.OnComponentBeginOverlap`
  (params (OverlappedComponent :type "PrimitiveComponent Object Reference") (OtherActor :type "Actor Object Reference") (OtherComp :type "PrimitiveComponent Object Reference") (OtherBodyIndex :type Integer) (bFromSweep :type Boolean) (SweepResult :type "HitResult Structure (by ref)"))
  (if (`ActorComponent.ComponentHasTag` OtherComp "MURO")
    (`self.SlowDie`)))

(event `self.SM_Collision.OnComponentBeginOverlap`
  (params (OverlappedComponent :type "PrimitiveComponent Object Reference") (OtherActor :type "Actor Object Reference") (OtherComp :type "PrimitiveComponent Object Reference") (OtherBodyIndex :type Integer) (bFromSweep :type Boolean) (SweepResult :type "HitResult Structure (by ref)"))
  (bind _ref_pawn (`self.Ref_Pawn`))
  (bind _refgm (`self.refGM`))
  (bind _returnvalue (`SceneComponent.K2_GetComponentLocation` (`self.SM_Slow_Torso`)))
  (`|ExecutionSequence`
    (:`then_0`
      (bind _asbp_bullets (cast `/Game/CORE/Blueprints/Pawn/BP_Bullets` OtherActor)
        (:`then`
          (`/Game/CORE/Blueprints/Pawn/BP_Bullets.Hit` _asbp_bullets)
          (bind _output_get (set `self.Vida` (- (`self.Vida`) (`/Game/CORE/Blueprints/Pawn/NEW_Pawn.Damage` (`self.Ref_Pawn`)))))
          (if (<= _output_get 0)
            (`/Engine/EditorBlueprintResources/StandardMacros.DoOnce` false :!label _label
              (:`Completed`
                (bind _result (`/Engine/EditorBlueprintResources/StandardMacros.IncrementInt` (`/Game/CORE/Blueprints/GM_Shooter.#SlowKill` _refgm))
                  (:`  `
                    (set `/Game/CORE/Blueprints/GM_Shooter.#SlowKill` _result _refgm)
                    (bind _outactors (`GameplayStatics.GetAllActorsOfClass` "/Game/CORE/Blueprints/Pawn/BP_AreaSpawn.BP_AreaSpawn_C"))
                    (`/Game/CORE/Blueprints/Pawn/BP_AreaSpawn.Another Slow` (`|GetArrayItem` _outactors))
                    (`|SpawnActorFromClass` "/Game/CORE/Blueprints/Sangre/NEW_Blood.NEW_Blood_C" (`KismetMathLibrary.MakeTransform` _returnvalue (struct) (1.2 1.2 1.0)) "Undefined" "OverrideRootScale" null null)
                    (`GameplayStatics.SpawnEmitterAtLocation` "/Game/CORE/Particles/P_Die_Slow.P_Die_Slow" _returnvalue)
                    (`self.K2_DestroyActor`)))))))
        (:`CastFailed`
          (bind _asnew_pawn (cast `/Game/CORE/Blueprints/Pawn/NEW_Pawn` OtherActor))
          (`/Engine/EditorBlueprintResources/StandardMacros.DoOnce` false
            (:`Completed`
              (if (not (`/Game/CORE/Blueprints/Pawn/NEW_Pawn.Parpadeante` _ref_pawn))
                (bind _output_get_2 (set `/Game/CORE/Blueprints/Pawn/NEW_Pawn.Vidas` (- (`/Game/CORE/Blueprints/Pawn/NEW_Pawn.Vidas` _ref_pawn) 1) _ref_pawn))
                (if (<= _output_get_2 0)
                  (`/Game/CORE/Blueprints/Pawn/NEW_Pawn.PawnDie` _asnew_pawn (`KismetSystemLibrary.GetDisplayName` self)))))))))))

(event `SlowDie`
  (goto _label))

(event `self.ReceiveTick`
  (params (DeltaSeconds :type "Float (single-precision)"))
  (bind _time (`self.time`))
  (`|ExecutionSequence`
    (:`then_0`
      (if (`self.Cerca?`)
        (if (>= (`self.GetDistanceTo` self (`self.Ref_Pawn`)) 850.0)
          (if (>= (`self.time`) 5)
            (`/Engine/EditorBlueprintResources/StandardMacros.IsValid` self
              (:`Is Valid`
                (goto _label)))))))
    (:`then_1`
      (`KismetSystemLibrary.Delay` 1.0)
      (bind _result (`/Engine/EditorBlueprintResources/StandardMacros.IncrementInt` _time)
        (:`  `
          (set `self.time` _result)
          (if (== _time 11)
            (if (`self.RadioActivo`)
              (set `CharacterMovementComponent.MaxWalkSpeed` 350.0 (`self.CharacterMovement`)))))))
    (:`then_2`
      (if (`self.RadioActivo`)
        (if (<= (`KismetMathLibrary.VSize` (`self.GetVelocity`)) 0.0)
          (`SceneComponent.K2_SetWorldRotation` (`self.SM_Slow_Torso`) (`KismetMathLibrary.FindLookAtRotation` (`SceneComponent.K2_GetComponentLocation` (`self.SM_Slow_Torso`)) (`SceneComponent.K2_GetComponentLocation` (`/Game/CORE/Blueprints/Pawn/NEW_Pawn.SM_Torso` (`self.Ref_Pawn`)))) false false))))))

(event `self.Radio.OnComponentBeginOverlap`
  (params (OverlappedComponent :type "PrimitiveComponent Object Reference") (OtherActor :type "Actor Object Reference") (OtherComp :type "PrimitiveComponent Object Reference") (OtherBodyIndex :type Integer) (bFromSweep :type Boolean) (SweepResult :type "HitResult Structure (by ref)"))
  (cast `/Game/CORE/Blueprints/Pawn/NEW_Pawn` OtherActor)
  (set `self.RadioActivo` true))

(event `self.Radio.OnComponentEndOverlap`
  (params (OverlappedComponent :type "PrimitiveComponent Object Reference") (OtherActor :type "Actor Object Reference") (OtherComp :type "PrimitiveComponent Object Reference") (OtherBodyIndex :type Integer))
  (cast `/Game/CORE/Blueprints/Pawn/NEW_Pawn` OtherActor)
  (set `self.RadioActivo` false))

(fn `UserConstructionScript`)