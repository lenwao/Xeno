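; BP_ElBolas is a boss alien that turns its torso toward the player's NEW_Pawn and periodically fires BP_Bola actors.
; A looping timer spawns staggered pairs of balls from two fire points.
; Collision overlaps kill the pawn on contact, while bullet hits subtract the pawn's damage from Vida.
; At zero Vida it spawns blood and particles, notifies the pawn, clears BossSpawn on BP_AreaSpawn and destroys itself.
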(event `Bolitas`
  (`KismetSystemLibrary.K2_SetTimerDelegate` (delegate `Bolitas`) 6.0 true)
  (`|ExecutionSequence`
    (:`then_0`
      (`|SpawnActorFromClass` "/Game/CORE/Blueprints/Aliens/BP_Bola.BP_Bola_C" (`KismetMathLibrary.MakeTransform` (`SceneComponent.K2_GetComponentLocation` (`self.PuntoDisparo2`))) "Undefined" "OverrideRootScale" null null)
      (`KismetSystemLibrary.Delay` 0.5)
      (`|SpawnActorFromClass` "/Game/CORE/Blueprints/Aliens/BP_Bola.BP_Bola_C" (`KismetMathLibrary.MakeTransform` (`SceneComponent.K2_GetComponentLocation` (`self.PuntoDisparo2`))) "Undefined" "OverrideRootScale" null null))
    (:`then_1`
      (`|SpawnActorFromClass` "/Game/CORE/Blueprints/Aliens/BP_Bola.BP_Bola_C" (`KismetMathLibrary.MakeTransform` (`SceneComponent.K2_GetComponentLocation` (`self.PuntoDisparo`))) "Undefined" "OverrideRootScale" null null)
      (`KismetSystemLibrary.Delay` 0.5)
      (`|SpawnActorFromClass` "/Game/CORE/Blueprints/Aliens/BP_Bola.BP_Bola_C" (`KismetMathLibrary.MakeTransform` (`SceneComponent.K2_GetComponentLocation` (`self.PuntoDisparo`))) "Undefined" "OverrideRootScale" null null))))

(event `self.ReceiveBeginPlay`
  (`KismetSystemLibrary.PrintString` (`KismetStringLibrary.Conv_NameToString` (`self.Type`)))
  (bind _outactors (`GameplayStatics.GetAllActorsOfClass` "/Game/CORE/Blueprints/Pawn/NEW_Pawn.NEW_Pawn_C"))
  (set `self.Pawn` (`|GetArrayItem` _outactors))
  (`KismetSystemLibrary.Delay` 0.2)
  (`self.Bolitas`))

(event `self.ReceiveTick`
  (params (DeltaSeconds :type "Float (single-precision)"))
  (bind _sm_torso (`/Game/CORE/Blueprints/Pawn/NEW_Pawn.SM_Torso` (`self.Pawn`)))
  ;[1 1 1] Movement and Rotation
  (`/Engine/EditorBlueprintResources/StandardMacros.IsValid` _sm_torso
    (:`Is Valid`
      (`SceneComponent.K2_SetWorldRotation` (`self.Torso`) (`KismetMathLibrary.Conv_VectorToRotator` (* (- (`SceneComponent.K2_GetComponentLocation` _sm_torso) (`SceneComponent.K2_GetComponentLocation` (`self.Torso`))) DeltaSeconds)) false false))))

(event `self.Collision.OnComponentBeginOverlap`
  (params (OverlappedComponent :type "PrimitiveComponent Object Reference") (OtherActor :type "Actor Object Reference") (OtherComp :type "PrimitiveComponent Object Reference") (OtherBodyIndex :type Integer) (bFromSweep :type Boolean) (SweepResult :type "HitResult Structure (by ref)"))
  (bind _torso (`self.Torso`))
  (bind _returnvalue (`SceneComponent.K2_GetComponentLocation` _torso))
  (bind (_returnvalue_roll _returnvalue_pitch _returnvalue_yaw) (`KismetMathLibrary.BreakRotator` (`SceneComponent.K2_GetComponentRotation` _torso)))
  ;[1 1 1] Kill Pawn by Proximity
  (`|ExecutionSequence`
    (:`then_0`
      (bind _asnew_pawn (cast `/Game/CORE/Blueprints/Pawn/NEW_Pawn` OtherActor))
      (`/Game/CORE/Blueprints/Pawn/NEW_Pawn.PawnDie` _asnew_pawn ""))
    (:`then_1`
      ;[1 1 1] Got Shot
      (bind _asbp_bullets (cast `/Game/CORE/Blueprints/Pawn/BP_Bullets` OtherActor))
      (`/Game/CORE/Blueprints/Pawn/BP_Bullets.Hit` _asbp_bullets)
      (bind _output_get (set `self.Vida` (- (`self.Vida`) (`/Game/CORE/Blueprints/Pawn/NEW_Pawn.Damage` (`self.Pawn`)))))
      ;[1 1 1] Slow Die
      (`KismetSystemLibrary.PrintString` (`KismetStringLibrary.Conv_IntToString` _output_get))
      (if (<= (`self.Vida`) 0)
        (`|SpawnActorFromClass` "/Game/CORE/Blueprints/Sangre/NEW_Blood.NEW_Blood_C" (`KismetMathLibrary.MakeTransform` _returnvalue (`KismetMathLibrary.MakeRotator` _returnvalue_roll _returnvalue_pitch (+ _returnvalue_yaw 90.0)) (1.5 1.5 1.0)) "Undefined" "OverrideRootScale" null null)
        (`GameplayStatics.SpawnEmitterAtLocation` "/Game/CORE/Particles/P_Die_Boss.P_Die_Boss" _returnvalue)
        (`/Game/CORE/Blueprints/Pawn/NEW_Pawn.EVENT` (`self.Pawn`) "BP_ElBolas_C")
        (bind _outactors (`GameplayStatics.GetAllActorsOfClass` "/Game/CORE/Blueprints/Pawn/BP_AreaSpawn.BP_AreaSpawn_C"))
        (set `/Game/CORE/Blueprints/Pawn/BP_AreaSpawn.BossSpawn` false (`|GetArrayItem` _outactors))
        (`self.K2_DestroyActor`)))))

(fn `UserConstructionScript`)