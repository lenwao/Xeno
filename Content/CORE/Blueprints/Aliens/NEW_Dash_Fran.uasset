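; Dashing alien enemy that chases the player pawn, kills it on contact and kills slow aliens while dashing.
; Tick approaches until close, then locks aim and, after delays, drives jittered timeline dashes that spawn splashes.
; Bullets spark off its body, and only rear hits reduce health.
; Death or touching a MURO-tagged wall, which triggers a scale-driven fall, calls AnotherDash on BP_AreaSpawn.
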(event `self.DashCube.OnComponentBeginOverlap`
  (params (OverlappedComponent :type "PrimitiveComponent Object Reference") (OtherActor :type "Actor Object Reference") (OtherComp :type "PrimitiveComponent Object Reference") (OtherBodyIndex :type Integer) (bFromSweep :type Boolean) (SweepResult :type "HitResult Structure (by ref)")))

(event `self.ReceiveBeginPlay`
  (bind _outactors (`GameplayStatics.GetAllActorsOfClass` "/Game/CORE/Blueprints/Pawn/NEW_Pawn.NEW_Pawn_C"))
  (set `self.Ref_Pawn` (`|GetArrayItem` _outactors))
  (bind _asgm_shooter (cast `/Game/CORE/Blueprints/GM_Shooter` (`GameplayStatics.GetGameMode`)))
  (set `self.Ref_GM` _asgm_shooter))

(event `ResetAim`
  (`/Engine/EditorBlueprintResources/StandardMacros.DoOnce` false :!via `Reset`
    (:`Completed`
      (set `self.Aim` true))))

(event `ResetDashes`
  (goto _label_2 :!via `Reset`))

(event `self.ReceiveTick`
  (params (DeltaSeconds :type "Float (single-precision)"))
  (bind _returnvalue (- (`SceneComponent.K2_GetComponentLocation` (`/Game/CORE/Blueprints/Pawn/NEW_Pawn.SM_Torso` (`self.Ref_Pawn`))) (`SceneComponent.K2_GetComponentLocation` (`self.Torso`))))
  (bind _returnvalue_2 (* (- (`SceneComponent.K2_GetComponentLocation` (`/Game/CORE/Blueprints/Pawn/NEW_Pawn.SM_Torso` (`self.Ref_Pawn`))) (`SceneComponent.K2_GetComponentLocation` (`self.Torso`))) DeltaSeconds))
  (bind (_returnvalue_roll _returnvalue_pitch _returnvalue_yaw) (`KismetMathLibrary.BreakRotator` (`KismetMathLibrary.Conv_VectorToRotator` (* _returnvalue DeltaSeconds))))
  (bind (_returnvalue_roll_2 _returnvalue_pitch_2 _returnvalue_yaw_2) (`KismetMathLibrary.BreakRotator` (`KismetMathLibrary.Conv_VectorToRotator` _returnvalue_2)))
  (`|ExecutionSequence`
    (:`then_0`
      (if (`self.Aim`)
        (if (`self.Dashea`) :!label _label
          (`/Engine/EditorBlueprintResources/StandardMacros.DoOnce` false :!label _label_2
            (:`Completed`
              (bind (_direction _newtrack_0) (`Timeline|Timeline_0` :!via `PlayFromStart`)
                (:`Update`
                  (bind (_returnvalue_x _returnvalue_y) (`KismetMathLibrary.BreakVector` (* (`KismetMathLibrary.Normal` (`self.Locked_To_Pawn`)) (/ (`self.DashLength`) (`KismetMathLibrary.FTrunc` _newtrack_0)))))
                  (`SceneComponent.K2_AddRelativeLocation` (`self.CapsuleComponent`) (`KismetMathLibrary.MakeVector` (+ _returnvalue_x (`KismetMathLibrary.RandomFloatInRange` -3.0 3.0)) (+ _returnvalue_y (`KismetMathLibrary.RandomFloatInRange` -3.0 3.0))) false false)
                  (if (not (`self.STOPSPLASH`))
                    (`|SpawnActorFromClass` "/Game/CORE/Blueprints/Sangre/BP_Dash_Splash.BP_Dash_Splash_C" (`KismetMathLibrary.Conv_VectorToTransform` (`SceneComponent.K2_GetComponentLocation` (`self.Torso`))) "DontSpawnIfColliding" "OverrideRootScale" self null)))
                (:`Finished`
                  (`KismetSystemLibrary.Delay` (`self.Delay_Post_Dash`))
                  (set `self.Dashea` false)
                  (bind _result (`/Engine/EditorBlueprintResources/StandardMacros.IncrementInt` (`self.#Times`))
                    (:`  `
                      (bind _output_get (set `self.#Times` _result))
                      (if (>= _output_get 3)
                        (set `self.Aim` false)
                        (set `self.#Times` 0)
                        (`self.ResetDashes`)
                        (else
                          (`self.ResetDashes`)))))))))
          (elif (`self.Locked`)
            (`KismetSystemLibrary.Delay` (`self.Delay_Pre_Dash`))
            (set `self.Dashea` true)
            (set `self.Locked` false)
            (else
              (`SceneComponent.K2_SetWorldRotation` (`self.Torso`) (`KismetMathLibrary.MakeRotator` _returnvalue_roll_2 _returnvalue_pitch_2 (+ _returnvalue_yaw_2 90.0)) false false)
              (`KismetSystemLibrary.Delay` (`self.Aim_delay`))
              (set `self.Locked_To_Pawn` _returnvalue_2)
              (set `self.Locked` true))))
        (elif (>= (`self.GetDistanceTo` (`self.Ref_Pawn`)) 300.0)
          (`SceneComponent.K2_SetWorldRotation` (`self.Torso`) (`KismetMathLibrary.MakeRotator` _returnvalue_roll _returnvalue_pitch (+ _returnvalue_yaw 90.0)) false false)
          (`SceneComponent.K2_AddRelativeLocation` (`self.CapsuleComponent`) (* (`KismetMathLibrary.Normal` _returnvalue 1e-06) (`self.MovementSpeed`)) false false)
          (else
            (goto _label)))))
    (:`then_1`
      (if (`self.IsOverlappingActor` (`self.Ref_Pawn`))
        (set `self.Aim` true)))))

(event `self.parteTrasera.OnComponentBeginOverlap`
  (params (OverlappedComponent :type "PrimitiveComponent Object Reference") (OtherActor :type "Actor Object Reference") (OtherComp :type "PrimitiveComponent Object Reference") (OtherBodyIndex :type Integer) (bFromSweep :type Boolean) (SweepResult :type "HitResult Structure (by ref)"))
  (bind _returnvalue (`SceneComponent.K2_GetComponentLocation` (`self.Torso`)))
  ;[1 1 1] Got Shot
  (bind _asbp_bullets (cast `/Game/CORE/Blueprints/Pawn/BP_Bullets` OtherActor))
  (`self.K2_DestroyActor` _asbp_bullets)
  (bind _result (`/Engine/EditorBlueprintResources/StandardMacros.DecrementInt` (`self.Vida`))
    (:`  `
      (bind _output_get (set `self.Vida` _result))
      (if (<= _output_get 0)
        (`GameplayStatics.SpawnEmitterAtLocation` "/Game/CORE/Particles/P_Die_Boss.P_Die_Boss" _returnvalue (struct) (1.6 1.6 1.0))
        (`|SpawnActorFromClass` "/Game/CORE/Blueprints/Sangre/NEW_Blood.NEW_Blood_C" (`KismetMathLibrary.MakeTransform` _returnvalue (struct) (2.0 2.0 1.0)) "Undefined" "OverrideRootScale" null null)
        (bind _outactors (`GameplayStatics.GetAllActorsOfClass` "/Game/CORE/Blueprints/Pawn/BP_AreaSpawn.BP_AreaSpawn_C"))
        (`/Game/CORE/Blueprints/Pawn/BP_AreaSpawn.Another Dash` (`|GetArrayItem` _outactors))
        (`self.K2_DestroyActor`)))))

(event `self.Collision.OnComponentBeginOverlap`
  (params (OverlappedComponent :type "PrimitiveComponent Object Reference") (OtherActor :type "Actor Object Reference") (OtherComp :type "PrimitiveComponent Object Reference") (OtherBodyIndex :type Integer) (bFromSweep :type Boolean) (SweepResult :type "HitResult Structure (by ref)"))
  ;[1 1 1] Kill Pawn by Proximity
  (`|ExecutionSequence`
    (:`then_0`
      (bind _asnew_slow_ia (cast `/Game/CORE/Blueprints/Aliens/NEW_Slow_IA` OtherActor)
        (:`then`
          (if (`self.Dashea`)
            (`/Game/CORE/Blueprints/Aliens/NEW_Slow_IA.SlowDie` _asnew_slow_ia)))
        (:`CastFailed`
          (bind _asnew_pawn (cast `/Game/CORE/Blueprints/Pawn/NEW_Pawn` OtherActor)
            (:`then`
              (`/Game/CORE/Blueprints/Pawn/NEW_Pawn.PawnDie` _asnew_pawn ""))
            (:`CastFailed`
              (bind _asbp_bullets (cast `/Game/CORE/Blueprints/Pawn/BP_Bullets` OtherActor))
              (if (`/Game/CORE/Blueprints/GM_Shooter.SoundOn?` (`self.Ref_GM`))
                (`GameplayStatics.PlaySound2D` "/Game/CORE/Audio/metalsound.metalsound" 1.0 (`KismetMathLibrary.RandomFloatInRange` 0.0 1.0) 0.0 null null))
              (bind (_returnvalue_x _returnvalue_y _returnvalue_z) (`KismetMathLibrary.BreakVector` (`SceneComponent.K2_GetComponentLocation` (`/Game/CORE/Blueprints/Pawn/BP_Bullets.Plane` _asbp_bullets))))
              (`GameplayStatics.SpawnEmitterAtLocation` "/Game/CORE/Particles/P_Hit_Sparks.P_Hit_Sparks" (`KismetMathLibrary.MakeVector` _returnvalue_x _returnvalue_y _returnvalue_z) (struct) (0.5 0.5 0.5))
              (`self.K2_DestroyActor` _asbp_bullets))))))
    (:`then_1`
      (if (`ActorComponent.ComponentHasTag` OtherComp "MURO")
        (set `self.FallPoint` (`self.K2_GetActorLocation`))
        (bind (_direction _caida) (`Timeline|Timeline_1`)
          (:`Update`
            (set `self.STOPSPLASH` true)
            (`self.K2_SetActorTransform` (`KismetMathLibrary.MakeTransform` (`self.FallPoint`) (struct) (`KismetMathLibrary.Conv_DoubleToVector` _caida)))
            (bind _outactors (`GameplayStatics.GetAllActorsOfClass` "/Game/CORE/Blueprints/Pawn/BP_AreaSpawn.BP_AreaSpawn_C"))
            (`/Game/CORE/Blueprints/Pawn/BP_AreaSpawn.Another Dash` (`|GetArrayItem` _outactors)))
          (:`Finished`
            (`self.K2_DestroyActor`)))))))

(fn `UserConstructionScript`)