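; Boss alien that kills the player pawn on contact and is protected by a regenerating shield barrier.
; Bullets hitting GrabSphere, or danorayo calls, add flat wounds (Heridas), changing walk speed at a threshold and eventually killing it.
; Barrera absorbs bullets using per-weapon DataTable damage, switches off briefly when depleted, then restores.
; Death spawns an effect, notifies the pawn and schedules BP_AreaSpawn's next event from GM_Shooter's time.
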(event `self.ReceiveBeginPlay`
  (bind _outactors (`GameplayStatics.GetAllActorsOfClass` "/Game/CORE/Blueprints/Pawn/NEW_Pawn.NEW_Pawn_C"))
  (set `self.Ref_Pawn` (`|GetArrayItem` _outactors)))

(event `self.GrabSphere.OnComponentBeginOverlap`
  (params (OverlappedComponent :type "PrimitiveComponent Object Reference") (OtherActor :type "Actor Object Reference") (OtherComp :type "PrimitiveComponent Object Reference") (OtherBodyIndex :type Integer) (bFromSweep :type Boolean) (SweepResult :type "HitResult Structure (by ref)"))
  (bind _heridas (`self.Heridas`))
  ;[1 1 1] Kill Pawn by Proximity
  (`|ExecutionSequence`
    (:`then_0`
      (bind _asnew_pawn (cast `/Game/CORE/Blueprints/Pawn/NEW_Pawn` OtherActor))
      (`/Game/CORE/Blueprints/Pawn/NEW_Pawn.PawnDie` _asnew_pawn ""))
    (:`then_1`
      ;[1 1 1] Got Shot
      (bind _asbp_bullets (cast `/Game/CORE/Blueprints/Pawn/BP_Bullets` OtherActor))
      ;[1 1 1] Slow Die
      (`self.K2_DestroyActor` _asbp_bullets)
      (`/Engine/EditorBlueprintResources/StandardMacros.IncrementInt` _heridas :!label _label
        (:`  `
          (if (== _heridas 20)
            (`GameplayStatics.SpawnEmitterAtLocation` "/Game/CORE/Particles/P_Die_Boss.P_Die_Boss" (`SceneComponent.K2_GetComponentLocation` (`self.Torso`)) (struct) (1.5 1.5 1.0))
            (`/Game/CORE/Blueprints/Pawn/NEW_Pawn.EVENT` (`self.Ref_Pawn`) "BP_BossWao_IA_C")
            (bind _outactors (`GameplayStatics.GetAllActorsOfClass` "/Game/CORE/Blueprints/Pawn/BP_AreaSpawn.BP_AreaSpawn_C"))
            (bind _asgm_shooter (cast `/Game/CORE/Blueprints/GM_Shooter` (`GameplayStatics.GetGameMode`)))
            (set `/Game/CORE/Blueprints/Pawn/BP_AreaSpawn.NextEventAtTime` (+ (`/Game/CORE/Blueprints/GM_Shooter.Time` _asgm_shooter) 26) (`|GetArrayItem` _outactors))
            (`self.K2_DestroyActor`)
            (elif (== _heridas 14)
              (set `CharacterMovementComponent.MaxWalkSpeed` 450.0 (`self.CharacterMovement`)))))))))

(event `danorayo`
  ;[1 1 1] Slow Die
  (goto _label))

(event `self.Barrera.OnComponentBeginOverlap`
  (params (OverlappedComponent :type "PrimitiveComponent Object Reference") (OtherActor :type "Actor Object Reference") (OtherComp :type "PrimitiveComponent Object Reference") (OtherBodyIndex :type Integer) (bFromSweep :type Boolean) (SweepResult :type "HitResult Structure (by ref)"))
  (bind _heridasescudo (`self.HeridasEscudo`))
  (bind _barrera (`self.Barrera`))
  (bind _barrera_2 (`self.Barrera`))
  (`|ExecutionSequence`
    (:`then_0`
      (bind _asnew_pawn (cast `/Game/CORE/Blueprints/Pawn/NEW_Pawn` OtherActor))
      (`/Game/CORE/Blueprints/Pawn/NEW_Pawn.PawnDie` _asnew_pawn ""))
    (:`then_1`
      (bind _asbp_bullets (cast `/Game/CORE/Blueprints/Pawn/BP_Bullets` OtherActor))
      (`self.K2_DestroyActor` _asbp_bullets)
      (bind _returnvalue (`|GetDataTableRow` "/Game/CORE/Blueprints/DataTable_Bullets.DataTable_Bullets" (`/Game/CORE/Blueprints/Pawn/NEW_Pawn.Weapon` (`self.Ref_Pawn`)))
        (:`then`
          (set `self.HeridasEscudo` (- _heridasescudo (`.Damage_9_BDD6E2AC4207F3E6B04BD08945F5EBC7` (break `/Game/CORE/Blueprints/Struct_Bullets` _returnvalue))))
          (if (<= _heridasescudo 0)
            (`PrimitiveComponent.SetCollisionEnabled` _barrera_2 "NoCollision")
            (`SceneComponent.SetVisibility` _barrera_2 false false)
            (`SceneComponent.SetVisibility` (`self.Plane`) false false)
            (`KismetSystemLibrary.Delay` 2.5)
            (`PrimitiveComponent.SetCollisionEnabled` _barrera "QueryAndPhysics")
            (`SceneComponent.SetVisibility` _barrera true false)
            (`SceneComponent.SetVisibility` (`self.Plane`) true false)
            (set `self.HeridasEscudo` 10)))))))

(fn `UserConstructionScript`)