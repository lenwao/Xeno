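; BP_Dash_Humo is a short-lived dash smoke actor from the Aliens folder that slows any NEW_Pawn entering its Cube volume.
; On overlap it lowers that pawn's MovementSpeed2, then after a delay restores the speed of the cached first player pawn, not necessarily the overlapping one.
; BeginPlay caches that pawn, waits a few seconds, restores its speed if still slowed, and destroys the actor.
; End overlap does nothing.
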(event `self.ReceiveBeginPlay`
  (bind _asnew_pawn (cast `/Game/CORE/Blueprints/Pawn/NEW_Pawn` (`GameplayStatics.GetPlayerPawn` 0)))
  (set `self.Ref Pawn` _asnew_pawn)
  (`KismetSystemLibrary.Delay` 3.0)
  (if (<= (`/Game/CORE/Blueprints/Pawn/NEW_Pawn.MovementSpeed2` (`self.Ref Pawn`)) 300.0)
    (set `/Game/CORE/Blueprints/Pawn/NEW_Pawn.MovementSpeed2` 500.0 (`self.Ref Pawn`))
    (`self.K2_DestroyActor`)
    (else
      (`self.K2_DestroyActor`))))

(event `self.Cube.OnComponentBeginOverlap`
  (params (OverlappedComponent :type "PrimitiveComponent Object Reference") (OtherActor :type "Actor Object Reference") (OtherComp :type "PrimitiveComponent Object Reference") (OtherBodyIndex :type Integer) (bFromSweep :type Boolean) (SweepResult :type "HitResult Structure (by ref)"))
  (bind _ref_pawn (`self.Ref Pawn`))
  (bind _asnew_pawn (cast `/Game/CORE/Blueprints/Pawn/NEW_Pawn` OtherActor))
  (set `/Game/CORE/Blueprints/Pawn/NEW_Pawn.MovementSpeed2` 300.0 _asnew_pawn)
  (`KismetSystemLibrary.Delay` 1.0)
  (`/Engine/EditorBlueprintResources/StandardMacros.IsValid` _ref_pawn
    (:`Is Valid`
      (set `/Game/CORE/Blueprints/Pawn/NEW_Pawn.MovementSpeed2` 500.0 _ref_pawn))
    (:`Is Not Valid`
      (set `/Game/CORE/Blueprints/Pawn/NEW_Pawn.MovementSpeed2` 500.0 _ref_pawn))))

(event `self.Cube.OnComponentEndOverlap`
  (params (OverlappedComponent :type "PrimitiveComponent Object Reference") (OtherActor :type "Actor Object Reference") (OtherComp :type "PrimitiveComponent Object Reference") (OtherBodyIndex :type Integer)))

(fn `UserConstructionScript`)