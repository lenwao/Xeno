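; BP_BossWaoHijo is a minion of the Wao boss that kills the player pawn on overlap with its GrabSphere.
; Each tick its Torso turns to face the player and moves toward one of three boss anchor points, chosen by NumeroHijo.
; Bullet overlaps or SlowDie add wounds; the third hides it and disables collision briefly before it revives, while Muerte destroys it outright.
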(event `self.ReceiveBeginPlay`
  (bind _outactors (`GameplayStatics.GetAllActorsOfClass` "/Game/CORE/Blueprints/Pawn/NEW_Pawn.NEW_Pawn_C"))
  (set `self.Ref_Pawn` (`|GetArrayItem` _outactors))
  (bind _outactors_2 (`GameplayStatics.GetAllActorsOfClass` "/Game/CORE/FALTA/BP_BossWao_IA.BP_BossWao_IA_C"))
  (set `self.boss wao` (`|GetArrayItem` _outactors_2)))

(event `self.ReceiveTick`
  (params (DeltaSeconds :type "Float (single-precision)"))
  (bind _boss_wao (`self.boss wao`))
  (bind _numerohijo (`self.NumeroHijo`))
  (bind _returnvalue (`SceneComponent.K2_GetComponentLocation` (`self.Torso`)))
  (bind _sm_torso (`/Game/CORE/Blueprints/Pawn/NEW_Pawn.SM_Torso` (`self.Ref_Pawn`)))
  ;[1 1 1] Movement and Rotation
  (`/Engine/EditorBlueprintResources/StandardMacros.IsValid` _sm_torso
    (:`Is Valid`
      (`SceneComponent.K2_SetWorldRotation` (`self.Torso`) (`KismetMathLibrary.Conv_VectorToRotator` (* (- (`SceneComponent.K2_GetComponentLocation` _sm_torso) _returnvalue) DeltaSeconds)) false false)
      (if (== _numerohijo 0)
        (`SceneComponent.K2_AddRelativeLocation` (`self.Torso`) (* (`KismetMathLibrary.Normal` (- (`SceneComponent.K2_GetComponentLocation` (`/Game/CORE/FALTA/BP_BossWao_IA.Hijo1Sitio` _boss_wao)) _returnvalue)) (`self.MovementSpeed`)) false false)
        (elif (== _numerohijo 1)
          (`SceneComponent.K2_AddRelativeLocation` (`self.Torso`) (* (`KismetMathLibrary.Normal` (- (`SceneComponent.K2_GetComponentLocation` (`/Game/CORE/FALTA/BP_BossWao_IA.Hijo2Sitio` _boss_wao)) _returnvalue)) (`self.MovementSpeed`)) false false)
          (elif (== _numerohijo 2)
            (`SceneComponent.K2_AddRelativeLocation` (`self.Torso`) (* (`KismetMathLibrary.Normal` (- (`SceneComponent.K2_GetComponentLocation` (`/Game/CORE/FALTA/BP_BossWao_IA.Hijo3Stio` _boss_wao)) _returnvalue)) (`self.MovementSpeed`)) false false)))))))

(event `Muerte`
  (`self.K2_DestroyActor`))

(event `self.GrabSphere.OnComponentBeginOverlap`
  (params (OverlappedComponent :type "PrimitiveComponent Object Reference") (OtherActor :type "Actor Object Reference") (OtherComp :type "PrimitiveComponent Object Reference") (OtherBodyIndex :type Integer) (bFromSweep :type Boolean) (SweepResult :type "HitResult Structure (by ref)"))
  (bind _grabsphere (`self.GrabSphere`))
  (bind _heridas (`self.Heridas`))
  ;[1 1 1] Kill Pawn by Proximity
  (`|ExecutionSequence`
    (:`then_0`
      (bind _asnew_pawn (cast `/Game/CORE/Blueprints/Pawn/NEW_Pawn` OtherActor))
      (`/Game/CORE/Blueprints/Pawn/NEW_Pawn.PawnDie` _asnew_pawn ""))
    (:`then_1`
      ;[1 1 1] Got Shot
      (cast `/Game/CORE/Blueprints/Pawn/BP_Bullets` OtherActor)
      ;[1 1 1] Slow Die
      (`/Engine/EditorBlueprintResources/StandardMacros.IncrementInt` _heridas :!label _label
        (:`  `
          (if (== _heridas 3)
            (`GameplayStatics.SpawnEmitterAtLocation` "/Game/CORE/Particles/P_Die_Boss.P_Die_Boss" (`SceneComponent.K2_GetComponentLocation` (`self.Torso`)))
            (`SceneComponent.SetVisibility` (`self.StaticMesh`) false false)
            (`SceneComponent.SetVisibility` (`self.Torso`) false false)
            (`PrimitiveComponent.SetCollisionEnabled` _grabsphere "NoCollision")
            (`KismetSystemLibrary.Delay` 2.0)
            (`PrimitiveComponent.SetCollisionEnabled` _grabsphere "QueryAndPhysics")
            (`SceneComponent.SetVisibility` (`self.Torso`) true false)
            (`SceneComponent.SetVisibility` (`self.StaticMesh`) true false)
            (set `self.Heridas` 0)))))))

(event `SlowDie`
  ;[1 1 1] Slow Die
  (goto _label))

(fn `UserConstructionScript`)